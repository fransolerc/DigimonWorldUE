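; Digiegg actor that plays a one-shot hatching sequence for the Digimon partner.
; The first event picks the egg material from a clamped index across Botamon, Punimon, Poyomon and Yuramon.
; The second sways the egg through its anim instance while a timeline drives point light glow, then removes both components.
; It then triggers the partner's animation and, after a delay, notifies dialogue and audio actors through interfaces before destroying itself.
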(event EventDigieggSequence2
  (bind _skeletalmesh_digiegg (Variables|Default|GetSkeletalMesh_Digiegg))
  (bind _returnvalue (Components|SkeletalMesh|GetAnimInstance _skeletalmesh_digiegg))
  ;[1 1 1 1 200] Digiegg Sequence
  (Utilities|FlowControl|DoOnce false
    (:Completed
      (Utilities|FlowControl|Sequence
        (:then_0
          (bind _asanimation_digiegg (Utilities|Casting|CastToAnimation_Digiegg _returnvalue))
          (Variables|/Game/Digimon/Digiegg/Animation_Digiegg.Animation_Digiegg_C|SetIsSway? _asanimation_digiegg true))
        (:then_1
          (bind _glow_intensity (Timeline|Línea%20de%20tiempo_0 PlayFromStart)
            (:Update
              (Rendering|Components|Light|SetIntensity (Variables|Default|GetPointLight) _glow_intensity))
            (:Finished
              (Utilities|FlowControl|Sequence
                (:then_0
                  (bind _asanimation_digiegg_2 (Utilities|Casting|CastToAnimation_Digiegg _returnvalue))
                  (Variables|/Game/Digimon/Digiegg/Animation_Digiegg.Animation_Digiegg_C|SetIsSway? _asanimation_digiegg_2 false))
                (:then_1
                  (Components|DestroyComponent (Variables|Default|GetSkeletalMesh_Digiegg)))
                (:then_2
                  (bind _outactors (Actor|GetAllActorswithInterface "/Game/BluePrints/BPI/BPI_Animation.BPI_Animation_C"))
                  (for _array_element _outactors
                    (bind _asai_digimon_partner (Utilities|Casting|CastToAI_DigimonPartner _array_element))
                    (CallFunction|SetAnimation _asai_digimon_partner 0 8)))
                (:then_3
                  (Utilities|FlowControl|Delay 2.0)
                  (Utilities|FlowControl|Sequence
                    (:then_0
                      (bind _outactors_2 (Actor|GetAllActorswithInterface "/Game/BluePrints/BPI/BPI_Dialogue.BPI_Dialogue_C"))
                      (for _array_element_2 _outactors_2
                        (Class|BPIDialogue|DialogueSystemUpdate(Message) _array_element_2 false)))
                    (:then_1
                      (bind _outactors_3 (Actor|GetAllActorswithInterface "/Game/BluePrints/BPI/BPI_Audio.BPI_Audio_C"))
                      (for _array_element_3 _outactors_3
                        (Class|BPIAudio|AudioSetBGM(Message) _array_element_3)))
                    (:then_2
                      (Actor|DestroyActor self))))))))))))

(event EventDigieggSequence1
  (params (Digiegg%20Index :type Integer))
  ;[1 1 1 1 100] Set Digiegg
  (Utilities|FlowControl|DoOnce false
    (:Completed
      (bind _output_get (Variables|Default|SetDigiegg_Index (Math|Integer|Clamp(Integer) Digiegg%20Index 0 3)))
      (Rendering|Material|SetMaterial (Variables|Default|GetSkeletalMesh_Digiegg) 0 (Utilities|Select :Index _output_get :Option%200 "/Game/Digimon/Digiegg/Material_Digiegg_Botamon.Material_Digiegg_Botamon" :Option%201 "/Game/Digimon/Digiegg/Material_Digiegg_Punimon.Material_Digiegg_Punimon" :Option%202 "/Game/Digimon/Digiegg/Material_Digiegg_Poyomon.Material_Digiegg_Poyomon" :Option%203 "/Game/Digimon/Digiegg/Material_Digiegg_Yuramon.Material_Digiegg_Yuramon")))))

(fn ConstructionScript)