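; Interactible poop actor that a Sukamon or Numemon partner eats when the player overlaps it.
; Construction scales the mesh by Size and picks brown or pink material from game settings.
; Eating pauses BPI_Time actors and player input for the partner's animation duration, then restores both.
; It then raises partner weight, HP and MP, writes PoopSlot into the GameInstance slot matching Index, and destroys itself.
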(event OnComponentBeginOverlap(CapsuleCollision)
  (params (OverlappedComponent :type Primitive%20Component%20Object%20Reference) (OtherActor :type Actor%20Object%20Reference) (OtherComp :type Primitive%20Component%20Object%20Reference) (OtherBodyIndex :type Integer) (bFromSweep :type Boolean) (SweepResult :type Hit%20Result%20Structure%20%28by%20ref%29))
  (bind _returnvalue (Game|GetPlayerCharacter 0))
  (bind _returnvalue_2 (Game|GetPlayerCharacter 0))
  ;[1 1 1 1 100] Sphere Collision
  (bind _asjugador (Utilities|Casting|CastToJugador OtherActor))
  (if (Variables|/Game/ThirdPersonBP/Jugador.Jugador_C|GetIsInputEnabled? _asjugador)
    (if (CallFunction|GetDigimonName)
      ;[1 1 1 1 100] EAT EVENT
      (Utilities|FlowControl|DoOnce false
        (:Completed
          (Utilities|FlowControl|Sequence
            (:then_0
              (bind _outactors (Actor|GetAllActorswithInterface "/Game/BluePrints/BPI/BPI_Time.BPI_Time_C"))
              (for _array_element _outactors
                (Class|BPITime|TimeStop(Message) _array_element)))
            (:then_1
              (Input|DisableInput _returnvalue_2 (Game|GetPlayerController 0))
              (bind _asjugador_2 (Utilities|Casting|CastToJugador _returnvalue_2))
              (Variables|/Game/ThirdPersonBP/Jugador.Jugador_C|SetIsInputEnabled? _asjugador_2 false))
            (:then_2
              (Utilities|FlowControl|Delay (CallFunction|AnimationEating))
              (Utilities|FlowControl|Sequence
                (:then_0
                  (bind _outactors_2 (Actor|GetAllActorswithInterface "/Game/BluePrints/BPI/BPI_Time.BPI_Time_C"))
                  (for _array_element_2 _outactors_2
                    (Class|BPITime|TimeStart(Message) _array_element_2)))
                (:then_1
                  (Input|EnableInput _returnvalue (Game|GetPlayerController 0))
                  (bind _asjugador_3 (Utilities|Casting|CastToJugador _returnvalue))
                  (Variables|/Game/ThirdPersonBP/Jugador.Jugador_C|SetIsInputEnabled? _asjugador_3 true))
                (:then_2
                  (CallFunction|PoopStats)
                  (Actor|DestroyActor self))))))))))

(fn ConstructionScript
  (bind _size (Variables|Default|GetSize))
  (bind _returnvalue (Math|Conversions|ToFloat(Byte) _size))
  (bind _returnvalue_2 (Math|Float|Clamp(Float) _returnvalue 1.0 3.0))
  (Transformation|SetRelativeScale3D (Variables|Default|GetStaticMesh_Poop) (Math|Vector|MakeVector _returnvalue_2 _returnvalue_2 _returnvalue_2))
  (bind _asdw1_game_instance (Utilities|Casting|CastToDW1_GameInstance (Game|GetGameInstance))
    (:then
      (CallFunction|PoopMaterial (Utilities|Struct|BreakStruct_Game_Settings (Variables|/Game/Game/DW1_GameInstance.DW1_GameInstance_C|GetGame%20Settings _asdw1_game_instance))))
    (:CastFailed
      (CallFunction|PoopMaterial false))))

(fn PoopMaterial
  (params (Original? :type Boolean))
  (Rendering|Material|SetMaterial (Variables|Default|GetStaticMesh_Poop) 0 (select Original? "/Game/StaticMeshes/Poop/Material_Poop_Brown.Material_Poop_Brown" "/Game/StaticMeshes/Poop/Material_Poop_Pink.Material_Poop_Pink")))

(fn PoopStats
  (bind _poopslot (LocalVariables|GetPoopSlot))
  (bind _asdw1_game_instance (Utilities|Casting|CastToDW1_GameInstance (Game|GetGameInstance)))
  (LocalVariables|SetGameInstance _asdw1_game_instance)
  (Utilities|Struct|SetmembersinStruct_Digimon_Partner_Info (Variables|/Game/Game/DW1_GameInstance.DW1_GameInstance_C|GetPartner%20Info (LocalVariables|GetGameInstance)) (Math|Integer|Clamp(Integer) (+ (.Weight (Utilities|Struct|BreakStruct_Digimon_Partner_Info (Variables|/Game/Game/DW1_GameInstance.DW1_GameInstance_C|GetPartner%20Info (LocalVariables|GetGameInstance)))) 3) 1 99) (Math|Integer|Clamp(Integer) (+ (.CurrentHP (Utilities|Struct|BreakStruct_Digimon_Partner_Info (Variables|/Game/Game/DW1_GameInstance.DW1_GameInstance_C|GetPartner%20Info (LocalVariables|GetGameInstance)))) (/ (.MaxHP (Utilities|Struct|BreakStruct_Digimon_Partner_Info (Variables|/Game/Game/DW1_GameInstance.DW1_GameInstance_C|GetPartner%20Info (LocalVariables|GetGameInstance)))) 10)) 1 (.MaxHP (Utilities|Struct|BreakStruct_Digimon_Partner_Info (Variables|/Game/Game/DW1_GameInstance.DW1_GameInstance_C|GetPartner%20Info (LocalVariables|GetGameInstance))))) (Math|Integer|Clamp(Integer) (+ (.CurrentMP (Utilities|Struct|BreakStruct_Digimon_Partner_Info (Variables|/Game/Game/DW1_GameInstance.DW1_GameInstance_C|GetPartner%20Info (LocalVariables|GetGameInstance)))) (/ (.MaxMP (Utilities|Struct|BreakStruct_Digimon_Partner_Info (Variables|/Game/Game/DW1_GameInstance.DW1_GameInstance_C|GetPartner%20Info (LocalVariables|GetGameInstance)))) 20)) 1 (.MaxMP (Utilities|Struct|BreakStruct_Digimon_Partner_Info (Variables|/Game/Game/DW1_GameInstance.DW1_GameInstance_C|GetPartner%20Info (LocalVariables|GetGameInstance))))))
  (switch int (Math|Integer|Clamp(Integer) (Variables|Default|GetIndex) 0 19)
    (:0
      (Utilities|Struct|SetmembersinStruct_Poop_Slots (Variables|/Game/Game/DW1_GameInstance.DW1_GameInstance_C|GetPoop%20Array (LocalVariables|GetGameInstance)) _poopslot))
    (:1
      (Utilities|Struct|SetmembersinStruct_Poop_Slots (Variables|/Game/Game/DW1_GameInstance.DW1_GameInstance_C|GetPoop%20Array (LocalVariables|GetGameInstance)) _poopslot))
    (:2
      (Utilities|Struct|SetmembersinStruct_Poop_Slots (Variables|/Game/Game/DW1_GameInstance.DW1_GameInstance_C|GetPoop%20Array (LocalVariables|GetGameInstance)) _poopslot))
    (:3
      (Utilities|Struct|SetmembersinStruct_Poop_Slots (Variables|/Game/Game/DW1_GameInstance.DW1_GameInstance_C|GetPoop%20Array (LocalVariables|GetGameInstance)) _poopslot))
    (:4
      (Utilities|Struct|SetmembersinStruct_Poop_Slots (Variables|/Game/Game/DW1_GameInstance.DW1_GameInstance_C|GetPoop%20Array (LocalVariables|GetGameInstance)) _poopslot))
    (:5
      (Utilities|Struct|SetmembersinStruct_Poop_Slots (Variables|/Game/Game/DW1_GameInstance.DW1_GameInstance_C|GetPoop%20Array (LocalVariables|GetGameInstance)) _poopslot))
    (:6
      (Utilities|Struct|SetmembersinStruct_Poop_Slots (Variables|/Game/Game/DW1_GameInstance.DW1_GameInstance_C|GetPoop%20Array (LocalVariables|GetGameInstance)) _poopslot))
    (:7
      (Utilities|Struct|SetmembersinStruct_Poop_Slots (Variables|/Game/Game/DW1_GameInstance.DW1_GameInstance_C|GetPoop%20Array (LocalVariables|GetGameInstance)) _poopslot))
    (:8
      (Utilities|Struct|SetmembersinStruct_Poop_Slots (Variables|/Game/Game/DW1_GameInstance.DW1_GameInstance_C|GetPoop%20Array (LocalVariables|GetGameInstance)) _poopslot))
    (:9
      (Utilities|Struct|SetmembersinStruct_Poop_Slots (Variables|/Game/Game/DW1_GameInstance.DW1_GameInstance_C|GetPoop%20Array (LocalVariables|GetGameInstance)) _poopslot))
    (:10
      (Utilities|Struct|SetmembersinStruct_Poop_Slots (Variables|/Game/Game/DW1_GameInstance.DW1_GameInstance_C|GetPoop%20Array (LocalVariables|GetGameInstance)) _poopslot))
    (:11
      (Utilities|Struct|SetmembersinStruct_Poop_Slots (Variables|/Game/Game/DW1_GameInstance.DW1_GameInstance_C|GetPoop%20Array (LocalVariables|GetGameInstance)) _poopslot))
    (:12
      (Utilities|Struct|SetmembersinStruct_Poop_Slots (Variables|/Game/Game/DW1_GameInstance.DW1_GameInstance_C|GetPoop%20Array (LocalVariables|GetGameInstance)) _poopslot))
    (:13
      (Utilities|Struct|SetmembersinStruct_Poop_Slots (Variables|/Game/Game/DW1_GameInstance.DW1_GameInstance_C|GetPoop%20Array (LocalVariables|GetGameInstance)) _poopslot))
    (:14
      (Utilities|Struct|SetmembersinStruct_Poop_Slots (Variables|/Game/Game/DW1_GameInstance.DW1_GameInstance_C|GetPoop%20Array (LocalVariables|GetGameInstance)) _poopslot))
    (:15
      (Utilities|Struct|SetmembersinStruct_Poop_Slots (Variables|/Game/Game/DW1_GameInstance.DW1_GameInstance_C|GetPoop%20Array (LocalVariables|GetGameInstance)) _poopslot))
    (:16
      (Utilities|Struct|SetmembersinStruct_Poop_Slots (Variables|/Game/Game/DW1_GameInstance.DW1_GameInstance_C|GetPoop%20Array (LocalVariables|GetGameInstance)) _poopslot))
    (:17
      (Utilities|Struct|SetmembersinStruct_Poop_Slots (Variables|/Game/Game/DW1_GameInstance.DW1_GameInstance_C|GetPoop%20Array (LocalVariables|GetGameInstance)) _poopslot))
    (:18
      (Utilities|Struct|SetmembersinStruct_Poop_Slots (Variables|/Game/Game/DW1_GameInstance.DW1_GameInstance_C|GetPoop%20Array (LocalVariables|GetGameInstance)) _poopslot))
    (:19
      (Utilities|Struct|SetmembersinStruct_Poop_Slots (Variables|/Game/Game/DW1_GameInstance.DW1_GameInstance_C|GetPoop%20Array (LocalVariables|GetGameInstance)) _poopslot))))

(fn GetDigimonName
  (bind _asdw1_game_instance (Utilities|Casting|CastToDW1_GameInstance (Game|GetGameInstance))
    (:then
      (bind _output_get (LocalVariables|SetDigimonName_Local (Utilities|Struct|BreakStruct_Digimon_Partner_Info (Variables|/Game/Game/DW1_GameInstance.DW1_GameInstance_C|GetPartner%20Info _asdw1_game_instance))))
      (if (or (Utilities|Name|Equal(Name) _output_get "Sukamon") (Utilities|Name|Equal(Name) _output_get "Numemon"))
        (bind _returnvalue (Class|DataTableFunctionLibrary|DoesDataTableRowExist "/Game/Game/DataTables/DigimonInfo/DataTable_Digimon_Info.DataTable_Digimon_Info" (LocalVariables|GetDigimonName_Local)))
        (return _returnvalue)
        (else
          (return false))))
    (:CastFailed
      (return false))))

(fn AnimationEating
  (bind _outactors (Actor|GetAllActorsOfClass "/Game/AI/Pawn_Partner/AI_DigimonPartner.AI_DigimonPartner_C"))
  (bind _array_element (Utilities|Array|ForEachLoopwithBreak _outactors :!label _label)
    (:LoopBody
      (Utilities|IsValid _array_element
        (:Is%20Valid
          (bind _duration (CallFunction|SetAnimation _array_element 0 9))
          (LocalVariables|SetAnimation_Duration _duration)
          (goto _label Break))))
    (:Completed
      (return (LocalVariables|GetAnimation_Duration)))))