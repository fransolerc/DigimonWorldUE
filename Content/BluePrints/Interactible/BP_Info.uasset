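; BP_Info is an interactible info point that plays dialogue from its Database table when the player interacts nearby.
; A box, sized in the construction script, registers it with Jugador on overlap, switches the interaction bubble and tracks proximity.
; Interaction unlocks every BPI_Dialogue actor and sends it the table with autoplay; leaving the box resets their messages.
; A failed proximity or Database check on interaction prints an invalid-datatable error.
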(event OnComponentBeginOverlap(BoxCollision)
  (params (OverlappedComponent :type Primitive%20Component%20Object%20Reference) (OtherActor :type Actor%20Object%20Reference) (OtherComp :type Primitive%20Component%20Object%20Reference) (OtherBodyIndex :type Integer) (bFromSweep :type Boolean) (SweepResult :type Hit%20Result%20Structure%20%28by%20ref%29))
  ;[1 1 1 1 100] Overlap
  (bind _asjugador (Utilities|Casting|CastToJugador OtherActor))
  (if (Utilities|IsValid (Variables|Text|GetDatabase))
    (Class|BPIInteract|InteractibleSet(Message) _asjugador self)
    (Default|InteractionBubble _asjugador "NewEnumerator0")
    (Variables|Default|SetIsCloseToPlayer? true)))

(event OnComponentEndOverlap(BoxCollision)
  (params (OverlappedComponent :type Primitive%20Component%20Object%20Reference) (OtherActor :type Actor%20Object%20Reference) (OtherComp :type Primitive%20Component%20Object%20Reference) (OtherBodyIndex :type Integer))
  ;[1 1 1 1 100] Overlap
  (bind _asjugador (Utilities|Casting|CastToJugador OtherActor))
  (if (Utilities|IsValid (Variables|Text|GetDatabase))
    (Class|BPIInteract|InteractibleUnset(Message) _asjugador)
    (Default|InteractionBubble _asjugador "NewEnumerator3")
    (Variables|Default|SetIsCloseToPlayer? false)
    (bind _outactors (Actor|GetAllActorswithInterface "/Game/BluePrints/BPI/BPI_Dialogue.BPI_Dialogue_C"))
    (for _array_element _outactors
      (Class|BPIDialogue|DialogueSystemReset(Message) _array_element))))

(event EventInteraction
  ;[1 1 1 1 100] Interaction
  (if (and (Variables|Default|GetIsCloseToPlayer?) (Utilities|IsValid (Variables|Text|GetDatabase)))
    (Utilities|FlowControl|Sequence
      (:then_0
        (bind _outactors (Actor|GetAllActorswithInterface "/Game/BluePrints/BPI/BPI_Dialogue.BPI_Dialogue_C"))
        (for _array_element _outactors
          (Class|BPIDialogue|DialogueSystemLock(Message) _array_element false)
          (Class|BPIDialogue|DialogueSystemValuesSet(Message) _array_element self (Variables|Text|GetDatabase) true)))
      (:then_1
        (bind _asjugador (Utilities|Casting|CastToJugador (Game|GetPlayerCharacter 0)))
        (Default|InteractionBubble _asjugador "NewEnumerator3")))
    (else
      (Development|PrintString "Datatable NOT VALID" true true "(R=1.000000,G=0.000000,B=0.000000,A=1.000000)"))))

(fn ConstructionScript
  (Components|Box|SetBoxExtent (Variables|Default|GetBoxCollision) (Variables|BoxCollision|GetBoxCollisionSize) true))