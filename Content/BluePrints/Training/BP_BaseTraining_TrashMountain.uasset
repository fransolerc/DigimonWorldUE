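; Trash mountain training station in a Digimon raising game, configured from the TrashMountain_MP row of the training info data table.
; On training start it disables mesh collision, sends every partner Digimon's AI to the mesh with a set behaviour, and blends the view to the training camera.
; When a partner leaves the sphere trigger, the mesh returns to query-only collision.
; Construction loads the row before running the parent's setup.
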(event OnComponentEndOverlap(SphereCollision)
  (params (OverlappedComponent :type Primitive%20Component%20Object%20Reference) (OtherActor :type Actor%20Object%20Reference) (OtherComp :type Primitive%20Component%20Object%20Reference) (OtherBodyIndex :type Integer))
  ;[1 1 1 1 100] POOP
  (Utilities|Casting|CastToAI_DigimonPartner OtherActor)
  (Collision|SetCollisionEnabled (Variables|Default|GetStaticMesh) "QueryOnly"))

(event EventTrainingStart
  ;[1 1 1 1 100] POOP
  (Utilities|FlowControl|Sequence
    (:then_0
      (Collision|SetCollisionEnabled (Variables|Default|GetStaticMesh) "NoCollision")
      (bind _outactors (Actor|GetAllActorsOfClass "/Game/AI/Pawn_Partner/AI_DigimonPartner.AI_DigimonPartner_C"))
      (for _array_element _outactors
        (Utilities|IsValid _array_element
          (:Is%20Valid
            (Default|AILocation _array_element (Transformation|GetWorldLocation (Variables|Default|GetStaticMesh)))
            (Default|AIBehaviourNormal _array_element "NewEnumerator8")))))
    (:then_1
      (Game|Player|SetViewTargetwithBlend (Game|GetPlayerController 0) (Components|GetOwner (Variables|Default|GetTrainingCamera)) 0.4 "VTBlend_EaseInOut" 1.0 false))))

(fn ConstructionScript
  (bind _returnvalue (Utilities|GetDataTableRow "/Game/Game/DataTables/Training/DataTable_Training_Info.DataTable_Training_Info" "TrashMountain_MP")
    (:then
      (Variables|Default|SetBaseTraining_Info _returnvalue)
      (|CallParentFunction))))