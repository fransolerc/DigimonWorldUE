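; Misty Trees brains training spot, where the partner Digimon trains with Cherrymon.
; On training start it caches Cherrymon from the game instance NPC array and finds the partner, moves the player to the billboard and blends to the training camera.
; A timeline's event tracks trigger animations on both Digimon and Cherrymon's sound until training stops.
; The construction script loads its training info row from a data table before running the parent's setup.
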(event EventTrainingStop
  ;[1 1 1 1 100] Cherrymon
  (Timeline|Timeline_0 Stop
    (:Cherrymon
      (CallFunction|SetAnimation (Variables|Default|GetCherrymon) 0 8)
      (Audio|PlaySound2D "/Game/Audio/SFX/DigimonVoices/Cherrymon.Cherrymon" 1.0 1.0 0.0 0 0))
    (:Partner
      (CallFunction|SetAnimation (Variables|Default|GetPartner)))))

(event EventTrainingStart
  ;[1 1 1 1 100] Cherrymon
  (Utilities|FlowControl|Sequence
    (:then_0
      (Utilities|IsValid (Variables|Default|GetCherrymon)
        (:Is%20Not%20Valid
          (bind _asdw1_game_instance (Utilities|Casting|CastToDW1_GameInstance (Game|GetGameInstance)))
          (Variables|Default|SetCherrymon (Utilities|Struct|BreakStruct_NPC_Array (Variables|/Game/Game/DW1_GameInstance.DW1_GameInstance_C|GetNPC_Array _asdw1_game_instance))))))
    (:then_1
      (Utilities|IsValid (Variables|Default|GetPartner)
        (:Is%20Not%20Valid
          (bind _outactors (Actor|GetAllActorsOfClass "/Game/AI/Pawn_Partner/AI_DigimonPartner.AI_DigimonPartner_C"))
          (for _array_element _outactors
            (Utilities|IsValid _array_element
              (:Is%20Valid
                (Variables|Default|SetPartner _array_element)))))))
    (:then_2
      (AI|Navigation|SimpleMovetoLocation (Game|GetPlayerController 0) (Transformation|GetWorldLocation (Variables|Default|GetBillboard))))
    (:then_3
      (if (and (Utilities|IsValid (Variables|Default|GetCherrymon)) (Utilities|IsValid (Variables|Default|GetPartner)))
        (Timeline|Timeline_0 PlayFromStart
          (:Cherrymon
            (CallFunction|SetAnimation (Variables|Default|GetCherrymon) 0 8)
            (Audio|PlaySound2D "/Game/Audio/SFX/DigimonVoices/Cherrymon.Cherrymon" 1.0 1.0 0.0 0 0))
          (:Partner
            (CallFunction|SetAnimation (Variables|Default|GetPartner))))))
    (:then_4
      (Game|Player|SetViewTargetwithBlend (Game|GetPlayerController 0) (Components|GetOwner (Variables|Default|GetTrainingCamera)) 0.4 "VTBlend_EaseInOut" 1.0 false))))

(fn ConstructionScript
  (bind _returnvalue (Utilities|GetDataTableRow "/Game/Game/DataTables/Training/DataTable_Training_Info.DataTable_Training_Info" "MistyTrees_Brains")
    (:then
      (Variables|Default|SetBaseTraining_Info _returnvalue)
      (|CallParentFunction))))