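; Defense training station in the Ice Sanctuary, built on a base training Blueprint, with its info read from a data table row at construction.
; TrainingStart sends partner Digimon to the Billboard location, sets their behaviour and blends to the training camera.
; Once a partner overlaps the box, Tick fires a DoOnce-gated looping timeline that moves icicles, flips their visibility and triggers the partner's animation.
; TrainingStop clears state and resets the gate.
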(event OnComponentBeginOverlap(BoxCollision)
  (params (OverlappedComponent :type Primitive%20Component%20Object%20Reference) (OtherActor :type Actor%20Object%20Reference) (OtherComp :type Primitive%20Component%20Object%20Reference) (OtherBodyIndex :type Integer) (bFromSweep :type Boolean) (SweepResult :type Hit%20Result%20Structure%20%28by%20ref%29))
  ;[1 1 1 1 100] Defense
  (bind _asai_digimon_partner (Utilities|Casting|CastToAI_DigimonPartner OtherActor))
  (Variables|Default|SetDigimonPartnerRef _asai_digimon_partner)
  (Variables|Default|SetIsInBaseTraining? true))

(event OnComponentEndOverlap(BoxCollision)
  (params (OverlappedComponent :type Primitive%20Component%20Object%20Reference) (OtherActor :type Actor%20Object%20Reference) (OtherComp :type Primitive%20Component%20Object%20Reference) (OtherBodyIndex :type Integer))
  ;[1 1 1 1 100] Defense
  (bind _asai_digimon_partner (Utilities|Casting|CastToAI_DigimonPartner OtherActor))
  (Variables|Default|SetDigimonPartnerRef _asai_digimon_partner)
  (Variables|Default|SetIsInBaseTraining? false))

(event EventTick
  (params (DeltaSeconds :type Float%20%28single-precision%29))
  (bind _sm_icicles (Variables|Default|GetSM_Icicles))
  ;[1 1 1 1 100] Defense
  (if (and (Variables|Default|GetIsInBaseTraining?) (Variables|Default|GetStarted?))
    (Utilities|FlowControl|DoOnce false
      (:Completed
        (bind _location (Timeline|Icicle%20Timeline PlayFromStart)
          (:Update
            (Transformation|SetRelativeLocation _sm_icicles (Math|Vector|MakeVector 0.0 0.0 _location) false false))
          (:Finished
            (if (Variables|Default|GetStarted?)
              (Timeline|Icicle%20Timeline PlayFromStart)
              (else
                (Development|SetHiddeninGame _sm_icicles true false))))
          (:Animation
            (CallFunction|SetAnimation (Variables|Default|GetDigimonPartnerRef) 0 5))
          (:Visibility
            (bind _isa (Utilities|FlowControl|FlipFlop)
              (:A
                _)
              (:B
                _))
            (Development|SetHiddeninGame _sm_icicles _isa false)))))))

(event EventTrainingStop
  (bind _sm_icicles (Variables|Default|GetSM_Icicles))
  ;[1 1 1 1 100] Defense
  (Variables|Default|SetIsInBaseTraining? false)
  (Variables|Default|SetStarted? false)
  (Actor|Tick|SetActorTickEnabled false)
  (Utilities|FlowControl|DoOnce false) ; enters at Reset
)

(event EventTrainingStart
  ;[1 1 1 1 100] Defense
  (Utilities|FlowControl|Sequence
    (:then_0
      (Actor|Tick|SetActorTickEnabled true)
      (Variables|Default|SetStarted? true)
      (bind _outactors (Actor|GetAllActorsOfClass "/Game/AI/Pawn_Partner/AI_DigimonPartner.AI_DigimonPartner_C"))
      (for _array_element _outactors
        (Utilities|IsValid _array_element
          (:Is%20Valid
            (Variables|Default|SetDigimonPartnerRef _array_element)
            (Default|AILocation (Variables|Default|GetDigimonPartnerRef) (Transformation|GetWorldLocation (Variables|Default|GetBillboard)))
            (Default|AIBehaviourNormal (Variables|Default|GetDigimonPartnerRef) "NewEnumerator8")))))
    (:then_1
      (Game|Player|SetViewTargetwithBlend (Game|GetPlayerController 0) (Components|GetOwner (Variables|Default|GetTrainingCamera)) 0.4 "VTBlend_EaseInOut" 1.0 false))))

(fn ConstructionScript
  (bind _returnvalue (Utilities|GetDataTableRow "/Game/Game/DataTables/Training/DataTable_Training_Info.DataTable_Training_Info" "IceSanctuary_Defense")
    (:then
      (Variables|Default|SetBaseTraining_Info _returnvalue)
      (|CallParentFunction))))