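; MP training station for Digimon partners, a child Blueprint of a base training actor.
; The construction script loads the GreenGym_MP row from the training info data table into BaseTrainingInfo, then runs the parent script if the row is found.
; On TrainingStart, it passes the billboard's location to every valid AI_DigimonPartner, sets their behaviour state, and blends the player's view to the training camera.
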(event EventTrainingStart
  ;[1 1 1 1 100] MP
  (Utilities|FlowControl|Sequence
    (:then_0
      (bind _outactors (Actor|GetAllActorsOfClass "/Game/AI/Pawn_Partner/AI_DigimonPartner.AI_DigimonPartner_C"))
      (for _array_element _outactors
        (Utilities|IsValid _array_element
          (:Is%20Valid
            (Default|AILocation _array_element (Transformation|GetWorldLocation (Variables|Default|GetBillboard)))
            (Default|AIBehaviourNormal _array_element "NewEnumerator8")))))
    (:then_1
      (Game|Player|SetViewTargetwithBlend (Game|GetPlayerController 0) (Components|GetOwner (Variables|Default|GetTrainingCamera)) 0.4 "VTBlend_EaseInOut" 1.0 false))))

(fn ConstructionScript
  (bind _returnvalue (Utilities|GetDataTableRow "/Game/Game/DataTables/Training/DataTable_Training_Info.DataTable_Training_Info" "GreenGym_MP")
    (:then
      (Variables|Default|SetBaseTraining_Info _returnvalue)
      (|CallParentFunction))))