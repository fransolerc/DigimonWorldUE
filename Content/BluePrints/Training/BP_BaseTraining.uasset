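; Base training station actor that lets the player raise their partner Digimon's stats.
; Box overlap toggles an interaction bubble, and interacting sends its DataTable to dialogue actors.
; Confirm input plays sounds, stops training input and shows a gains widget fed by CalculateStatsGain.
; That function scales gains by preference, level, manual, recruit bonuses and tiredness, and also writes clamped stats and condition costs to GameInstance PartnerInfo.
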(event OnComponentBeginOverlap(BasePlayer_Box)
  (params (OverlappedComponent :type Primitive%20Component%20Object%20Reference) (OtherActor :type Actor%20Object%20Reference) (OtherComp :type Primitive%20Component%20Object%20Reference) (OtherBodyIndex :type Integer) (bFromSweep :type Boolean) (SweepResult :type Hit%20Result%20Structure%20%28by%20ref%29))
  ;[1 1 1 1 200] Overlap
  (bind _asjugador (Utilities|Casting|CastToJugador OtherActor))
  (if (Utilities|IsValid (Utilities|Struct|BreakStruct_Training_Info (Variables|BaseTrainingInfo|GetBaseTraining_Info)))
    (Class|BPIInteract|InteractibleSet(Message) _asjugador self)
    (Default|InteractionBubble _asjugador "NewEnumerator0")))

(event OnComponentEndOverlap(BasePlayer_Box)
  (params (OverlappedComponent :type Primitive%20Component%20Object%20Reference) (OtherActor :type Actor%20Object%20Reference) (OtherComp :type Primitive%20Component%20Object%20Reference) (OtherBodyIndex :type Integer))
  ;[1 1 1 1 200] Overlap
  (bind _asjugador (Utilities|Casting|CastToJugador OtherActor))
  (if (Utilities|IsValid (Utilities|Struct|BreakStruct_Training_Info (Variables|BaseTrainingInfo|GetBaseTraining_Info)))
    (Class|BPIInteract|InteractibleUnset(Message) _asjugador)
    (Default|InteractionBubble _asjugador "NewEnumerator3")))

(event EventInteraction
  (bind _basetraining_info (Variables|BaseTrainingInfo|GetBaseTraining_Info))
  (bind _datatable (Utilities|Struct|BreakStruct_Training_Info _basetraining_info))
  ;[1 1 1 1 200] Interaction
  (if (Utilities|IsValid _datatable)
    (Utilities|FlowControl|Sequence
      (:then_0
        (bind _outactors (Actor|GetAllActorswithInterface "/Game/BluePrints/BPI/BPI_Dialogue.BPI_Dialogue_C"))
        (for _array_element _outactors
          (Class|BPIDialogue|DialogueSystemValuesSet(Message) _array_element self _datatable true)))
      (:then_1
        (bind _asjugador (Utilities|Casting|CastToJugador (Game|GetPlayerCharacter 0)))
        (Default|InteractionBubble _asjugador "NewEnumerator3")))))

(event Input|ActionEvents|InputActionInteraction[Cross]
  (params (Key :type Key%20Structure :default "None"))
  (bind (_hp_gain _mp_gain _offense_gain _defense_gain _speed_gain _brains_gain) (CallFunction|CalculateStatsGain))
  (bind _self self)
  ;[1 1 1 1 200] END
  (:Pressed
    (if (Utilities|IsValid (Utilities|Struct|BreakStruct_Training_Info (Variables|BaseTrainingInfo|GetBaseTraining_Info)))
      (Utilities|FlowControl|Sequence
        (:then_0
          ;;[1 1 1 1 100] SOUND
          (Audio|PlaySound2D "/Game/Audio/SFX/UI/UI_Button_WindowOpen.UI_Button_WindowOpen" 0.5 1.0 0.0 0 0)
          (Audio|PlaySound2D "/Game/Audio/SFX/Ambient/GreenGym_bell02.GreenGym_bell02" 0.5 1.0 0.0 0 0))
        (:then_1
          ;;[1 1 1 1 100] STOP
          (Input|DisableInput _self (Game|GetPlayerController 0))
          (Class|BPITraining|TrainingStop(Message) _self))
        (:then_2
          ;;[1 1 1 1 100] WIDGET
          (bind _returnvalue (UserInterface|CreateWidget "/Game/UI/Battle_Stats_Bits.Battle_Stats_Bits_C"))
          (UserInterface|Viewport|AddtoViewport _returnvalue 99)
          (Default|TrainingStatsEvent _returnvalue (Utilities|Struct|BreakStruct_Training_Info (Variables|BaseTrainingInfo|GetBaseTraining_Info)) _hp_gain _mp_gain _offense_gain _defense_gain _speed_gain _brains_gain))))))

(fn ConstructionScript)

(fn CalculateStatsGain
  (bind _asdw1_game_instance (Utilities|Casting|CastToDW1_GameInstance (Game|GetGameInstance))
    (:then
      (LocalVariables|SetGameInstance _asdw1_game_instance)
      (LocalVariables|SetPartnerInfo (Variables|/Game/Game/DW1_GameInstance.DW1_GameInstance_C|GetPartner%20Info (LocalVariables|GetGameInstance)))
      (LocalVariables|SetIsKuwagamon? (.Trigger14-RecruitedKuwagamon (Utilities|Struct|BreakStruct_Game_Triggers (Variables|/Game/Game/DW1_GameInstance.DW1_GameInstance_C|GetGame%20Triggers (LocalVariables|GetGameInstance)))))
      (LocalVariables|SetIsKabuterimon? (.Trigger34-RecruitedKabuterimon (Utilities|Struct|BreakStruct_Game_Triggers (Variables|/Game/Game/DW1_GameInstance.DW1_GameInstance_C|GetGame%20Triggers (LocalVariables|GetGameInstance)))))
      (LocalVariables|SetTrainingManual? (.Found? (CallFunction|InventoryItemFind "TrainingManual")))
      (bind _returnvalue (Class|DataTableFunctionLibrary|DoesDataTableRowExist "/Game/Game/DataTables/DigimonInfo/DataTable_Digimon_Info.DataTable_Digimon_Info" (Utilities|Struct|BreakStruct_Digimon_Partner_Info (LocalVariables|GetPartnerInfo))))
      (if _returnvalue
        (bind _returnvalue_2 (Utilities|GetDataTableRow "/Game/Game/DataTables/DigimonInfo/DataTable_Digimon_Info.DataTable_Digimon_Info" (Utilities|Struct|BreakStruct_Digimon_Partner_Info (LocalVariables|GetPartnerInfo)))
          (:then
            (LocalVariables|SetDigimonInfo _returnvalue_2)
            (LocalVariables|SetLevelFactor (Utilities|Select :Index (Utilities|Struct|BreakStruct_Digimon_Info (LocalVariables|GetDigimonInfo)) :NewEnumerator0 0.9 :NewEnumerator1 0.9 :NewEnumerator2 1.0 :NewEnumerator3 1.1 :NewEnumerator4 1.2 :NewEnumerator5 1.2))
            (LocalVariables|SetHP%20Integer (Math|Float|Truncate (* (Math|Conversions|ToFloat(Byte) (Utilities|Struct|BreakStruct_Training_Info (Variables|BaseTrainingInfo|GetBaseTraining_Info))) (Utilities|Select :Index (Utilities|Struct|BreakStruct_Digimon_Info (LocalVariables|GetDigimonInfo)) :NewEnumerator1 1.0 :NewEnumerator2 1.1 :NewEnumerator3 0.9 :NewEnumerator4 1.0 :NewEnumerator5 0.8) (LocalVariables|GetLevelFactor) (select (LocalVariables|GetTrainingManual?) 1.1 1.0) (select (and (LocalVariables|GetIsKabuterimon?) (Utilities|Struct|BreakStruct_Training_Info (Variables|BaseTrainingInfo|GetBaseTraining_Info))) 1.2 1.0) (select (>= (Utilities|Struct|BreakStruct_Digimon_Partner_Info (LocalVariables|GetPartnerInfo)) 80) 0.8 1.0))))
            (LocalVariables|SetMP%20Integer (Math|Float|Truncate (* (Math|Conversions|ToFloat(Byte) (Utilities|Struct|BreakStruct_Training_Info (Variables|BaseTrainingInfo|GetBaseTraining_Info))) (Utilities|Select :Index (Utilities|Struct|BreakStruct_Digimon_Info (LocalVariables|GetDigimonInfo)) :NewEnumerator1 1.0 :NewEnumerator2 1.0 :NewEnumerator3 1.1 :NewEnumerator4 0.9 :NewEnumerator5 0.8) (LocalVariables|GetLevelFactor) (select (LocalVariables|GetTrainingManual?) 1.1 1.0) (select (and (LocalVariables|GetIsKuwagamon?) (Utilities|Struct|BreakStruct_Training_Info (Variables|BaseTrainingInfo|GetBaseTraining_Info))) 1.2 1.0) (select (>= (Utilities|Struct|BreakStruct_Digimon_Partner_Info (LocalVariables|GetPartnerInfo)) 80) 0.8 1.0))))
            (LocalVariables|SetOffense%20Integer (Math|Float|Truncate (* (Math|Conversions|ToFloat(Byte) (Utilities|Struct|BreakStruct_Training_Info (Variables|BaseTrainingInfo|GetBaseTraining_Info))) (Utilities|Select :Index (Utilities|Struct|BreakStruct_Digimon_Info (LocalVariables|GetDigimonInfo)) :NewEnumerator1 1.0 :NewEnumerator2 0.9 :NewEnumerator3 1.0 :NewEnumerator4 1.1 :NewEnumerator5 0.8) (LocalVariables|GetLevelFactor) (select (LocalVariables|GetTrainingManual?) 1.1 1.0) (select (and (LocalVariables|GetIsKuwagamon?) (Utilities|Struct|BreakStruct_Training_Info (Variables|BaseTrainingInfo|GetBaseTraining_Info))) 1.2 1.0) (select (>= (Utilities|Struct|BreakStruct_Digimon_Partner_Info (LocalVariables|GetPartnerInfo)) 80) 0.8 1.0))))
            (LocalVariables|SetDefense%20Integer (Math|Float|Truncate (* (Math|Conversions|ToFloat(Byte) (Utilities|Struct|BreakStruct_Training_Info (Variables|BaseTrainingInfo|GetBaseTraining_Info))) (Utilities|Select :Index (Utilities|Struct|BreakStruct_Digimon_Info (LocalVariables|GetDigimonInfo)) :NewEnumerator1 1.0 :NewEnumerator2 1.1 :NewEnumerator3 0.9 :NewEnumerator4 1.0 :NewEnumerator5 0.8) (LocalVariables|GetLevelFactor) (select (LocalVariables|GetTrainingManual?) 1.1 1.0) (select (and (LocalVariables|GetIsKabuterimon?) (Utilities|Struct|BreakStruct_Training_Info (Variables|BaseTrainingInfo|GetBaseTraining_Info))) 1.2 1.0) (select (>= (Utilities|Struct|BreakStruct_Digimon_Partner_Info (LocalVariables|GetPartnerInfo)) 80) 0.8 1.0))))
            (LocalVariables|SetSpeed%20Integer (Math|Float|Truncate (* (Math|Conversions|ToFloat(Byte) (Utilities|Struct|BreakStruct_Training_Info (Variables|BaseTrainingInfo|GetBaseTraining_Info))) (Utilities|Select :Index (Utilities|Struct|BreakStruct_Digimon_Info (LocalVariables|GetDigimonInfo)) :NewEnumerator1 1.0 :NewEnumerator2 0.9 :NewEnumerator3 1.0 :NewEnumerator4 1.1 :NewEnumerator5 0.8) (LocalVariables|GetLevelFactor) (select (LocalVariables|GetTrainingManual?) 1.1 1.0) (select (and (LocalVariables|GetIsKabuterimon?) (Utilities|Struct|BreakStruct_Training_Info (Variables|BaseTrainingInfo|GetBaseTraining_Info))) 1.2 1.0) (select (>= (Utilities|Struct|BreakStruct_Digimon_Partner_Info (LocalVariables|GetPartnerInfo)) 80) 0.8 1.0))))
            (LocalVariables|SetBrains%20Integer (Math|Float|Truncate (* (Math|Conversions|ToFloat(Byte) (Utilities|Struct|BreakStruct_Training_Info (Variables|BaseTrainingInfo|GetBaseTraining_Info))) (Utilities|Select :Index (Utilities|Struct|BreakStruct_Digimon_Info (LocalVariables|GetDigimonInfo)) :NewEnumerator1 1.0 :NewEnumerator2 1.0 :NewEnumerator3 1.1 :NewEnumerator4 0.9 :NewEnumerator5 0.8) (LocalVariables|GetLevelFactor) (select (LocalVariables|GetTrainingManual?) 1.1 1.0) (select (and (LocalVariables|GetIsKuwagamon?) (Utilities|Struct|BreakStruct_Training_Info (Variables|BaseTrainingInfo|GetBaseTraining_Info))) 1.2 1.0) (select (>= (Utilities|Struct|BreakStruct_Digimon_Partner_Info (LocalVariables|GetPartnerInfo)) 80) 0.8 1.0))))
            ;[1 1 1 1 200] END
            (Utilities|Struct|SetmembersinStruct_Digimon_Partner_Info (Variables|/Game/Game/DW1_GameInstance.DW1_GameInstance_C|GetPartner%20Info (LocalVariables|GetGameInstance)) (Math|Integer|Clamp(Integer) (+ (.Tiredness (Utilities|Struct|BreakStruct_Digimon_Partner_Info (LocalVariables|GetPartnerInfo))) (Math|Conversions|ToInteger(Byte) (Utilities|Struct|BreakStruct_Training_Info (Variables|BaseTrainingInfo|GetBaseTraining_Info)))) 0 100) (Math|Integer|Clamp(Integer) (- (.EnergyLevel (Utilities|Struct|BreakStruct_Digimon_Partner_Info (LocalVariables|GetPartnerInfo))) 6) 0 80) (Math|Integer|Clamp(Integer) (- (.Happiness (Utilities|Struct|BreakStruct_Digimon_Partner_Info (LocalVariables|GetPartnerInfo))) 1) -100 100) (Math|Integer|Clamp(Integer) (- (.RemainingLifetimeHours (Utilities|Struct|BreakStruct_Digimon_Partner_Info (LocalVariables|GetPartnerInfo))) 1) 0 999) (Math|Integer|Clamp(Integer) (+ (.AgeinHoursforEvolve (Utilities|Struct|BreakStruct_Digimon_Partner_Info (LocalVariables|GetPartnerInfo))) 1) 0 999) (Math|Integer|Clamp(Integer) (+ (.MaxHP (Utilities|Struct|BreakStruct_Digimon_Partner_Info (LocalVariables|GetPartnerInfo))) (LocalVariables|GetHP%20Integer)) 1 9999) (Math|Integer|Clamp(Integer) (+ (.MaxMP (Utilities|Struct|BreakStruct_Digimon_Partner_Info (LocalVariables|GetPartnerInfo))) (LocalVariables|GetMP%20Integer)) 1 9999) (Math|Integer|Clamp(Integer) (+ (.Offense (Utilities|Struct|BreakStruct_Digimon_Partner_Info (LocalVariables|GetPartnerInfo))) (LocalVariables|GetOffense%20Integer)) 1 999) (Math|Integer|Clamp(Integer) (+ (.Defense (Utilities|Struct|BreakStruct_Digimon_Partner_Info (LocalVariables|GetPartnerInfo))) (LocalVariables|GetDefense%20Integer)) 1 999) (Math|Integer|Clamp(Integer) (+ (.Speed (Utilities|Struct|BreakStruct_Digimon_Partner_Info (LocalVariables|GetPartnerInfo))) (LocalVariables|GetSpeed%20Integer)) 1 999) (Math|Integer|Clamp(Integer) (+ (.Brains (Utilities|Struct|BreakStruct_Digimon_Partner_Info (LocalVariables|GetPartnerInfo))) (LocalVariables|GetBrains%20Integer)) 1 999))
            (return (LocalVariables|GetHP%20Integer) (LocalVariables|GetMP%20Integer) (LocalVariables|GetOffense%20Integer) (LocalVariables|GetDefense%20Integer) (LocalVariables|GetSpeed%20Integer) (LocalVariables|GetBrains%20Integer)))
          (:RowNotFound
            _)))
      (Development|PrintString "DigimonName NOT FOUND" true true "(R=1.000000,G=0.000000,B=0.000000,A=1.000000)")
      (return 0 0 0 0 0 0))
    (:CastFailed
      (return 0 0 0 0 0 0))))