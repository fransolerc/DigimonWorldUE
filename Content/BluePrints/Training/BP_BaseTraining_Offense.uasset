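; Offense training station for Digimon partners at the Green Gym, a child Blueprint that loads its info row from the training data table on construction.
; TrainingStart sends every partner AI to the billboard location, changes its behaviour and blends the view to the training camera.
; Once a partner overlaps the box, Tick fires once to start a repeating animation and timeline that moves the gym tree until TrainingStop resets it.
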(event OnComponentBeginOverlap(BoxCollision)
  (params (OverlappedComponent :type Primitive%20Component%20Object%20Reference) (OtherActor :type Actor%20Object%20Reference) (OtherComp :type Primitive%20Component%20Object%20Reference) (OtherBodyIndex :type Integer) (bFromSweep :type Boolean) (SweepResult :type Hit%20Result%20Structure%20%28by%20ref%29))
  ;[1 1 1 1 100] Offense
  (bind _asai_digimon_partner (Utilities|Casting|CastToAI_DigimonPartner OtherActor))
  (Variables|Default|SetDigimonPartnerRef _asai_digimon_partner)
  (Variables|Default|SetIsInBaseTraining? true))

(event OnComponentEndOverlap(BoxCollision)
  (params (OverlappedComponent :type Primitive%20Component%20Object%20Reference) (OtherActor :type Actor%20Object%20Reference) (OtherComp :type Primitive%20Component%20Object%20Reference) (OtherBodyIndex :type Integer))
  ;[1 1 1 1 100] Offense
  (bind _asai_digimon_partner (Utilities|Casting|CastToAI_DigimonPartner OtherActor))
  (Variables|Default|SetDigimonPartnerRef _asai_digimon_partner)
  (Variables|Default|SetIsInBaseTraining? false))

(event EventTrainingStart
  ;[1 1 1 1 100] Offense
  (Utilities|FlowControl|Sequence
    (:then_0
      (Variables|Default|SetStarted? true)
      (Actor|Tick|SetActorTickEnabled true)
      (bind _outactors (Actor|GetAllActorsOfClass "/Game/AI/Pawn_Partner/AI_DigimonPartner.AI_DigimonPartner_C"))
      (for _array_element _outactors
        (Utilities|IsValid _array_element
          (:Is%20Valid
            (Variables|Default|SetDigimonPartnerRef _array_element)
            (Default|AILocation (Variables|Default|GetDigimonPartnerRef) (Transformation|GetWorldLocation (Variables|Default|GetBillboard)))
            (Default|AIBehaviourNormal (Variables|Default|GetDigimonPartnerRef) "NewEnumerator8")))))
    (:then_1
      (Game|Player|SetViewTargetwithBlend (Game|GetPlayerController 0) (Components|GetOwner (Variables|Default|GetTrainingCamera)) 0.4 "VTBlend_EaseInOut" 1.0 false))))

(event EventTick
  (params (DeltaSeconds :type Float%20%28single-precision%29))
  ;[1 1 1 1 100] Offense
  (if (and (Variables|Default|GetIsInBaseTraining?) (Variables|Default|GetStarted?))
    (Utilities|FlowControl|DoOnce false
      (:Completed
        (CallFunction|SetAnimation (Variables|Default|GetDigimonPartnerRef) :!label _label)
        (bind _location (Timeline|Línea%20de%20tiempo_Offense PlayFromStart)
          (:Update
            (Transformation|SetRelativeLocation (Variables|Default|GetGreenGym_Tree) (Math|Vector|MakeVector -2.9e+02 _location 0.0) false false))
          (:Finished
            (if (Variables|Default|GetStarted?)
              (goto _label))))))))

(event EventTrainingStop
  ;[1 1 1 1 100] Offense
  (Variables|Default|SetIsInBaseTraining? false)
  (Variables|Default|SetStarted? false)
  (Actor|Tick|SetActorTickEnabled false)
  (Utilities|FlowControl|DoOnce false) ; enters at Reset
)

(fn ConstructionScript
  (bind _returnvalue (Utilities|GetDataTableRow "/Game/Game/DataTables/Training/DataTable_Training_Info.DataTable_Training_Info" "GreenGym_Offense")
    (:then
      (Variables|Default|SetBaseTraining_Info _returnvalue)
      (|CallParentFunction))))