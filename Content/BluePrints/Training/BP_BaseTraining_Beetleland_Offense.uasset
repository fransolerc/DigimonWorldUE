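; Beetleland Offense base training station, where the Digimon partner performs a looping punch exercise.
; Training start sends the partner to the billboard spot, finding it if needed, and blends the view to the training camera.
; While the partner overlaps the box, Tick starts a self-replaying timeline that slides the movable part and triggers partner animations until training stops.
; The construction script loads its training info from a data table row before running the parent's.
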(event OnComponentBeginOverlap(BoxCollision)
  (params (OverlappedComponent :type Primitive%20Component%20Object%20Reference) (OtherActor :type Actor%20Object%20Reference) (OtherComp :type Primitive%20Component%20Object%20Reference) (OtherBodyIndex :type Integer) (bFromSweep :type Boolean) (SweepResult :type Hit%20Result%20Structure%20%28by%20ref%29))
  ;[1 1 1 1 100] Defense
  (bind _asai_digimon_partner (Utilities|Casting|CastToAI_DigimonPartner OtherActor))
  (Variables|Default|SetPartner _asai_digimon_partner)
  (Variables|Default|SetIsInBaseTraining? true))

(event OnComponentEndOverlap(BoxCollision)
  (params (OverlappedComponent :type Primitive%20Component%20Object%20Reference) (OtherActor :type Actor%20Object%20Reference) (OtherComp :type Primitive%20Component%20Object%20Reference) (OtherBodyIndex :type Integer))
  ;[1 1 1 1 100] Defense
  (bind _asai_digimon_partner (Utilities|Casting|CastToAI_DigimonPartner OtherActor))
  (Variables|Default|SetPartner _asai_digimon_partner)
  (Variables|Default|SetIsInBaseTraining? false))

(event EventTick
  (params (DeltaSeconds :type Float%20%28single-precision%29))
  ;[1 1 1 1 100] Defense
  (if (and (Variables|Default|GetIsInBaseTraining?) (Variables|Default|GetStarted?))
    (Utilities|FlowControl|DoOnce false
      (:Completed
        (bind _location (Timeline|Punch%20Timeline PlayFromStart)
          (:Update
            (Transformation|SetRelativeLocation (Variables|Default|GetMovable) (Math|Vector|MakeVector _location 0.0 0.0) false false))
          (:Finished
            (if (Variables|Default|GetStarted?)
              (Timeline|Punch%20Timeline PlayFromStart)))
          (:Animation
            (CallFunction|SetAnimation (Variables|Default|GetPartner))))))))

(event EventTrainingStop
  ;[1 1 1 1 100] Defense
  (Variables|Default|SetIsInBaseTraining? false)
  (Variables|Default|SetStarted? false)
  (Actor|Tick|SetActorTickEnabled false)
  (Utilities|FlowControl|DoOnce false) ; enters at Reset
)

(event EventTrainingStart
  ;[1 1 1 1 100] Defense
  (Utilities|FlowControl|Sequence
    (:then_0
      (Actor|Tick|SetActorTickEnabled true)
      (Variables|Default|SetStarted? true)
      (Utilities|IsValid (Variables|Default|GetPartner)
        (:Is%20Valid
          (Default|AILocation (Variables|Default|GetPartner) (Transformation|GetWorldLocation (Variables|Default|GetBillboard)) :!label _label)
          (Default|AIBehaviourNormal (Variables|Default|GetPartner) "NewEnumerator8"))
        (:Is%20Not%20Valid
          (bind _outactors (Actor|GetAllActorsOfClass "/Game/AI/Pawn_Partner/AI_DigimonPartner.AI_DigimonPartner_C"))
          (for _array_element _outactors
            (Utilities|IsValid _array_element
              (:Is%20Valid
                (Variables|Default|SetPartner _array_element)
                (goto _label)))))))
    (:then_1
      (Game|Player|SetViewTargetwithBlend (Game|GetPlayerController 0) (Components|GetOwner (Variables|Default|GetTrainingCamera)) 0.4 "VTBlend_EaseInOut" 1.0 false))))

(fn ConstructionScript
  (bind _returnvalue (Utilities|GetDataTableRow "/Game/Game/DataTables/Training/DataTable_Training_Info.DataTable_Training_Info" "Beetleland_Offense")
    (:then
      (Variables|Default|SetBaseTraining_Info _returnvalue)
      (|CallParentFunction))))