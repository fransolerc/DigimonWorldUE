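; Procedural wall Blueprint that builds stacked rings of instanced meshes with a digits material, apparently for the MtInfinity environment.
; The construction script loops over floors and elements, placing instances evenly by angle at a set radius and floor height, leaving every fifth slot empty.
; Each instance is rolled upright, yawed tangent to the ring and uniformly scaled by a clamped size.
; The angle step uses integer division of 360 by the element count.
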(fn ConstructionScript
  (bind _size (Variables|Default|GetSize))
  (bind _elements (Variables|Default|GetElements))
  (bind _returnvalue (/ 360 _elements))
  (bind _returnvalue_2 (Math|Integer|Clamp(Integer) _size 1 8))
  (bind _returnvalue_3 (Math|Conversions|ToFloat(Integer) _returnvalue_2))
  (for _index (range 1 (Variables|Default|GetFloors))
    (for _index_2 (range 1 (Variables|Default|GetElements))
      (LocalVariables|SetArrayElement _index_2)
      ;[1 1 1 1 100] Spawn Item
      (if (> (Math|Integer|%(Integer) (LocalVariables|GetArrayElement) 5) 0)
        (Rendering|Material|SetMaterial (Variables|Default|GetInstancedStaticMesh) 0 "/Game/Material/Neon/MtInfinity/Materials/Material_MtInfinity_Digits_Inst.Material_MtInfinity_Digits_Inst")
        (Components|StaticMesh|SetStaticMesh (Variables|Default|GetInstancedStaticMesh) (Variables|Default|GetStaticMesh))
        (Components|InstancedStaticMesh|AddInstance (Variables|Default|GetInstancedStaticMesh) (Math|Transform|MakeTransform (Math|Vector|MakeVector (.X (Math|Vector|BreakVector (* (Math|Vector|GetForwardVector (Math|Rotator|MakeRotator 0.0 0.0 (Math|Conversions|ToFloat(Integer) (* (LocalVariables|GetArrayElement) _returnvalue)))) (Variables|Default|GetRadius)))) (.Y (Math|Vector|BreakVector (* (Math|Vector|GetForwardVector (Math|Rotator|MakeRotator 0.0 0.0 (Math|Conversions|ToFloat(Integer) (* (LocalVariables|GetArrayElement) _returnvalue)))) (Variables|Default|GetRadius)))) (* _index (Variables|Default|GetHeightBetweenFloors))) (Math|Rotator|MakeRotator 9e+01 0.0 (+ (Math|Conversions|ToFloat(Integer) (* (LocalVariables|GetArrayElement) _returnvalue)) 9e+01)) (Math|Vector|MakeVector _returnvalue_3 _returnvalue_3 _returnvalue_3)))))))