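; Procedural Mt Infinity floor builder that lays out cubes and planes from a DataTable at construction time.
; The construction script passes each table row to SpawnMesh, whose clamped Instance index picks the mesh, scale and material.
; Grid coordinates are multiplied by the scaled mesh bounds to position each piece.
; Pieces become instances in per-type Instanced Static Mesh components: circuit variants, wireframe, red, green and floor plane.
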(fn ConstructionScript
  (bind _datatable (Variables|Default|GetDataTable))
  (Utilities|IsValid _datatable
    (:Is%20Valid
      (bind _outrownames (DataTable|GetDataTableRowNames _datatable))
      (for _array_element _outrownames
        (bind _returnvalue (Utilities|GetDataTableRow _datatable _array_element)
          (:then
            (CallFunction|SpawnMesh _returnvalue)))))))

(fn SpawnMesh
  (params (MtInfinity_Floor_Struct :type Struct%20Mt%20Infinity%20Floor%20Structure%20%28by%20ref%29))
  (bind _instancedstaticmesh_plane (Variables|Default|GetInstancedStaticMesh_Plane))
  (bind _instancedstaticmesh_wireframe (Variables|Default|GetInstancedStaticMesh_Wireframe))
  (bind _cube_normal (LocalVariables|GetCube_Normal))
  (bind _cube_green (LocalVariables|GetCube_Green))
  (bind _instancedstaticmesh_red (Variables|Default|GetInstancedStaticMesh_Red))
  (bind _instancedstaticmesh_0 (Variables|Default|GetInstancedStaticMesh_0))
  (bind _cube_green_2 (LocalVariables|GetCube_Green))
  (bind _instancedstaticmesh_1 (Variables|Default|GetInstancedStaticMesh_1))
  (bind _instancedstaticmesh_2 (Variables|Default|GetInstancedStaticMesh_2))
  (bind _instancedstaticmesh_3 (Variables|Default|GetInstancedStaticMesh_3))
  (bind _instancedstaticmesh_4 (Variables|Default|GetInstancedStaticMesh_4))
  (bind _instancedstaticmesh_5 (Variables|Default|GetInstancedStaticMesh_5))
  (bind _instancedstaticmesh_6 (Variables|Default|GetInstancedStaticMesh_6))
  (bind _instancedstaticmesh_green (Variables|Default|GetInstancedStaticMesh_Green))
  (bind _instancedstaticmesh_7 (Variables|Default|GetInstancedStaticMesh_7))
  (bind _cube_normal_2 (LocalVariables|GetCube_Normal))
  (LocalVariables|SetStructLocal MtInfinity_Floor_Struct)
  (LocalVariables|SetInstanceIndex (Math|Integer|Clamp(Integer) (Utilities|Struct|BreakStruct_MtInfinity_Floor (LocalVariables|GetStructLocal)) 0 12))
  (LocalVariables|SetTransform (Math|Transform|MakeTransform (Math|Vector|MakeVector (* (.X (Utilities|Struct|BreakStruct_MtInfinity_Floor (LocalVariables|GetStructLocal))) (* (* (Utilities|Select :Index (LocalVariables|GetInstanceIndex) :Option%200 8 :Option%201 8 :Option%202 8 :Option%203 8 :Option%204 8 :Option%205 8 :Option%206 8 :Option%207 8 :Option%208 8 :Option%209 8 :Option%2010 8 :Option%2011 8 :Option%2012 4) 2) (.X (Math|Vector|BreakVector (.BoxExtent (Math|BoxSphereBounds|BreakBoxSphereBounds (StaticMesh|GetBounds (Utilities|Select :Index (LocalVariables|GetInstanceIndex) :Option%200 _cube_normal :Option%201 _cube_normal :Option%202 _cube_normal :Option%203 _cube_normal :Option%204 _cube_normal :Option%205 _cube_normal :Option%206 _cube_normal :Option%207 _cube_normal :Option%208 (LocalVariables|GetCube_Wireframe) :Option%209 (LocalVariables|GetCube_Red) :Option%2010 _cube_green :Option%2011 _cube_green :Option%2012 (LocalVariables|GetPlane))))))))) (* (.Y (Utilities|Struct|BreakStruct_MtInfinity_Floor (LocalVariables|GetStructLocal))) (* (* (Utilities|Select :Index (LocalVariables|GetInstanceIndex) :Option%200 8 :Option%201 8 :Option%202 8 :Option%203 8 :Option%204 8 :Option%205 8 :Option%206 8 :Option%207 8 :Option%208 8 :Option%209 8 :Option%2010 8 :Option%2011 8 :Option%2012 4) 2) (.Y (Math|Vector|BreakVector (.BoxExtent (Math|BoxSphereBounds|BreakBoxSphereBounds (StaticMesh|GetBounds (Utilities|Select :Index (LocalVariables|GetInstanceIndex) :Option%200 _cube_normal :Option%201 _cube_normal :Option%202 _cube_normal :Option%203 _cube_normal :Option%204 _cube_normal :Option%205 _cube_normal :Option%206 _cube_normal :Option%207 _cube_normal :Option%208 (LocalVariables|GetCube_Wireframe) :Option%209 (LocalVariables|GetCube_Red) :Option%2010 _cube_green :Option%2011 _cube_green :Option%2012 (LocalVariables|GetPlane))))))))) (* (.Z (Utilities|Struct|BreakStruct_MtInfinity_Floor (LocalVariables|GetStructLocal))) (* (* (Utilities|Select :Index (LocalVariables|GetInstanceIndex) :Option%200 8 :Option%201 8 :Option%202 8 :Option%203 8 :Option%204 8 :Option%205 8 :Option%206 8 :Option%207 8 :Option%208 8 :Option%209 8 :Option%2010 8 :Option%2011 8 :Option%2012 4) 2) (.Z (Math|Vector|BreakVector (.BoxExtent (Math|BoxSphereBounds|BreakBoxSphereBounds (StaticMesh|GetBounds (Utilities|Select :Index (LocalVariables|GetInstanceIndex) :Option%200 _cube_normal :Option%201 _cube_normal :Option%202 _cube_normal :Option%203 _cube_normal :Option%204 _cube_normal :Option%205 _cube_normal :Option%206 _cube_normal :Option%207 _cube_normal :Option%208 (LocalVariables|GetCube_Wireframe) :Option%209 (LocalVariables|GetCube_Red) :Option%2010 _cube_green :Option%2011 _cube_green :Option%2012 (LocalVariables|GetPlane)))))))))) "0, 0, 0" (Math|Vector|MakeVector (Math|Conversions|ToFloat(Integer) (Utilities|Select :Index (LocalVariables|GetInstanceIndex) :Option%200 8 :Option%201 8 :Option%202 8 :Option%203 8 :Option%204 8 :Option%205 8 :Option%206 8 :Option%207 8 :Option%208 8 :Option%209 8 :Option%2010 8 :Option%2011 8 :Option%2012 4)) (Math|Conversions|ToFloat(Integer) (Utilities|Select :Index (LocalVariables|GetInstanceIndex) :Option%200 8 :Option%201 8 :Option%202 8 :Option%203 8 :Option%204 8 :Option%205 8 :Option%206 8 :Option%207 8 :Option%208 8 :Option%209 8 :Option%2010 8 :Option%2011 8 :Option%2012 4)) (Math|Conversions|ToFloat(Integer) (Utilities|Select :Index (LocalVariables|GetInstanceIndex) :Option%200 8 :Option%201 8 :Option%202 8 :Option%203 8 :Option%204 8 :Option%205 8 :Option%206 8 :Option%207 8 :Option%208 8 :Option%209 8 :Option%2010 8 :Option%2011 8 :Option%2012 4)))))
  (switch int (LocalVariables|GetInstanceIndex)
    (:0
      (Components|StaticMesh|SetStaticMesh _instancedstaticmesh_0 _cube_normal_2)
      (Components|InstancedStaticMesh|AddInstance _instancedstaticmesh_0 (LocalVariables|GetTransform))
      (Rendering|Material|SetMaterial _instancedstaticmesh_0 0 "/Game/Material/Neon/MtInfinity/Materials/Material_MtInfinity_Circuit_Inst1.Material_MtInfinity_Circuit_Inst1"))
    (:1
      (Components|StaticMesh|SetStaticMesh _instancedstaticmesh_1 _cube_normal_2)
      (Components|InstancedStaticMesh|AddInstance _instancedstaticmesh_1 (LocalVariables|GetTransform))
      (Rendering|Material|SetMaterial _instancedstaticmesh_1 0 "/Game/Material/Neon/MtInfinity/Materials/Material_MtInfinity_Circuit_Inst2.Material_MtInfinity_Circuit_Inst2"))
    (:2
      (Components|StaticMesh|SetStaticMesh _instancedstaticmesh_2 _cube_normal_2)
      (Components|InstancedStaticMesh|AddInstance _instancedstaticmesh_2 (LocalVariables|GetTransform))
      (Rendering|Material|SetMaterial _instancedstaticmesh_2 0 "/Game/Material/Neon/MtInfinity/Materials/Material_MtInfinity_Circuit_Inst3.Material_MtInfinity_Circuit_Inst3"))
    (:3
      (Components|StaticMesh|SetStaticMesh _instancedstaticmesh_3 _cube_normal_2)
      (Components|InstancedStaticMesh|AddInstance _instancedstaticmesh_3 (LocalVariables|GetTransform))
      (Rendering|Material|SetMaterial _instancedstaticmesh_3 0 "/Game/Material/Neon/MtInfinity/Materials/Material_MtInfinity_Circuit_Inst4.Material_MtInfinity_Circuit_Inst4"))
    (:4
      (Components|StaticMesh|SetStaticMesh _instancedstaticmesh_4 _cube_normal_2)
      (Components|InstancedStaticMesh|AddInstance _instancedstaticmesh_4 (LocalVariables|GetTransform))
      (Rendering|Material|SetMaterial _instancedstaticmesh_4 0 "/Game/Material/Neon/MtInfinity/Materials/Material_MtInfinity_Circuit_Inst5.Material_MtInfinity_Circuit_Inst5"))
    (:5
      (Components|StaticMesh|SetStaticMesh _instancedstaticmesh_5 _cube_normal_2)
      (Components|InstancedStaticMesh|AddInstance _instancedstaticmesh_5 (LocalVariables|GetTransform))
      (Rendering|Material|SetMaterial _instancedstaticmesh_5 0 "/Game/Material/Neon/MtInfinity/Materials/Material_MtInfinity_Circuit_Inst6.Material_MtInfinity_Circuit_Inst6"))
    (:6
      (Components|StaticMesh|SetStaticMesh _instancedstaticmesh_6 _cube_normal_2)
      (Components|InstancedStaticMesh|AddInstance _instancedstaticmesh_6 (LocalVariables|GetTransform))
      (Rendering|Material|SetMaterial _instancedstaticmesh_6 0 "/Game/Material/Neon/MtInfinity/Materials/Material_MtInfinity_Circuit_Inst7.Material_MtInfinity_Circuit_Inst7"))
    (:7
      (Components|StaticMesh|SetStaticMesh _instancedstaticmesh_7 _cube_normal_2)
      (Components|InstancedStaticMesh|AddInstance _instancedstaticmesh_7 (LocalVariables|GetTransform))
      (Rendering|Material|SetMaterial _instancedstaticmesh_7 0 "/Game/Material/Neon/MtInfinity/Materials/Material_MtInfinity_Circuit_Inst8.Material_MtInfinity_Circuit_Inst8"))
    (:8
      (Components|StaticMesh|SetStaticMesh _instancedstaticmesh_wireframe (LocalVariables|GetCube_Wireframe))
      (Components|InstancedStaticMesh|AddInstance _instancedstaticmesh_wireframe (LocalVariables|GetTransform))
      (Rendering|Material|SetMaterial _instancedstaticmesh_wireframe 0 "/Game/Material/Neon/MtInfinity/Materials/Material_MtInfinity_GreenWireframe_Inst.Material_MtInfinity_GreenWireframe_Inst"))
    (:9
      (Components|StaticMesh|SetStaticMesh _instancedstaticmesh_red (LocalVariables|GetCube_Red))
      (Components|InstancedStaticMesh|AddInstance _instancedstaticmesh_red (LocalVariables|GetTransform))
      (Rendering|Material|SetMaterial _instancedstaticmesh_red 0 "/Game/Material/Neon/MtInfinity/Materials/Material_MtInfinity_Circuit.Material_MtInfinity_Circuit")
      (Rendering|Material|SetMaterial _instancedstaticmesh_red 1 "/Game/Material/Neon/MtInfinity/Materials/Material_MtInfinity_Circuit1.Material_MtInfinity_Circuit1"))
    (:10
      (Components|StaticMesh|SetStaticMesh _instancedstaticmesh_green _cube_green_2)
      (Components|InstancedStaticMesh|AddInstance _instancedstaticmesh_green (LocalVariables|GetTransform))
      (Rendering|Material|SetMaterial _instancedstaticmesh_green 0 "/Game/Material/Neon/SimpleGlow/Material_Glow_Inst3.Material_Glow_Inst3"))
    (:11
      (Components|StaticMesh|SetStaticMesh _instancedstaticmesh_green _cube_green_2)
      (Components|InstancedStaticMesh|AddInstance _instancedstaticmesh_green (LocalVariables|GetTransform))
      (Rendering|Material|SetMaterial _instancedstaticmesh_green 0 "/Game/Material/Neon/SimpleGlow/Material_Glow_Inst3.Material_Glow_Inst3"))
    (:12
      (Components|StaticMesh|SetStaticMesh _instancedstaticmesh_plane (LocalVariables|GetPlane))
      (Components|InstancedStaticMesh|AddInstance _instancedstaticmesh_plane (LocalVariables|GetTransform))
      (Rendering|Material|SetMaterial _instancedstaticmesh_plane 0 "/Game/Material/Neon/MtInfinity/Materials/Material_MtInfinity_Floor_Inst.Material_MtInfinity_Floor_Inst"))))