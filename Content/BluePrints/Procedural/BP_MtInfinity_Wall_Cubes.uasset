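; BP_MtInfinity_Wall_Cubes procedurally builds a broken wall or cluster of cubes from one instanced static mesh in the Construction Script.
; Each cell of the Rows by Columns grid has a random chance to call SpawnStaticMeshFunction.
; That function adds a four-instance vertical stack starting at a random level below Height.
; Spacing follows the mesh bounds times a clamped uniform Size, so instances sit flush on the grid.
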(fn ConstructionScript
  (for _index (range 0 (- (Variables|Default|GetRows) 1))
    (for _index_2 (range 0 (- (Variables|Default|GetColumns) 1))
      (if (Math|Random|RandomBool)
        (CallFunction|SpawnStaticMeshFunction _index _index_2)))))

(fn SpawnStaticMeshFunction
  (params (Row%20Index :type Integer) (Column%20Index :type Integer))
  (bind _size (Variables|Default|GetSize))
  (bind _staticmesh (Variables|Default|GetStaticMesh))
  (bind _returnvalue (Math|Integer|Clamp(Integer) _size 1 8))
  (bind _returnvalue_2 (StaticMesh|GetBounds _staticmesh))
  (bind _boxextent (Math|BoxSphereBounds|BreakBoxSphereBounds _returnvalue_2))
  (bind _returnvalue_3 (Math|Conversions|ToFloat(Integer) _returnvalue))
  (bind _returnvalue_4 (* _returnvalue 2))
  (bind (_x _y _z) (Math|Vector|BreakVector _boxextent))
  ;[1 1 1 1 100] Height
  (bind _output_get (LocalVariables|SetRand1 (Math|Random|RandomIntegerinRange 0 (- (Variables|Default|GetHeight) 1))))
  (LocalVariables|SetRand2 (+ _output_get 3))
  (for _index (range (LocalVariables|GetRand1) (LocalVariables|GetRand2))
    (Components|StaticMesh|SetStaticMesh (Variables|Default|GetInstancedStaticMesh) (Variables|Default|GetStaticMesh))
    (Components|InstancedStaticMesh|AddInstance (Variables|Default|GetInstancedStaticMesh) (Math|Transform|MakeTransform (Math|Vector|MakeVector (* Row%20Index (* _returnvalue_4 _x)) (* Column%20Index (* _returnvalue_4 _y)) (* _index (* _returnvalue_4 _z))) "0, 0, 0" (Math|Vector|MakeVector _returnvalue_3 _returnvalue_3 _returnvalue_3)))
    (Rendering|Material|SetMaterial (Variables|Default|GetInstancedStaticMesh) 0 (Variables|Default|GetMaterial))))