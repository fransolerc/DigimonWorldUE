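; Procedural bridge whose construction script builds a span from a configurable element count, uniform scale and material.
; Two instanced mesh components repeat Bridge and Bridge2 along local X, spaced by Bridge's bounds, up to 19 segments.
; Both enable collision, but the Bridge2 layer is hidden in game.
; Two static end pieces share the scale and material, with one moved to the span's end using the unclamped count.
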(fn ConstructionScript
  (bind _scale (Variables|Bridge|GetScale))
  (bind _instancedstaticmesh (Variables|Default|GetInstancedStaticMesh))
  (bind _scale_2 (Variables|Bridge|GetScale))
  (Rendering|Material|SetMaterial (Variables|Default|GetStaticMesh) 0 (Variables|Bridge|GetMaterial))
  (Transformation|SetRelativeScale3D (Variables|Default|GetStaticMesh) (Math|Vector|MakeVector _scale _scale _scale))
  (Transformation|SetRelativeLocation (Variables|Default|GetStaticMesh1) (Math|Vector|MakeVector (* (* (Variables|Bridge|GetElements) (.X (Math|Vector|BreakVector (.BoxExtent (Math|BoxSphereBounds|BreakBoxSphereBounds (StaticMesh|GetBounds (Variables|Bridge|GetBridge))))))) 2.0 (Variables|Bridge|GetScale)) 0.0 0.0) false true)
  (for _index (range 0 (- (Math|Integer|Clamp(Integer) (Variables|Bridge|GetElements) 0 19) 1))
    (Components|StaticMesh|SetStaticMesh (Variables|Default|GetInstancedStaticMesh) (Variables|Bridge|GetBridge))
    (Components|StaticMesh|SetStaticMesh (Variables|Default|GetInstancedStaticMesh1) (Variables|Bridge|GetBridge2))
    (Components|InstancedStaticMesh|AddInstance _instancedstaticmesh (Math|Transform|MakeTransform (Math|Vector|MakeVector (* (* _index (.X (Math|Vector|BreakVector (.BoxExtent (Math|BoxSphereBounds|BreakBoxSphereBounds (StaticMesh|GetBounds (Variables|Bridge|GetBridge))))))) 2.0 (Variables|Bridge|GetScale)) 0.0 0.0) "0, 0, 0" (Math|Vector|MakeVector _scale_2 _scale_2 _scale_2)))
    (Components|InstancedStaticMesh|AddInstance (Variables|Default|GetInstancedStaticMesh1) (Math|Transform|MakeTransform (Math|Vector|MakeVector (* (* _index (.X (Math|Vector|BreakVector (.BoxExtent (Math|BoxSphereBounds|BreakBoxSphereBounds (StaticMesh|GetBounds (Variables|Bridge|GetBridge))))))) 2.0 (Variables|Bridge|GetScale)) 0.0 0.0) "0, 0, 0" (Math|Vector|MakeVector _scale_2 _scale_2 _scale_2)))
    (Collision|SetCollisionEnabled _instancedstaticmesh "QueryAndPhysics")
    (Rendering|Material|SetMaterial _instancedstaticmesh 0 (Variables|Bridge|GetMaterial))
    (Development|SetHiddeninGame (Variables|Default|GetInstancedStaticMesh1) true true)))