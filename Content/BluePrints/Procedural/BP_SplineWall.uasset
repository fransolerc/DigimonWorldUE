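; BP_SplineWall is a procedural invisible wall that follows a spline to block everything except the Camera channel.
; The construction script divides the spline into fixed-length segments and adds a spline mesh component using the plane mesh for each.
; Each segment takes its endpoints from the spline, with tangents clamped to the segment length so consecutive pieces join along the curve.
; The meshes are hidden in game but keep query and physics collision.
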(fn ConstructionScript
  (bind _spline (Variables|Default|GetSpline))
  (bind _length (Variables|Default|GetLength))
  (bind _length_2 (Variables|Default|GetLength))
  (for _index (range 0 (Math|Float|Truncate (/ (Spline|GetSplineLength (Variables|Default|GetSpline)) (Variables|Default|GetLength))))
    (LocalVariables|SetIndexLocal _index)
    (bind _returnvalue (AddComponent|AddSplineMeshComponent false))
    (SplineMesh|SetForwardAxis _returnvalue "X" true)
    (SplineMesh|SetStartandEnd _returnvalue (Spline|GetLocationatDistanceAlongSpline _spline (* (LocalVariables|GetIndexLocal) _length) "Local") (Math|Vector|ClampVectorSize (Spline|GetTangentatDistanceAlongSpline _spline (* (LocalVariables|GetIndexLocal) _length) "Local") _length_2 _length_2) (Spline|GetLocationatDistanceAlongSpline _spline (* (+ (LocalVariables|GetIndexLocal) 1) _length) "Local") (Math|Vector|ClampVectorSize (Spline|GetTangentatDistanceAlongSpline _spline (* (+ (LocalVariables|GetIndexLocal) 1) _length) "Local") _length_2 _length_2) true :!class /Script/Engine.SplineMeshComponent)
    (Components|StaticMesh|SetStaticMesh _returnvalue "/Engine/BasicShapes/Plane.Plane")
    (Collision|SetCollisionEnabled _returnvalue "QueryAndPhysics")
    (Collision|SetCollisionResponsetoAllChannels _returnvalue "ECR_Block")
    (Collision|SetCollisionResponsetoChannel _returnvalue "ECC_Camera" "ECR_Ignore")
    (Development|SetHiddeninGame _returnvalue true true)))