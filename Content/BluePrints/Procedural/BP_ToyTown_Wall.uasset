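; Procedural toy town wall that builds a straight row of wall segments from a single mesh in the Construction Script.
; Each segment is randomly assigned to one of four instanced static mesh components, each with its own pairing of plastic materials for color variety.
; Segments are spaced along local X by the mesh's bounds width times Scale, with Elements setting the loop count and collision enabled for query and physics.
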(fn ConstructionScript
  (bind _instancedstaticmesh (Variables|Default|GetInstancedStaticMesh))
  (bind _instancedstaticmesh1 (Variables|Default|GetInstancedStaticMesh1))
  (bind _instancedstaticmesh2 (Variables|Default|GetInstancedStaticMesh2))
  (bind _instancedstaticmesh3 (Variables|Default|GetInstancedStaticMesh3))
  (bind _instancedstaticmesh3_2 (Variables|Default|GetInstancedStaticMesh3))
  (bind _instancedstaticmesh2_2 (Variables|Default|GetInstancedStaticMesh2))
  (bind _instancedstaticmesh1_2 (Variables|Default|GetInstancedStaticMesh1))
  (bind _instancedstaticmesh_2 (Variables|Default|GetInstancedStaticMesh))
  (bind _scale (Variables|Default|GetScale))
  (for _index (range 0 (Variables|Default|GetElements))
    (switch int (Math|Random|RandomIntegerinRange 0 3)
      (:0
        (Components|StaticMesh|SetStaticMesh _instancedstaticmesh_2 (Variables|Default|GetToyTownWall))
        (Rendering|Material|SetMaterial _instancedstaticmesh_2 0 "/Game/StaticMeshes/ToyTown/Material_ToyTown_Plastic_Inst3.Material_ToyTown_Plastic_Inst3")
        (Rendering|Material|SetMaterial _instancedstaticmesh_2 1 "/Game/StaticMeshes/ToyTown/Material_ToyTown_Plastic_Inst2.Material_ToyTown_Plastic_Inst2")
        (Components|InstancedStaticMesh|AddInstance _instancedstaticmesh (Math|Transform|MakeTransform (Math|Vector|MakeVector (* (* _index (.X (Math|Vector|BreakVector (.BoxExtent (Math|BoxSphereBounds|BreakBoxSphereBounds (StaticMesh|GetBounds (Variables|Default|GetToyTownWall))))))) 2.0 (Variables|Default|GetScale)) 0.0 0.0) "0, 0, 0" (Math|Vector|MakeVector _scale _scale _scale)))
        (Collision|SetCollisionEnabled _instancedstaticmesh "QueryAndPhysics"))
      (:1
        (Components|StaticMesh|SetStaticMesh _instancedstaticmesh1 (Variables|Default|GetToyTownWall))
        (Rendering|Material|SetMaterial _instancedstaticmesh1 0 "/Game/StaticMeshes/ToyTown/Material_ToyTown_Plastic_Inst4.Material_ToyTown_Plastic_Inst4")
        (Rendering|Material|SetMaterial _instancedstaticmesh1 1 "/Game/StaticMeshes/ToyTown/Material_ToyTown_Plastic_Inst3.Material_ToyTown_Plastic_Inst3")
        (Components|InstancedStaticMesh|AddInstance _instancedstaticmesh1_2 (Math|Transform|MakeTransform (Math|Vector|MakeVector (* (* _index (.X (Math|Vector|BreakVector (.BoxExtent (Math|BoxSphereBounds|BreakBoxSphereBounds (StaticMesh|GetBounds (Variables|Default|GetToyTownWall))))))) 2.0 (Variables|Default|GetScale)) 0.0 0.0) "0, 0, 0" (Math|Vector|MakeVector _scale _scale _scale)))
        (Collision|SetCollisionEnabled _instancedstaticmesh1_2 "QueryAndPhysics"))
      (:2
        (Components|StaticMesh|SetStaticMesh _instancedstaticmesh2 (Variables|Default|GetToyTownWall))
        (Rendering|Material|SetMaterial _instancedstaticmesh2 0 "/Game/StaticMeshes/ToyTown/Material_ToyTown_Plastic_Inst3.Material_ToyTown_Plastic_Inst3")
        (Rendering|Material|SetMaterial _instancedstaticmesh2 1 "/Game/StaticMeshes/ToyTown/Material_ToyTown_Plastic_Inst5.Material_ToyTown_Plastic_Inst5")
        (Components|InstancedStaticMesh|AddInstance _instancedstaticmesh2_2 (Math|Transform|MakeTransform (Math|Vector|MakeVector (* (* _index (.X (Math|Vector|BreakVector (.BoxExtent (Math|BoxSphereBounds|BreakBoxSphereBounds (StaticMesh|GetBounds (Variables|Default|GetToyTownWall))))))) 2.0 (Variables|Default|GetScale)) 0.0 0.0) "0, 0, 0" (Math|Vector|MakeVector _scale _scale _scale)))
        (Collision|SetCollisionEnabled _instancedstaticmesh2_2 "QueryAndPhysics"))
      (:3
        (Components|StaticMesh|SetStaticMesh _instancedstaticmesh3 (Variables|Default|GetToyTownWall))
        (Rendering|Material|SetMaterial _instancedstaticmesh3 0 "/Game/StaticMeshes/ToyTown/Material_ToyTown_Plastic_Inst5.Material_ToyTown_Plastic_Inst5")
        (Rendering|Material|SetMaterial _instancedstaticmesh3 1 "/Game/StaticMeshes/ToyTown/Material_ToyTown_Plastic_Inst4.Material_ToyTown_Plastic_Inst4")
        (Components|InstancedStaticMesh|AddInstance _instancedstaticmesh3_2 (Math|Transform|MakeTransform (Math|Vector|MakeVector (* (* _index (.X (Math|Vector|BreakVector (.BoxExtent (Math|BoxSphereBounds|BreakBoxSphereBounds (StaticMesh|GetBounds (Variables|Default|GetToyTownWall))))))) 2.0 (Variables|Default|GetScale)) 0.0 0.0) "0, 0, 0" (Math|Vector|MakeVector _scale _scale _scale)))
        (Collision|SetCollisionEnabled _instancedstaticmesh3_2 "QueryAndPhysics")))))