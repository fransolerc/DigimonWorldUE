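; Exterior of the File City clinic, whose point light switches with day and night once the Elecmon recruitment trigger is set.
; BeginPlay caches the DW1 game instance to read that trigger.
; LightingFade, labeled for the weather Blueprint, drives intensity through a timeline played forward for day and reversed for night.
; LightingonOff, labeled for level streaming, sets the light instantly off by day and on at night.
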(event EventBeginPlay
  ;[1 1 1 1 100] Begin Play
  (bind _asdw1_game_instance (Utilities|Casting|CastToDW1_GameInstance (Game|GetGameInstance)))
  (Variables|Default|SetAs%20DW1%20Game%20Instance _asdw1_game_instance))

(event EventLightingonOff
  (params (IsDay? :type Boolean))
  ;[1 1 1 1 100] On/Off - LEVEL STREAMING
  (if (Utilities|Struct|BreakStruct_Game_Triggers (Variables|/Game/Game/DW1_GameInstance.DW1_GameInstance_C|GetGame%20Triggers (Variables|Default|GetAs%20DW1%20Game%20Instance)))
    (Rendering|Components|Light|SetIntensity (Variables|Default|GetPointLight) (select IsDay? 0.0 1e+05))))

(event EventLightingFade
  (params (IsDay? :type Boolean))
  ;[1 1 1 1 100] FADE - BP WEATHER
  (if (Utilities|Struct|BreakStruct_Game_Triggers (Variables|/Game/Game/DW1_GameInstance.DW1_GameInstance_C|GetGame%20Triggers (Variables|Default|GetAs%20DW1%20Game%20Instance)))
    (if IsDay?
      (bind _lightintensity (Timeline|Línea%20de%20tiempo_0 PlayFromStart)
        (:Update
          (Rendering|Components|Light|SetIntensity (Variables|Default|GetPointLight) _lightintensity)))
      (else
        (Timeline|Línea%20de%20tiempo_0 ReverseFromEnd)))))

(fn ConstructionScript)