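; Exterior actor for Jijimon's house in File City, shown in base or upgraded form and serving as a trigger into its level.
; A one-time event stores the recruit and upgrade flags, then destroys the unused variant's components.
; With Elecmon recruited and the house upgraded, day/night events fade or switch the point light.
; Player overlap on either box sends the JijimonHouse streaming message to all BPI_LevelStreaming actors.
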(event OnComponentBeginOverlap(Box1)
  (params (OverlappedComponent :type Primitive%20Component%20Object%20Reference) (OtherActor :type Actor%20Object%20Reference) (OtherComp :type Primitive%20Component%20Object%20Reference) (OtherBodyIndex :type Integer) (bFromSweep :type Boolean) (SweepResult :type Hit%20Result%20Structure%20%28by%20ref%29))
  ;[1 1 1 1 100] JijimonHouse
  (Utilities|Casting|CastToJugador OtherActor)
  (bind _outactors (Actor|GetAllActorswithInterface "/Game/BluePrints/BPI/BPI_LevelStreaming.BPI_LevelStreaming_C"))
  (for _array_element _outactors
    (Class|BPILevelStreaming|LevelStreaming(Message) _array_element "JijimonHouse")))

(event OnComponentBeginOverlap(Box2)
  (params (OverlappedComponent :type Primitive%20Component%20Object%20Reference) (OtherActor :type Actor%20Object%20Reference) (OtherComp :type Primitive%20Component%20Object%20Reference) (OtherBodyIndex :type Integer) (bFromSweep :type Boolean) (SweepResult :type Hit%20Result%20Structure%20%28by%20ref%29))
  ;[1 1 1 1 100] JijimonHouse
  (Utilities|Casting|CastToJugador OtherActor)
  (bind _outactors (Actor|GetAllActorswithInterface "/Game/BluePrints/BPI/BPI_LevelStreaming.BPI_LevelStreaming_C"))
  (for _array_element _outactors
    (Class|BPILevelStreaming|LevelStreaming(Message) _array_element "JijimonHouse")))

(event Custom|JijimonHouseEvent
  (params (ElecmonRecruited? :type Boolean) (HouseUpgraded? :type Boolean))
  ;[1 1 1 1 100] Begin Play
  (Utilities|FlowControl|DoOnce false
    (:Completed
      (Variables|Default|SetElecmonRecruited? ElecmonRecruited?)
      (bind _output_get (Variables|Default|SetHouseUpgraded? HouseUpgraded?))
      (if _output_get
        (Components|DestroyComponent (Variables|Default|GetStaticMesh_JijimonHouse))
        (else
          (Components|DestroyComponent (Variables|Default|GetStaticMesh_JijimonHouse2)))))))

(event EventLightingFade
  (params (IsDay? :type Boolean))
  ;[1 1 1 1 100] FADE
  (if (and (Variables|Default|GetElecmonRecruited?) (Variables|Default|GetHouseUpgraded?))
    (if IsDay?
      (bind _lightintensity (Timeline|Línea%20de%20tiempo_0 PlayFromStart)
        (:Update
          (Rendering|Components|Light|SetIntensity (Variables|Default|GetPointLight) _lightintensity)))
      (else
        (Timeline|Línea%20de%20tiempo_0 ReverseFromEnd)))))

(event EventLightingonOff
  (params (IsDay? :type Boolean))
  (bind _pointlight (Variables|Default|GetPointLight))
  ;[1 1 1 1 100] On/Off
  (if (and (Variables|Default|GetElecmonRecruited?) (Variables|Default|GetHouseUpgraded?))
    (if (Variables|Default|GetElecmonRecruited?)
      (Rendering|Components|Light|SetIntensity _pointlight (select IsDay? 0.0 1e+05))
      (else
        (Rendering|Components|Light|SetIntensity _pointlight 0.0)))))

(fn ConstructionScript)