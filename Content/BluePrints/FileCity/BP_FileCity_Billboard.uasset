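; BP_FileCity_Billboard is the interactable billboard in File City, present only once Shellmon has been recruited.
; On BeginPlay it destroys itself unless that recruitment trigger is set in the game instance.
; A box overlap registers it as the player's interactible and toggles an interaction bubble.
; Interaction sends the Shellmon billboard dialogue table, with autoplay, to all BPI_Dialogue actors, then updates the player's bubble.
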(event OnComponentBeginOverlap(Box)
  (params (OverlappedComponent :type Primitive%20Component%20Object%20Reference) (OtherActor :type Actor%20Object%20Reference) (OtherComp :type Primitive%20Component%20Object%20Reference) (OtherBodyIndex :type Integer) (bFromSweep :type Boolean) (SweepResult :type Hit%20Result%20Structure%20%28by%20ref%29))
  ;[1 1 1 1 200] Overlap
  (bind _asjugador (Utilities|Casting|CastToJugador OtherActor))
  (Class|BPIInteract|InteractibleSet(Message) _asjugador self)
  (Default|InteractionBubble _asjugador "NewEnumerator0"))

(event OnComponentEndOverlap(Box)
  (params (OverlappedComponent :type Primitive%20Component%20Object%20Reference) (OtherActor :type Actor%20Object%20Reference) (OtherComp :type Primitive%20Component%20Object%20Reference) (OtherBodyIndex :type Integer))
  ;[1 1 1 1 200] Overlap
  (bind _asjugador (Utilities|Casting|CastToJugador OtherActor))
  (Class|BPIInteract|InteractibleUnset(Message) _asjugador)
  (Default|InteractionBubble _asjugador "NewEnumerator3"))

(event EventBeginPlay
  ;[1 1 1] BeginPlay
  (bind _asdw1_game_instance (Utilities|Casting|CastToDW1_GameInstance (Game|GetGameInstance))
    (:then
      (if (not (Utilities|Struct|BreakStruct_Game_Triggers (Variables|/Game/Game/DW1_GameInstance.DW1_GameInstance_C|GetGame%20Triggers _asdw1_game_instance)))
        (Actor|DestroyActor self)))
    (:CastFailed
      (Development|PrintString "GAME INSTANCE FAILED"))))

(event EventInteraction
  ;[1 1 1 1 200] Interaction
  (Utilities|FlowControl|Sequence
    (:then_0
      (bind _outactors (Actor|GetAllActorswithInterface "/Game/BluePrints/BPI/BPI_Dialogue.BPI_Dialogue_C"))
      (for _array_element _outactors
        (Class|BPIDialogue|DialogueSystemValuesSet(Message) _array_element self "/Game/Game/DataTables/Dialogue/FileCity/DataTable_Dialogue_FileCity_Shellmon_Billboard.DataTable_Dialogue_FileCity_Shellmon_Billboard" true)))
    (:then_1
      (bind _asjugador (Utilities|Casting|CastToJugador (Game|GetPlayerCharacter 0)))
      (Default|InteractionBubble _asjugador "NewEnumerator3"))))

(fn ConstructionScript)