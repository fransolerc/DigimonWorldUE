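; File City item shop exterior Blueprint whose two spotlights depend on whether Elecmon has been recruited.
; On BeginPlay it reads the recruitment trigger from the DW1 game instance.
; If the trigger is set, a timeline drives the pitch of both spotlights' relative rotation, with the second offset by 180 degrees.
; Otherwise, both spotlight components are destroyed.
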(event EventBeginPlay
  ;[1 1 1 1 100] BeginPlay
  (bind _asdw1_game_instance (Utilities|Casting|CastToDW1_GameInstance (Game|GetGameInstance)))
  (bind _output_get (Variables|Default|SetAs%20DW1%20Game%20Instance _asdw1_game_instance))
  (if (Utilities|Struct|BreakStruct_Game_Triggers (Variables|/Game/Game/DW1_GameInstance.DW1_GameInstance_C|GetGame%20Triggers _output_get))
    (bind _newtrack_0 (Timeline|Línea%20de%20tiempo_0 PlayFromStart)
      (:Update
        (Transformation|SetRelativeRotation (Variables|Default|GetSpotLight1) (Math|Rotator|MakeRotator 0.0 _newtrack_0 0.0) false false)
        (Transformation|SetRelativeRotation (Variables|Default|GetSpotLight2) (Math|Rotator|MakeRotator 0.0 (- _newtrack_0 1.8e+02) 0.0) false false)))
    (else
      (Components|DestroyComponent (Variables|Default|GetSpotLight1)))))

(fn ConstructionScript)