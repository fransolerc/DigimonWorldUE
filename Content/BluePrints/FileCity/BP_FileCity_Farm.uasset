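; BP_FileCity_Farm is the File City meat farm, whose visible crop reflects which Digimon have been recruited.
; On BeginPlay it reads the recruitment triggers from DW1_GameInstance and destroys the components not yet unlocked.
; With Vegiemon recruited everything stays; with only Palmon, the MeatPalmon pieces survive the cull; with neither, those are removed too.
; The pruning runs only at BeginPlay, with a debug print if the GameInstance cast fails.
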(event EventBeginPlay
  (bind _asdw1_game_instance (Utilities|Casting|CastToDW1_GameInstance (Game|GetGameInstance))
    (:then
      (Variables|Default|SetGameInstance _asdw1_game_instance)
      (if (not (.Trigger22-RecruitedVegiemon (Utilities|Struct|BreakStruct_Game_Triggers (Variables|/Game/Game/DW1_GameInstance.DW1_GameInstance_C|GetGame%20Triggers (Variables|Default|GetGameInstance)))))
        (if (.Trigger06-RecruitedPalmon (Utilities|Struct|BreakStruct_Game_Triggers (Variables|/Game/Game/DW1_GameInstance.DW1_GameInstance_C|GetGame%20Triggers (Variables|Default|GetGameInstance))))
          ;[1 1 1 1 100] TANEMON
          (Components|DestroyComponent (Variables|Default|GetStaticMesh))
          (else
            ;[1 1 1 1 100] PALMON
            (Components|DestroyComponent (Variables|Default|GetStaticMesh))))))
    (:CastFailed
      (Development|PrintString "GAME INSTANCE FAILED"))))

(fn ConstructionScript)