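; Exterior of the File City Item Bank, whose look follows recruitment triggers in the game instance.
; BeginPlay picks the level 2 mesh if Agumon is recruited, otherwise level 1, and removes the RectLight and glow unless Elecmon is also recruited.
; With both recruited, day/night events drive light intensity and material glow, either faded by a timeline (reversed for night) or switched instantly.
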(event EventBeginPlay
  (bind _staticmesh_itembank (Variables|Default|GetStaticMesh_ItemBank))
  ;[1 1 1 1 100] BEGIN PLAY
  (bind _asdw1_game_instance (Utilities|Casting|CastToDW1_GameInstance (Game|GetGameInstance)))
  (Variables|Default|SetAs%20DW1%20Game%20Instance _asdw1_game_instance)
  (if (.Trigger01-RecruitedAgumon (Utilities|Struct|BreakStruct_Game_Triggers (Variables|/Game/Game/DW1_GameInstance.DW1_GameInstance_C|GetGame%20Triggers (Variables|Default|GetAs%20DW1%20Game%20Instance))))
    (Components|StaticMesh|SetStaticMesh _staticmesh_itembank "/Game/StaticMeshes/FileCity/ItemKeeper/Mesh_ItemBank_Exterior_Level_02.Mesh_ItemBank_Exterior_Level_02")
    (if (not (.Trigger08-RecruitedElecmon (Utilities|Struct|BreakStruct_Game_Triggers (Variables|/Game/Game/DW1_GameInstance.DW1_GameInstance_C|GetGame%20Triggers (Variables|Default|GetAs%20DW1%20Game%20Instance)))))
      (Rendering|Material|SetScalarParameterValueonMaterials (Variables|Default|GetStaticMesh_ItemBank) "Glow" 0.0 :!label _label)
      (Components|DestroyComponent (Variables|Default|GetRectLight)))
    (else
      (Components|StaticMesh|SetStaticMesh _staticmesh_itembank "/Game/StaticMeshes/FileCity/ItemKeeper/Mesh_ItemBank_Exterior_Level_01.Mesh_ItemBank_Exterior_Level_01")
      (goto _label))))

(event EventLightingFade
  (params (IsDay? :type Boolean))
  (bind _as_dw1_game_instance (Variables|Default|GetAs%20DW1%20Game%20Instance))
  (bind _game_triggers (Variables|/Game/Game/DW1_GameInstance.DW1_GameInstance_C|GetGame%20Triggers _as_dw1_game_instance))
  (bind (_trigger01_recruitedagumon _trigger08_recruitedelecmon) (Utilities|Struct|BreakStruct_Game_Triggers _game_triggers))
  ;[1 1 1 1 100] FADE
  (if (and _trigger01_recruitedagumon _trigger08_recruitedelecmon)
    (if IsDay?
      (bind (_direction _lightintensity _glowmaterial) (Timeline|Línea%20de%20tiempo_0 PlayFromStart)
        (:Update
          (Rendering|Components|Light|SetIntensity (Variables|Default|GetRectLight) _lightintensity)
          (Rendering|Material|SetScalarParameterValueonMaterials (Variables|Default|GetStaticMesh_ItemBank) "Glow" _glowmaterial)))
      (else
        (Timeline|Línea%20de%20tiempo_0 ReverseFromEnd)))))

(event EventLightingonOff
  (params (IsDay? :type Boolean))
  (bind _as_dw1_game_instance (Variables|Default|GetAs%20DW1%20Game%20Instance))
  (bind _game_triggers (Variables|/Game/Game/DW1_GameInstance.DW1_GameInstance_C|GetGame%20Triggers _as_dw1_game_instance))
  (bind (_trigger01_recruitedagumon _trigger08_recruitedelecmon) (Utilities|Struct|BreakStruct_Game_Triggers _game_triggers))
  ;[1 1 1 1 100] On/Off
  (if (and _trigger01_recruitedagumon _trigger08_recruitedelecmon)
    (Rendering|Components|Light|SetIntensity (Variables|Default|GetRectLight) (select IsDay? 0.0 1e+05))
    (Rendering|Material|SetScalarParameterValueonMaterials (Variables|Default|GetStaticMesh_ItemBank) "Glow" (select IsDay? 1.0 5e+01))))

(fn ConstructionScript)