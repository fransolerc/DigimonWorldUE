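; Exterior actor for the File City restaurant, whose components and night lighting depend on Enabled and Elecmon flags.
; RestaurantEvent stores both flags and destroys unused components, leaving either the restaurant or its plug mesh, with smoke, distortion and point light only for Elecmon.
; When both flags are set, LightingFade plays or reverses a timeline for rect light intensity and material glow on weather changes, while LightingonOff snaps them for level streaming.
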(event Custom|RestaurantEvent
  (params (Elecmon? :type Boolean) (Enabled? :type Boolean))
  ;[1 1 1 1 100] Begin Play
  (Variables|Default|SetElecmon? Elecmon?)
  (bind _output_get (Variables|Default|SetEnabled? Enabled?))
  (if _output_get
    (Components|DestroyComponent (Variables|Default|GetStaticMesh_Plug))
    (if (not (Variables|Default|GetElecmon?))
      (Components|DestroyComponent (Variables|Default|GetParticleSystem_Distortion)))
    (else
      (Components|DestroyComponent (Variables|Default|GetStaticMesh_Restaurant)))))

(event EventLightingonOff
  (params (IsDay? :type Boolean))
  (bind _returnvalue (Utilities|Name|MakeLiteralName "Glow"))
  (bind _rectlight (Variables|Default|GetRectLight))
  (bind _staticmesh_restaurant (Variables|Default|GetStaticMesh_Restaurant))
  ;[1 1 1 1 100] On / Off - LEVEL STREAMING
  (if (and (Variables|Default|GetEnabled?) (Variables|Default|GetElecmon?))
    (if IsDay?
      (Rendering|Components|Light|SetIntensity _rectlight 0.0)
      (Rendering|Material|SetScalarParameterValueonMaterials _staticmesh_restaurant _returnvalue 1.0)
      (else
        (Rendering|Components|Light|SetIntensity _rectlight 1e+05)
        (Rendering|Material|SetScalarParameterValueonMaterials _staticmesh_restaurant _returnvalue 1e+01)))))

(event EventLightingFade
  (params (IsDay? :type Boolean))
  ;[1 1 1 1 100] FADE - BP WEATHER
  (if (and (Variables|Default|GetEnabled?) (Variables|Default|GetElecmon?))
    (if IsDay?
      (bind (_direction _lightintensity _glow) (Timeline|Línea%20de%20tiempo_0 PlayFromStart)
        (:Finished
          (Rendering|Components|Light|SetIntensity (Variables|Default|GetRectLight) _lightintensity)
          (Rendering|Material|SetScalarParameterValueonMaterials (Variables|Default|GetStaticMesh_Restaurant) "Glow" _glow)))
      (else
        (Timeline|Línea%20de%20tiempo_0 ReverseFromEnd)))))

(fn ConstructionScript)