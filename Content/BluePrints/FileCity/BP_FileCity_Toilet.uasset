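; BP_FileCity_Toilet is the File City toilet, with a trigger box and a spotlight.
; When the player (Jugador) enters or leaves the box, it sends a true or false toilet message to all actors implementing BPI_DigimonPartnerSystem.
; Day/night events, labelled for BP Weather, either fade the spotlight through a timeline or switch it instantly, off by day and on at night.
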(event OnComponentBeginOverlap(BoxCollision)
  (params (OverlappedComponent :type Primitive%20Component%20Object%20Reference) (OtherActor :type Actor%20Object%20Reference) (OtherComp :type Primitive%20Component%20Object%20Reference) (OtherBodyIndex :type Integer) (bFromSweep :type Boolean) (SweepResult :type Hit%20Result%20Structure%20%28by%20ref%29))
  ;[1 1 1 1 100] Toilet
  (Utilities|Casting|CastToJugador OtherActor)
  (bind _outactors (Actor|GetAllActorswithInterface "/Game/BluePrints/BPI/BPI_DigimonPartnerSystem.BPI_DigimonPartnerSystem_C"))
  (for _array_element _outactors
    (Class|BPIDigimonPartnerSystem|DigimonPartnerSystemToilet(Message) _array_element true)))

(event OnComponentEndOverlap(BoxCollision)
  (params (OverlappedComponent :type Primitive%20Component%20Object%20Reference) (OtherActor :type Actor%20Object%20Reference) (OtherComp :type Primitive%20Component%20Object%20Reference) (OtherBodyIndex :type Integer))
  ;[1 1 1 1 100] Toilet
  (Utilities|Casting|CastToJugador OtherActor)
  (bind _outactors (Actor|GetAllActorswithInterface "/Game/BluePrints/BPI/BPI_DigimonPartnerSystem.BPI_DigimonPartnerSystem_C"))
  (for _array_element _outactors
    (Class|BPIDigimonPartnerSystem|DigimonPartnerSystemToilet(Message) _array_element false)))

(event EventLightingonOff
  (params (IsDay? :type Boolean))
  ;[1 1 1 1 100] On/Off
  (Rendering|Components|Light|SetIntensity (Variables|Default|GetSpotLight) (select IsDay? 0.0 5e+04)))

(event EventLightingFade
  (params (IsDay? :type Boolean))
  ;[1 1 1 1 100] FADE - BP WEATHER
  (if IsDay?
    (bind _lightintensity (Timeline|LightIntensity PlayFromStart)
      (:Update
        (Rendering|Components|Light|SetIntensity (Variables|Default|GetSpotLight) _lightintensity)))
    (else
      (Timeline|LightIntensity ReverseFromEnd))))

(fn ConstructionScript)