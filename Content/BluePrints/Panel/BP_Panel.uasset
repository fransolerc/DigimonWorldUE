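; BP_Panel is a mesh panel that cycles through display materials and blinks its text and arrow.
; The construction script puts a dynamic instance of the panel material on slot 3 and sets its clamped Rotator parameter.
; On BeginPlay, if the material array is filled, a timeline's event tracks step through it, reapplying Rotator, and FlipFlops toggle text and arrow intensity on and off.
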(event EventBeginPlay
  (bind _returnvalue (Utilities|Name|MakeLiteralName "ArrowIntensity"))
  (bind _returnvalue_2 (Utilities|Name|MakeLiteralName "TextIntensity"))
  (bind _staticmesh (Variables|Default|GetStaticMesh))
  (bind _staticmesh_2 (Variables|Default|GetStaticMesh))
  ;[1 1 1 1 100] BeginPlay
  (if (> (Utilities|Array|Length (Variables|Panel|GetMaterial)) 0)
    (Timeline|Línea%20de%20tiempo_Panel PlayFromStart
      (:Change%20Text%2001
        ;[1 1 1 1 100] Change Material
        (Variables|Panel|SetCounter (select (> (+ (Variables|Panel|GetCounter) 1) (- (Utilities|Array|Length (Variables|Panel|GetMaterial)) 1)) 0 (+ (Variables|Panel|GetCounter) 1)))
        (Rendering|Material|SetMaterial (Variables|Default|GetStaticMesh) 3 (Utilities|Array|Get(acopy) (Variables|Panel|GetMaterial) (Variables|Panel|GetCounter)))
        (Rendering|Material|SetScalarParameterValueonMaterials (Variables|Default|GetStaticMesh) (Utilities|Name|MakeLiteralName "Rotator") (Variables|Panel|GetRotator)))
      (:Text%20On/Off
        ;[1 1 1 1 100] Text Intensity
        (bind _isa (Utilities|FlowControl|FlipFlop)
          (:A
            _)
          (:B
            _))
        (if _isa
          (Rendering|Material|SetScalarParameterValueonMaterials _staticmesh _returnvalue_2 1.0)
          (else
            (Rendering|Material|SetScalarParameterValueonMaterials _staticmesh _returnvalue_2 0.0))))
      (:Arrow%20On/Off
        ;[1 1 1 1 100] Arrow Intensity
        (bind _isa_2 (Utilities|FlowControl|FlipFlop)
          (:A
            _)
          (:B
            _))
        (if _isa_2
          (Rendering|Material|SetScalarParameterValueonMaterials _staticmesh_2 _returnvalue 1.0)
          (else
            (Rendering|Material|SetScalarParameterValueonMaterials _staticmesh_2 _returnvalue 0.0)))))))

(fn ConstructionScript
  (bind _returnvalue (Rendering|Material|CreateDynamicMaterialInstance (Variables|Default|GetStaticMesh) 3 "/Game/Material/Material_Panel.Material_Panel" "None" :!class /Script/Engine.PrimitiveComponent))
  (LocalVariables|SetMaterialLocal _returnvalue)
  (Rendering|Material|SetScalarParameterValue (LocalVariables|GetMaterialLocal) "Rotator" (Math|Float|Clamp(Float) (Variables|Panel|GetRotator)) :!class /Script/Engine.MaterialInstanceDynamic))