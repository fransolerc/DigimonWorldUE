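; Curling minigame manager where the player and a random-angle AI take turns sliding BP_CurlingDisk actors at a lit target.
; One input steps through spawn, timeline-driven power and push, with left/right aiming shown by a debug line.
; Zone overlaps tag disks and light decals; CurlingReset replays scoring disks one by one and totals points on Curling_HUD.
; The camera follows along a spline, and the game ends after five player throws, notifying BPI_Dialogue actors.
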(event OnComponentBeginOverlap(Sphere_Good_1)
  (params (OverlappedComponent :type Primitive%20Component%20Object%20Reference) (OtherActor :type Actor%20Object%20Reference) (OtherComp :type Primitive%20Component%20Object%20Reference) (OtherBodyIndex :type Integer) (bFromSweep :type Boolean) (SweepResult :type Hit%20Result%20Structure%20%28by%20ref%29))
  ;[0.8863 0.698 1 1 100] GOOD [0]
  (bind _asbp_curling_disk (Utilities|Casting|CastToBP_CurlingDisk OtherActor))
  (Variables|/Game/BluePrints/Curling/BP_CurlingDisk.BP_CurlingDisk_C|SetLight _asbp_curling_disk 0)
  (Variables|/Game/BluePrints/Curling/BP_CurlingDisk.BP_CurlingDisk_C|SetEnabled? _asbp_curling_disk true)
  (CallFunction|LightGood true))

(event OnComponentBeginOverlap(Sphere_Bad)
  (params (OverlappedComponent :type Primitive%20Component%20Object%20Reference) (OtherActor :type Actor%20Object%20Reference) (OtherComp :type Primitive%20Component%20Object%20Reference) (OtherBodyIndex :type Integer) (bFromSweep :type Boolean) (SweepResult :type Hit%20Result%20Structure%20%28by%20ref%29))
  ;[0.8863 0.698 1 1 100] BAD [1]
  (bind _asbp_curling_disk (Utilities|Casting|CastToBP_CurlingDisk OtherActor))
  (Variables|/Game/BluePrints/Curling/BP_CurlingDisk.BP_CurlingDisk_C|SetLight _asbp_curling_disk 1)
  (Variables|/Game/BluePrints/Curling/BP_CurlingDisk.BP_CurlingDisk_C|SetEnabled? _asbp_curling_disk true)
  (CallFunction|LightBad true))

(event OnComponentBeginOverlap(Sphere_Good_2)
  (params (OverlappedComponent :type Primitive%20Component%20Object%20Reference) (OtherActor :type Actor%20Object%20Reference) (OtherComp :type Primitive%20Component%20Object%20Reference) (OtherBodyIndex :type Integer) (bFromSweep :type Boolean) (SweepResult :type Hit%20Result%20Structure%20%28by%20ref%29))
  ;[0.8863 0.698 1 1 100] INNER [3]
  (bind _asbp_curling_disk (Utilities|Casting|CastToBP_CurlingDisk OtherActor))
  (Variables|/Game/BluePrints/Curling/BP_CurlingDisk.BP_CurlingDisk_C|SetLight _asbp_curling_disk 3)
  (Variables|/Game/BluePrints/Curling/BP_CurlingDisk.BP_CurlingDisk_C|SetEnabled? _asbp_curling_disk true)
  (CallFunction|LightInner true)
  (CallFunction|LightOuter false))

(event OnComponentBeginOverlap(Sphere_OuterCircle)
  (params (OverlappedComponent :type Primitive%20Component%20Object%20Reference) (OtherActor :type Actor%20Object%20Reference) (OtherComp :type Primitive%20Component%20Object%20Reference) (OtherBodyIndex :type Integer) (bFromSweep :type Boolean) (SweepResult :type Hit%20Result%20Structure%20%28by%20ref%29))
  ;[0.8863 0.698 1 1 100] OUTER [2]
  (bind _asbp_curling_disk (Utilities|Casting|CastToBP_CurlingDisk OtherActor))
  (Variables|/Game/BluePrints/Curling/BP_CurlingDisk.BP_CurlingDisk_C|SetLight _asbp_curling_disk 2)
  (Variables|/Game/BluePrints/Curling/BP_CurlingDisk.BP_CurlingDisk_C|SetEnabled? _asbp_curling_disk true)
  (CallFunction|LightOuter true))

(event OnComponentEndOverlap(Sphere_OuterCircle)
  (params (OverlappedComponent :type Primitive%20Component%20Object%20Reference) (OtherActor :type Actor%20Object%20Reference) (OtherComp :type Primitive%20Component%20Object%20Reference) (OtherBodyIndex :type Integer))
  ;[0.8863 0.698 1 1 100] OUTER [2]
  (bind _asbp_curling_disk (Utilities|Casting|CastToBP_CurlingDisk OtherActor))
  (Variables|/Game/BluePrints/Curling/BP_CurlingDisk.BP_CurlingDisk_C|SetLight _asbp_curling_disk 4)
  (Variables|/Game/BluePrints/Curling/BP_CurlingDisk.BP_CurlingDisk_C|SetEnabled? _asbp_curling_disk false)
  (CallFunction|LightOuter false))

(event OnComponentEndOverlap(Sphere_Good_2)
  (params (OverlappedComponent :type Primitive%20Component%20Object%20Reference) (OtherActor :type Actor%20Object%20Reference) (OtherComp :type Primitive%20Component%20Object%20Reference) (OtherBodyIndex :type Integer))
  ;[0.8863 0.698 1 1 100] INNER [3]
  (bind _asbp_curling_disk (Utilities|Casting|CastToBP_CurlingDisk OtherActor))
  (Variables|/Game/BluePrints/Curling/BP_CurlingDisk.BP_CurlingDisk_C|SetLight _asbp_curling_disk 4)
  (Variables|/Game/BluePrints/Curling/BP_CurlingDisk.BP_CurlingDisk_C|SetEnabled? _asbp_curling_disk false)
  (CallFunction|LightInner false)
  (CallFunction|LightOuter true))

(event OnComponentEndOverlap(Sphere_Good_1)
  (params (OverlappedComponent :type Primitive%20Component%20Object%20Reference) (OtherActor :type Actor%20Object%20Reference) (OtherComp :type Primitive%20Component%20Object%20Reference) (OtherBodyIndex :type Integer))
  ;[0.8863 0.698 1 1 100] GOOD [0]
  (bind _asbp_curling_disk (Utilities|Casting|CastToBP_CurlingDisk OtherActor))
  (Variables|/Game/BluePrints/Curling/BP_CurlingDisk.BP_CurlingDisk_C|SetLight _asbp_curling_disk 4)
  (Variables|/Game/BluePrints/Curling/BP_CurlingDisk.BP_CurlingDisk_C|SetEnabled? _asbp_curling_disk false)
  (CallFunction|LightGood false))

(event OnComponentEndOverlap(Sphere_Bad)
  (params (OverlappedComponent :type Primitive%20Component%20Object%20Reference) (OtherActor :type Actor%20Object%20Reference) (OtherComp :type Primitive%20Component%20Object%20Reference) (OtherBodyIndex :type Integer))
  ;[0.8863 0.698 1 1 100] BAD [1]
  (bind _asbp_curling_disk (Utilities|Casting|CastToBP_CurlingDisk OtherActor))
  (Variables|/Game/BluePrints/Curling/BP_CurlingDisk.BP_CurlingDisk_C|SetLight _asbp_curling_disk 4)
  (Variables|/Game/BluePrints/Curling/BP_CurlingDisk.BP_CurlingDisk_C|SetEnabled? _asbp_curling_disk false)
  (CallFunction|LightBad false))

(event OnComponentHit(CurlingCave2_Cube_001)
  (params (HitComponent :type Primitive%20Component%20Object%20Reference) (OtherActor :type Actor%20Object%20Reference) (OtherComp :type Primitive%20Component%20Object%20Reference) (NormalImpulse :type Vector :default "0, 0, 0") (Hit :type Hit%20Result%20Structure%20%28by%20ref%29))
  ;[1 1 1 1 100] SOUNDS
  (Utilities|Casting|CastToBP_CurlingDisk OtherActor)
  (Utilities|FlowControl|DoOnce false :!label _label
    (:Completed
      (Audio|PlaySound2D "/Game/Audio/SFX/Curling/curling4.curling4" 1.0 1.0 0.0 0 0)
      (Utilities|FlowControl|Delay 0.2)
      (goto _label Reset))))

(event Custom|FocusCameraDisk
  ;[0.1989 1 0.8295 1 100] CAMERA DISK
  (Utilities|IsValid (Variables|Disks|GetDisk)
    (:Is%20Valid
      (Game|Player|SetViewTargetwithBlend (Game|GetPlayerController 0) (Components|GetOwner (Variables|Default|GetCamera)) 0.0 "VTBlend_Linear" 0.0 false)
      (Timeline|Línea%20de%20tiempo_1 PlayFromStart
        (:Update
          (Variables|Camera|SetCurrentCameraLocation (Spline|FindLocationClosesttoWorldLocation (Variables|Default|GetSpline) (Transformation|GetActorLocation (Variables|Disks|GetDisk)) "World"))
          (Transformation|SetRelativeLocation (Variables|Default|GetCamera) (Variables|Camera|GetCurrentCameraLocation) false false))))))

(event EventCurlingReset
  (bind _returnvalue (Class|KismetSystemLibrary|MakeLiteralBool false))
  (bind _returnvalue_2 (Class|KismetSystemLibrary|MakeLiteralBool true))
  (bind _returnvalue_3 (Class|KismetSystemLibrary|MakeLiteralBool false))
  ;[1 1 1 1 100] RESET
  (Utilities|FlowControl|Sequence
    (:then_0
      ;[0.1989 1 0.8295 1 100] CAMERA DISK
      (Timeline|Línea%20de%20tiempo_1 Stop
        (:Update
          (Variables|Camera|SetCurrentCameraLocation (Spline|FindLocationClosesttoWorldLocation (Variables|Default|GetSpline) (Transformation|GetActorLocation (Variables|Disks|GetDisk)) "World"))
          (Transformation|SetRelativeLocation (Variables|Default|GetCamera) (Variables|Camera|GetCurrentCameraLocation) false false))))
    (:then_1
      (CallFunction|LightOuter false)
      (CallFunction|LightInner false)
      (CallFunction|LightGood false)
      (CallFunction|LightBad false)
      (Variables|Disks|SetDiskAnimationCounter 0)
      (bind _outactors (Actor|GetAllActorsOfClass "/Game/BluePrints/Curling/BP_CurlingDisk.BP_CurlingDisk_C"))
      (Variables|Disks|SetDisk_Array _outactors)
      (if (Utilities|Array|IsValidIndex (Variables|Disks|GetDisk_Array) (Variables|Disks|GetDiskAnimationCounter)) :!label _label
        (Variables|Disks|SetDisk (Utilities|Array|Get(acopy) (Variables|Disks|GetDisk_Array) (Variables|Disks|GetDiskAnimationCounter)))
        (Math|Integer|IncrementInt (Variables|Disks|GetDiskAnimationCounter)
          (:%20%20
            (if (and (Utilities|IsValid (Variables|Disks|GetDisk)) (Utilities|DoesObjectImplementInterface (Variables|Disks|GetDisk) "/Game/BluePrints/BPI/BPI_Curling.BPI_Curling_C"))
              (if (and (Math|Integer|InRange(Integer) (Variables|/Game/BluePrints/Curling/BP_CurlingDisk.BP_CurlingDisk_C|GetLight (Variables|Disks|GetDisk)) 0 3) (Variables|/Game/BluePrints/Curling/BP_CurlingDisk.BP_CurlingDisk_C|GetEnabled? (Variables|Disks|GetDisk)))
                (CallFunction|UpdateScore)
                (Variables|Camera|SetCurrentCameraLocation (Spline|FindLocationClosesttoWorldLocation (Variables|Default|GetSpline) (Transformation|GetActorLocation (Variables|Disks|GetDisk)) "World"))
                (Transformation|SetRelativeLocation (Variables|Default|GetCamera) (Variables|Camera|GetCurrentCameraLocation) false false)
                (Audio|PlaySound2D (Utilities|Select :Index (Variables|/Game/BluePrints/Curling/BP_CurlingDisk.BP_CurlingDisk_C|GetLight (Variables|Disks|GetDisk)) :Option%200 "/Game/Audio/SFX/Curling/curling6.curling6" :Option%201 "/Game/Audio/SFX/Curling/curling7.curling7" :Option%202 "/Game/Audio/SFX/Curling/curling6.curling6" :Option%203 "/Game/Audio/SFX/Curling/curling6.curling6") 1.0 1.0 0.0 0 0)
                (Timeline|Línea%20de%20tiempo_0 PlayFromStart
                  (:Finished
                    (goto _label))
                  (:Visibility%201
                    ;;[1 0.5943 0.2639 1 100] Animation
                    (Development|SetHiddeninGame (Variables|/Game/BluePrints/Curling/BP_CurlingDisk.BP_CurlingDisk_C|GetCurlingDisk (Variables|Disks|GetDisk)) (Class|KismetSystemLibrary|MakeLiteralBool false) false)
                    (switch int (Variables|/Game/BluePrints/Curling/BP_CurlingDisk.BP_CurlingDisk_C|GetLight (Variables|Disks|GetDisk))
                      (:0
                        (CallFunction|LightGood _returnvalue_2))
                      (:1
                        (CallFunction|LightBad _returnvalue_2))
                      (:2
                        (CallFunction|LightOuter _returnvalue_2))
                      (:3
                        (CallFunction|LightInner _returnvalue_2))))
                  (:Visibility%202
                    (Development|SetHiddeninGame (Variables|/Game/BluePrints/Curling/BP_CurlingDisk.BP_CurlingDisk_C|GetCurlingDisk (Variables|Disks|GetDisk)) (Class|KismetSystemLibrary|MakeLiteralBool true) false)
                    (switch int (Variables|/Game/BluePrints/Curling/BP_CurlingDisk.BP_CurlingDisk_C|GetLight (Variables|Disks|GetDisk))
                      (:0
                        (CallFunction|LightGood _returnvalue_3))
                      (:1
                        (CallFunction|LightBad _returnvalue_3))
                      (:2
                        (CallFunction|LightOuter _returnvalue_3))
                      (:3
                        (CallFunction|LightInner _returnvalue_3))))
                  (:Visibility%203
                    (Development|SetHiddeninGame (Variables|/Game/BluePrints/Curling/BP_CurlingDisk.BP_CurlingDisk_C|GetCurlingDisk (Variables|Disks|GetDisk)) _returnvalue false)
                    (switch int (Variables|/Game/BluePrints/Curling/BP_CurlingDisk.BP_CurlingDisk_C|GetLight (Variables|Disks|GetDisk))
                      (:0
                        (CallFunction|LightGood _returnvalue))
                      (:1
                        (CallFunction|LightBad _returnvalue))
                      (:2
                        (CallFunction|LightOuter _returnvalue))
                      (:3
                        (CallFunction|LightInner _returnvalue)))))
                (else
                  (goto _label)))
              (else
                (goto _label)))))
        (else
          (CallFunction|UpdateScoreTotal)
          (Variables|Disks|SetDiskAnimationCounter 0)
          (Variables|Disks|SetDisk 0)
          (Utilities|Array|Clear (Variables|Disks|GetDisk_Array))
          (if (Variables|Default|GetPlayerTurn?)
            ;[1 1 1 1 100] CAMERA TO PLAYER
            (bind _time (Timeline|Línea%20de%20tiempo_3 PlayFromStart)
              (:Update
                (Transformation|SetRelativeLocation (Variables|Default|GetCamera) (Math|Interpolation|VInterpTo (Variables|Camera|GetCurrentCameraLocation) (Spline|FindLocationClosesttoWorldLocation (Variables|Default|GetSpline) (Transformation|GetWorldLocation (Variables|Default|GetBillboard_Disk_Player)) "World") _time 1.0) false false))
              (:Finished
                (Input|EnableInput self (Game|GetPlayerController 0))))
            (else
              ;[1 1 1 1 100] CAMERA TO ENEMY
              (bind _time_2 (Timeline|Línea%20de%20tiempo_4 PlayFromStart)
                (:Update
                  (Transformation|SetRelativeLocation (Variables|Default|GetCamera) (Math|Interpolation|VInterpTo (Variables|Camera|GetCurrentCameraLocation) (Spline|FindLocationClosesttoWorldLocation (Variables|Default|GetSpline) (Transformation|GetWorldLocation (Variables|Default|GetBillboard_Disk_Enemy)) "World") _time_2 1.0) false false))
                (:Finished
                  (Utilities|FlowControl|Delay 1.0)
                  (Math|Integer|IncrementInt (Variables|Default|GetEnemySpawnCounter)
                    (:%20%20
                      (bind _returnvalue_4 (Game|SpawnActorfromClass "/Game/BluePrints/Curling/BP_CurlingDisk.BP_CurlingDisk_C" (Math|Transform|MakeTransform (Transformation|GetWorldLocation (Variables|Default|GetBillboard_Disk_Enemy)) "0, 0, 0" "0.050000,0.050000,0.050000") "AlwaysSpawn" 0 false (Math|Random|RandomIntegerinRange 0 3) 0))
                      (Variables|Disks|SetDisk _returnvalue_4)
                      (Class|BPICurling|CurlingPush(Message) (Variables|Disks|GetDisk) (Math|Random|RandomFloatinRange 3e+01 1.5e+02) 2e+03)
                      (Variables|Default|SetPlayerTurn? true)
                      (CallFunction|FocusCameraDisk))))))))))))

(event EventBeginPlay
  ;[0.3037 0.5483 1 1 100] BeginPlay
  (CallFunction|LightOuter false)
  (CallFunction|LightInner false)
  (CallFunction|LightGood false)
  (CallFunction|LightBad false))

(event EventGameEvent
  (params (Boolean :type Boolean))
  (bind _camera (Variables|Default|GetCamera))
  ;[1 0.3577 0.2879 1 100] GameEvent
  (Utilities|FlowControl|DoOnce false
    (:Completed
      (Utilities|FlowControl|Sequence
        (:then_0
          (Input|EnableInput self (Game|GetPlayerController 0)))
        (:then_1
          (bind _returnvalue (UserInterface|CreateWidget "/Game/UI/Curling_HUD.Curling_HUD_C"))
          (bind _output_get (Variables|Default|SetCurlingHUD _returnvalue))
          (UserInterface|Viewport|AddtoViewport _output_get 99))
        (:then_2
          (bind _output_get_2 (Variables|Camera|SetCurrentCameraLocation (Spline|FindLocationClosesttoWorldLocation (Variables|Default|GetSpline) (Transformation|GetWorldLocation (Variables|Default|GetBillboard_Disk_Player)) "World")))
          (Transformation|SetRelativeLocation _camera _output_get_2 false false)
          (Game|Player|SetViewTargetwithBlend (Game|GetPlayerController 0) (Components|GetOwner _camera) 0.0 "VTBlend_Linear" 0.0 false))))))

(event Input|ActionEvents|InputActionInteraction[Cross]
  (params (Key :type Key%20Structure :default "None"))
  (bind _billboard_disk_player (Variables|Default|GetBillboard_Disk_Player))
  (bind _playerscore (Variables|Default|GetPlayerScore))
  (bind _enemyscore (Variables|Default|GetEnemyScore))
  (bind _returnvalue (Transformation|GetWorldLocation _billboard_disk_player))
  ;[0.5383 1 0.4202 1 100] PLAYER TURN
  (:Pressed
    (bind _counter (Utilities|FlowControl|DoN 3 :!label _label)
      (:Exit
        (switch int _counter
          (:1
            (bind _result (Math|Integer|IncrementInt (Variables|Default|GetPlayerSpawnCounter))
              (:%20%20
                (if (< _result 6)
                  (Variables|Default|SetPlayerTurn? false)
                  (bind _returnvalue_2 (Game|SpawnActorfromClass "/Game/BluePrints/Curling/BP_CurlingDisk.BP_CurlingDisk_C" (Math|Transform|MakeTransform (Transformation|GetWorldLocation (Variables|Default|GetBillboard_Disk_Player)) "0, 0, 0" "0.050000,0.050000,0.050000") "AlwaysSpawn" self true (Math|Random|RandomIntegerinRange 0 3) 0))
                  (Variables|Disks|SetDisk _returnvalue_2)
                  (else
                    ;[1 0.4948 0.5011 1 100] END GAME
                    (Utilities|FlowControl|DoOnce false
                      (:Completed
                        (Utilities|FlowControl|Sequence
                          (:then_0
                            (if (> _playerscore _enemyscore)
                              (Audio|PlaySound2D "/Game/Audio/SFX/Curling/curling8.curling8" 1.0 1.0 0.0 0 0)
                              (elif (== _playerscore _enemyscore)
                                (Audio|PlaySound2D "/Game/Audio/SFX/Curling/curling9.curling9" 1.0 1.0 0.0 0 0)
                                (else
                                  (Audio|PlaySound2D "/Game/Audio/SFX/Curling/curling7.curling7" 1.0 1.0 0.0 0 0)))))
                          (:then_1
                            (Game|Player|SetViewTargetwithBlend (Game|GetPlayerController 0) (Game|GetPlayerCharacter 0) 1.0 "VTBlend_Linear" 0.0 false)
                            (Utilities|FlowControl|Delay 1.0)
                            (bind _outactors (Actor|GetAllActorswithInterface "/Game/BluePrints/BPI/BPI_Dialogue.BPI_Dialogue_C"))
                            (for _array_element _outactors
                              (Class|BPIDialogue|DialogueSystemUpdate(Message) _array_element true)))))))))))
          (:2
            (Default|ProgressBarPlayerVisibility (Variables|Default|GetCurlingHUD) "HitTestInvisible")
            (bind _angle (Timeline|Línea%20de%20tiempo_2 PlayFromStart)
              (:Update
                (Variables|Disks|SetImpulse _angle)
                (Default|ProgressBarPlayerImpulse (Variables|Default|GetCurlingHUD) (Variables|Disks|GetImpulse))
                ;[1 0.8607 0.4989 1 100] DEBUG LINE
                (Rendering|Debug|DrawDebugLine _returnvalue (Math|Vector|MakeVector (.X (Math|Vector|BreakVector (+ _returnvalue (* (* (Math|Vector|GetForwardVector (Math|Rotator|MakeRotator 0.0 0.0 (Variables|Disks|GetAngle))) (Variables|Disks|GetImpulse)) -1)))) (.Y (Math|Vector|BreakVector (+ _returnvalue (* (* (Math|Vector|GetForwardVector (Math|Rotator|MakeRotator 0.0 0.0 (Variables|Disks|GetAngle))) (Variables|Disks|GetImpulse)) -1)))) (.Z (Math|Vector|BreakVector _returnvalue))) "(R=1.000000,G=0.000000,B=0.000000,A=1.000000)" 0.1 4.0))))
          (:3
            (Utilities|FlowControl|Sequence
              (:then_0
                (Timeline|Línea%20de%20tiempo_2 Stop))
              (:then_1
                (Input|DisableInput self (Game|GetPlayerController 0))
                (Class|BPICurling|CurlingPush(Message) (Variables|Disks|GetDisk) (Variables|Disks|GetAngle) (Variables|Disks|GetImpulse))
                (CallFunction|FocusCameraDisk)
                (Default|ProgressBarPlayerVisibility (Variables|Default|GetCurlingHUD) "Collapsed"))
              (:then_2
                (goto _label Reset)))))))))

(event Input|ActionEvents|InputActionKeyLeft
  (params (Key :type Key%20Structure :default "None"))
  (bind _billboard_disk_player (Variables|Default|GetBillboard_Disk_Player))
  (bind _returnvalue (Transformation|GetWorldLocation _billboard_disk_player))
  ;[1 0.8607 0.4989 1 100] DEBUG LINE
  (:Pressed
    (Utilities|FlowControl|Sequence
      (:then_0
        (bind _newtrack_0 (Timeline|Línea%20de%20tiempo_5 Stop)
          (:Update
            (Variables|Disks|SetAngle (Math|Float|Clamp(Float) (- (Variables|Disks|GetAngle) _newtrack_0) 3e+01 1.5e+02))
            (Rendering|Debug|DrawDebugLine _returnvalue (Math|Vector|MakeVector (.X (Math|Vector|BreakVector (+ _returnvalue (* (* (Math|Vector|GetForwardVector (Math|Rotator|MakeRotator 0.0 0.0 (Variables|Disks|GetAngle))) (Variables|Disks|GetImpulse)) -1)))) (.Y (Math|Vector|BreakVector (+ _returnvalue (* (* (Math|Vector|GetForwardVector (Math|Rotator|MakeRotator 0.0 0.0 (Variables|Disks|GetAngle))) (Variables|Disks|GetImpulse)) -1)))) (.Z (Math|Vector|BreakVector _returnvalue))) "(R=1.000000,G=0.000000,B=0.000000,A=1.000000)" 0.1 4.0 :!label _label))))
      (:then_1
        (bind _newtrack_0_2 (Timeline|Línea%20de%20tiempo_6 PlayFromStart)
          (:Update
            (Variables|Disks|SetAngle (Math|Float|Clamp(Float) (+ (Variables|Disks|GetAngle) _newtrack_0_2) 3e+01 1.5e+02))
            (goto _label))))))
  (:Released
    (Utilities|FlowControl|Sequence
      (:then_0
        (Timeline|Línea%20de%20tiempo_6 Stop))
      (:then_1
        (Timeline|Línea%20de%20tiempo_5 Stop)))))

(event Input|ActionEvents|InputActionKeyRight
  (params (Key :type Key%20Structure :default "None"))
  (bind _billboard_disk_player (Variables|Default|GetBillboard_Disk_Player))
  (bind _returnvalue (Transformation|GetWorldLocation _billboard_disk_player))
  ;[1 0.8607 0.4989 1 100] DEBUG LINE
  (:Pressed
    (Utilities|FlowControl|Sequence
      (:then_0
        (bind _newtrack_0 (Timeline|Línea%20de%20tiempo_6 Stop)
          (:Update
            (Variables|Disks|SetAngle (Math|Float|Clamp(Float) (+ (Variables|Disks|GetAngle) _newtrack_0) 3e+01 1.5e+02))
            (Rendering|Debug|DrawDebugLine _returnvalue (Math|Vector|MakeVector (.X (Math|Vector|BreakVector (+ _returnvalue (* (* (Math|Vector|GetForwardVector (Math|Rotator|MakeRotator 0.0 0.0 (Variables|Disks|GetAngle))) (Variables|Disks|GetImpulse)) -1)))) (.Y (Math|Vector|BreakVector (+ _returnvalue (* (* (Math|Vector|GetForwardVector (Math|Rotator|MakeRotator 0.0 0.0 (Variables|Disks|GetAngle))) (Variables|Disks|GetImpulse)) -1)))) (.Z (Math|Vector|BreakVector _returnvalue))) "(R=1.000000,G=0.000000,B=0.000000,A=1.000000)" 0.1 4.0 :!label _label))))
      (:then_1
        (bind _newtrack_0_2 (Timeline|Línea%20de%20tiempo_5 PlayFromStart)
          (:Update
            (Variables|Disks|SetAngle (Math|Float|Clamp(Float) (- (Variables|Disks|GetAngle) _newtrack_0_2) 3e+01 1.5e+02))
            (goto _label))))))
  (:Released
    (Utilities|FlowControl|Sequence
      (:then_0
        (Timeline|Línea%20de%20tiempo_6 Stop))
      (:then_1
        (Timeline|Línea%20de%20tiempo_5 Stop)))))

(fn ConstructionScript)

(fn LightOuter
  (params (Condition :type Boolean))
  (Rendering|Components|Decal|SetDecalMaterial (Variables|Default|GetDecal_OuterCircle) (select Condition "/Game/BluePrints/Curling/Material_Curling_Sign_Inst9.Material_Curling_Sign_Inst9" "/Game/BluePrints/Curling/Material_Curling_Sign_Inst5.Material_Curling_Sign_Inst5")))

(fn LightInner
  (params (Condition :type Boolean))
  (Rendering|Components|Decal|SetDecalMaterial (Variables|Default|GetDecal_Good2) (select Condition "/Game/BluePrints/Curling/Material_Curling_Sign_Inst8.Material_Curling_Sign_Inst8" "/Game/BluePrints/Curling/Material_Curling_Sign_Inst2.Material_Curling_Sign_Inst2")))

(fn LightGood
  (params (Condition :type Boolean))
  (Rendering|Components|Decal|SetDecalMaterial (Variables|Default|GetDecal_Good1) (select Condition "/Game/BluePrints/Curling/Material_Curling_Sign_Inst7.Material_Curling_Sign_Inst7" "/Game/BluePrints/Curling/Material_Curling_Sign_Inst1.Material_Curling_Sign_Inst1")))

(fn LightBad
  (params (Condition :type Boolean))
  (Rendering|Components|Decal|SetDecalMaterial (Variables|Default|GetDecal_Bad) (select Condition "/Game/BluePrints/Curling/Material_Curling_Sign_Inst6.Material_Curling_Sign_Inst6" "/Game/BluePrints/Curling/Material_Curling_Sign_Inst.Material_Curling_Sign_Inst")))

(fn UpdateScore
  (bind _disk (Variables|Disks|GetDisk))
  (bind _curlinghud (Variables|Default|GetCurlingHUD))
  (bind _light (Variables|/Game/BluePrints/Curling/BP_CurlingDisk.BP_CurlingDisk_C|GetLight _disk))
  (bind _returnvalue (Math|Integer|Clamp(Integer) _light 0 4))
  (bind _returnvalue_2 (Utilities|Select :Index _returnvalue :Option%200 2 :Option%201 -2 :Option%202 1 :Option%203 2 :Option%204 0))
  (if (Variables|/Game/BluePrints/Curling/BP_CurlingDisk.BP_CurlingDisk_C|GetIsPlayer? (Variables|Disks|GetDisk))
    (Utilities|IsValid _curlinghud
      (:Is%20Valid
        (Default|UpdateScorePlayer _curlinghud _returnvalue_2)))
    (else
      (Utilities|IsValid _curlinghud
        (:Is%20Valid
          (Default|UpdateScoreEnemy _curlinghud _returnvalue_2))))))

(fn UpdateScoreTotal
  (bind _curlinghud (Variables|Default|GetCurlingHUD))
  (Variables|Default|SetPlayerScore 0)
  (Variables|Default|SetEnemyScore 0)
  (bind _outactors (Actor|GetAllActorsOfClass "/Game/BluePrints/Curling/BP_CurlingDisk.BP_CurlingDisk_C"))
  (for _array_element _outactors
    (bind _output_get (LocalVariables|SetDiskLocal _array_element))
    (Utilities|IsValid _output_get
      (:Is%20Valid
        (Variables|/Game/BluePrints/Curling/BP_CurlingDisk.BP_CurlingDisk_C|SetEnabled? (LocalVariables|GetDiskLocal) false)
        (if (Variables|/Game/BluePrints/Curling/BP_CurlingDisk.BP_CurlingDisk_C|GetIsPlayer? (LocalVariables|GetDiskLocal))
          (Variables|Default|SetPlayerScore (Math|Integer|Clamp(Integer) (+ (Variables|Default|GetPlayerScore) (Utilities|Select :Index (Math|Integer|Clamp(Integer) (Variables|/Game/BluePrints/Curling/BP_CurlingDisk.BP_CurlingDisk_C|GetLight (LocalVariables|GetDiskLocal)) 0 4) :Option%200 2 :Option%201 -2 :Option%202 1 :Option%203 2 :Option%204 0)) -10 10))
          (else
            (Variables|Default|SetEnemyScore (Math|Integer|Clamp(Integer) (+ (Variables|Default|GetEnemyScore) (Utilities|Select :Index (Math|Integer|Clamp(Integer) (Variables|/Game/BluePrints/Curling/BP_CurlingDisk.BP_CurlingDisk_C|GetLight (LocalVariables|GetDiskLocal)) 0 4) :Option%200 2 :Option%201 -2 :Option%202 1 :Option%203 2 :Option%204 0)) -10 10)))))))
  (Utilities|IsValid _curlinghud
    (:Is%20Valid
      (Default|UpdateScorePlayer _curlinghud (Variables|Default|GetPlayerScore))
      (Default|UpdateScoreEnemy _curlinghud (Variables|Default|GetEnemyScore)))))