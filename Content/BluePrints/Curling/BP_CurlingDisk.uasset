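; Physics-driven curling disk with four variants (mesh, mass, damping) and side-specific materials, set in the construction script.
; CurlingPush launches it once with a clamped, mass-independent impulse and draws a debug line.
; Waking enables Tick, which detects near-rest once, sleeps the body and messages all BPI_Curling actors to reset.
; One variant stops simulating physics at rest with a sound; disk-to-disk hits play a throttled sound.
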(event OnComponentWake(CurlingDisk)
  (params (WakingComponent :type Primitive%20Component%20Object%20Reference) (BoneName :type Name :default "None"))
  ;[1 1 1 1 100] PHYSICS
  (Utilities|FlowControl|DoOnce false
    (:Completed
      (Actor|Tick|SetActorTickEnabled true))))

(event OnComponentHit(CurlingDisk)
  (params (HitComponent :type Primitive%20Component%20Object%20Reference) (OtherActor :type Actor%20Object%20Reference) (OtherComp :type Primitive%20Component%20Object%20Reference) (NormalImpulse :type Vector :default "0, 0, 0") (Hit :type Hit%20Result%20Structure%20%28by%20ref%29))
  ;[1 1 1 1 100] SOUND
  (Utilities|Casting|CastToBP_CurlingDisk OtherActor)
  (Utilities|FlowControl|DoOnce false :!label _label
    (:Completed
      (Audio|PlaySound2D "/Game/Audio/SFX/Curling/curling3.curling3" 1.0 1.0 0.0 0 0)
      (Utilities|FlowControl|Delay 0.2)
      (goto _label Reset))))

(event EventCurlingReset
  ;[1 1 1 1 100] PHYSICS
  (Class|PrimitiveComponent|PutRigidBodytoSleep (Variables|Default|GetCurlingDisk) "None"))

(event EventTick
  (params (DeltaSeconds :type Float%20%28single-precision%29))
  (bind _staticmesh (Variables|Default|GetStaticMesh))
  (bind _curlingdisk (Variables|Default|GetCurlingDisk))
  (bind _returnvalue (Math|Integer|Clamp(Integer) _staticmesh 0 3))
  (bind _returnvalue_2 (Utilities|Select :Index _returnvalue :Option%200 true :Option%201 true :Option%202 true :Option%203 false))
  ;[1 1 1 1 100] PHYSICS
  (bind _returnvalue_3 (Physics|GetPhysicsLinearVelocity (Variables|Default|GetCurlingDisk) "None"))
  (if (<= (Math|Vector|VectorLength _returnvalue_3) 1e+01)
    (Utilities|FlowControl|DoOnce false
      (:Completed
        (Utilities|FlowControl|Sequence
          (:then_0
            (Actor|Tick|SetActorTickEnabled false))
          (:then_1
            (Class|PrimitiveComponent|PutRigidBodytoSleep _curlingdisk "None")
            (Physics|SetSimulatePhysics _curlingdisk _returnvalue_2)
            (if (not _returnvalue_2)
              (Audio|PlaySound2D "/Game/Audio/SFX/Curling/curling5.curling5" 1.0 1.0 0.0 0 0)))
          (:then_2
            (bind _outactors (Actor|GetAllActorswithInterface "/Game/BluePrints/BPI/BPI_Curling.BPI_Curling_C"))
            (for _array_element _outactors
              (Class|BPICurling|CurlingReset(Message) _array_element))))))))

(event EventCurlingPush
  (params (Angle :type Float%20%28single-precision%29) (Impulse :type Float%20%28single-precision%29))
  (bind _self self)
  (bind _curlingdisk (Variables|Default|GetCurlingDisk))
  (bind _returnvalue (Transformation|GetActorLocation _self))
  ;[1 1 1 1 100] PHYSICS
  (Utilities|FlowControl|DoOnce false
    (:Completed
      (Variables|Default|SetAngle (Math|Float|Clamp(Float) Angle 3e+01 1.5e+02))
      (Variables|Default|SetImpulse (Math|Float|Clamp(Float) Impulse 2e+02 2e+03))
      (Rendering|Debug|DrawDebugLine _returnvalue (Math|Vector|MakeVector (.X (Math|Vector|BreakVector (+ _returnvalue (* (* (Math|Vector|GetForwardVector (Math|Rotator|MakeRotator 0.0 0.0 (Variables|Default|GetAngle))) (Variables|Default|GetImpulse)) -1)))) (.Y (Math|Vector|BreakVector (+ _returnvalue (* (* (Math|Vector|GetForwardVector (Math|Rotator|MakeRotator 0.0 0.0 (Variables|Default|GetAngle))) (Variables|Default|GetImpulse)) -1)))) (.Z (Math|Vector|BreakVector _returnvalue))) "(R=1.000000,G=0.000000,B=0.000000,A=1.000000)" 2.0 4.0)
      (Class|PrimitiveComponent|WakeRigidBody _curlingdisk "None")
      (Physics|AddImpulse _curlingdisk (* (* (Math|Vector|GetForwardVector (Math|Rotator|MakeRotator 0.0 0.0 (Variables|Default|GetAngle))) (Variables|Default|GetImpulse)) -1) "None" true))))

(fn ConstructionScript
  (bind _isplayer_ (Variables|Default|GetIsPlayer?))
  (bind _curlingdisk (Variables|Default|GetCurlingDisk))
  (bind _staticmesh (Variables|Default|GetStaticMesh))
  (bind _curlingdisk_2 (Variables|Default|GetCurlingDisk))
  (bind _returnvalue (Math|Integer|Clamp(Integer) _staticmesh 0 3))
  (bind _returnvalue_2 (select _isplayer_ "/Game/Material/Plastic/Material_Plastic_Inst13.Material_Plastic_Inst13" "/Game/Material/Plastic/Material_Plastic_Inst3.Material_Plastic_Inst3"))
  (Rendering|Material|SetMaterial _curlingdisk 1 _returnvalue_2)
  (Rendering|Material|SetMaterial _curlingdisk 2 _returnvalue_2)
  (Rendering|Material|SetMaterial _curlingdisk 3 _returnvalue_2)
  (Components|StaticMesh|SetStaticMesh _curlingdisk_2 (Utilities|Select :Index _returnvalue :Option%200 "/Game/StaticMeshes/Curling/CurlingDisks_Disk.CurlingDisks_Disk" :Option%201 "/Game/StaticMeshes/Curling/CurlingDisks_Disk_002.CurlingDisks_Disk_002" :Option%202 "/Game/StaticMeshes/Curling/CurlingDisks_Disk_003.CurlingDisks_Disk_003" :Option%203 "/Game/StaticMeshes/Curling/CurlingDisks_Disk_001.CurlingDisks_Disk_001"))
  (Class|PrimitiveComponent|SetMassOverrideinKg _curlingdisk_2 "None" (Utilities|Select :Index _returnvalue :Option%200 0.5 :Option%201 0.3 :Option%202 0.2 :Option%203 0.4) true)
  (Class|PrimitiveComponent|SetLinearDamping _curlingdisk_2 (Utilities|Select :Index _returnvalue :Option%200 0.5 :Option%201 0.3 :Option%202 0.2 :Option%203 0.4)))