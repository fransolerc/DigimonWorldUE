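; Interior camera actor that becomes player 0's view target on BeginPlay and tracks the player character within a box.
; Each tick, the camera's relative X and Y are set from the character's world position plus an offset, clamped to the box extents, with Z fixed at the offset.
; The construction script sizes the collision box and applies the camera's offset and rotation.
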(event EventBeginPlay
  ;[1 1 1 1 100] CAMERA
  (Game|Player|SetViewTargetwithBlend (Game|GetPlayerController 0) (Components|GetOwner (Variables|Default|GetCamera)) 0.0 "VTBlend_Linear" 0.0 false))

(event EventTick
  (params (DeltaSeconds :type Float%20%28single-precision%29))
  (bind _returnvalue (Math|Float|MakeLiteralFloat 0.0))
  (bind _returnvalue_2 (Game|GetPlayerCharacter 0))
  (bind _cameraoffsetlocation (Variables|Camera|GetCameraOffsetLocation))
  (bind _boxentension (Variables|Camera|GetBoxEntension))
  (bind (_x _y _z) (Math|Vector|BreakVector _cameraoffsetlocation))
  (bind (_x_2 _y_2) (Math|Vector|BreakVector _boxentension))
  (bind _returnvalue_3 (Transformation|GetActorLocation _returnvalue_2))
  (bind (_x_3 _y_3) (Math|Vector|BreakVector _returnvalue_3))
  ;[1 1 1 1 100] MOVE CAMERA
  (Transformation|SetRelativeLocation (Variables|Default|GetCamera) (Math|Vector|MakeVector (Math|Float|Clamp(Float) (+ _x_3 _x) (- _returnvalue _x_2) _x_2) (Math|Float|Clamp(Float) (+ _y_3 _y) (- _returnvalue _y_2) _y_2) _z) false false))

(fn ConstructionScript
  (Components|Box|SetBoxExtent (Variables|Default|GetBoxCollision) (Variables|Camera|GetBoxEntension) true)
  (Transformation|SetRelativeLocationAndRotation (Variables|Default|GetCamera) (Variables|Camera|GetCameraOffsetLocation) (Variables|Camera|GetCameraRotation) false false))