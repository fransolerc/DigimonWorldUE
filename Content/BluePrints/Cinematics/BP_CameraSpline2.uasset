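; Spline-following cinematic camera actor that becomes the player's view target on BeginPlay and tracks the player character.
; Each tick it moves the Camera to the spline point closest to the player, passing that world-space point as a relative location.
; The construction script applies an offset location and rotation; Tick overwrites the location, while the rotation stays fixed.
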(event EventBeginPlay
  ;[1 1 1 1 100] CAMERA
  (Game|Player|SetViewTargetwithBlend (Game|GetPlayerController 0) (Components|GetOwner (Variables|Default|GetCamera)) 0.0 "VTBlend_Linear" 0.0 false))

(event EventTick
  (params (DeltaSeconds :type Float%20%28single-precision%29))
  ;[1 1 1 1 100] MOVE CAMERA
  (Transformation|SetRelativeLocation (Variables|Default|GetCamera) (Spline|FindLocationClosesttoWorldLocation (Variables|Default|GetSpline) (Transformation|GetActorLocation (Game|GetPlayerCharacter 0)) "World") false false))

(fn ConstructionScript
  (Transformation|SetRelativeLocationAndRotation (Variables|Default|GetCamera) (Variables|Default|GetCameraOffsetLocation) (Variables|Default|GetCameraRotation) false false))