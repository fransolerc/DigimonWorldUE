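; Amida Forest cinematic shot actor that knocks back the player and Digimon partner when they overlap its box.
; Each target type gets a one-time velocity-change impulse along world Y and upward, with the Y push scaled by the actor's remaining lifespan and stronger for the player.
; The partner hit also clears the message lock on all BPI_Dialogue actors and passes them the Amida Forest Event 1 dialogue with auto-play.
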(event OnComponentBeginOverlap(Box)
  (params (OverlappedComponent :type Primitive%20Component%20Object%20Reference) (OtherActor :type Actor%20Object%20Reference) (OtherComp :type Primitive%20Component%20Object%20Reference) (OtherBodyIndex :type Integer) (bFromSweep :type Boolean) (SweepResult :type Hit%20Result%20Structure%20%28by%20ref%29))
  (bind _self self)
  (bind _returnvalue (Actor|GetLifeSpan _self))
  (bind _asjugador (Utilities|Casting|CastToJugador OtherActor)
    (:then
      (Utilities|FlowControl|DoOnce false
        (:Completed
          (Physics|AddImpulse (Variables|/Script/Engine.Character|GetCharacterMovement _asjugador) (Math|Vector|MakeVector 0.0 (* _returnvalue 2e+02) 2e+02) true))))
    (:CastFailed
      (bind _asai_digimon_partner (Utilities|Casting|CastToAI_DigimonPartner OtherActor))
      (Utilities|FlowControl|DoOnce false
        (:Completed
          (Physics|AddImpulse (Variables|/Script/Engine.Character|GetCharacterMovement _asai_digimon_partner) (Math|Vector|MakeVector 0.0 (* _returnvalue 1.5e+02) 2e+02) true)
          (bind _outactors (Actor|GetAllActorswithInterface "/Game/BluePrints/BPI/BPI_Dialogue.BPI_Dialogue_C"))
          (for _array_element _outactors
            (Class|BPIDialogue|DialogueSystemLock(Message) _array_element false)
            (Class|BPIDialogue|DialogueSystemValuesSet(Message) _array_element 0 "/Game/Game/DataTables/Dialogue/AmidaForest/DataTable_Dialogue_AmidaForest_Event1.DataTable_Dialogue_AmidaForest_Event1" true)))))))

(fn ConstructionScript)