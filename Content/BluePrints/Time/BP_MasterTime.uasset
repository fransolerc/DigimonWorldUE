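; BP_MasterTime is the master game clock, advancing minutes, hours, days and years in DW1_GameInstance's GameTime and updating the HUD clock.
; A looping timer ticks each game minute at an area-dependent rate, and speed-matched timelines interpolate sun rotation and intensity from day curves between minutes.
; Hour changes drive sun shadows, partner updates, day/night lighting and music, and new-day triggers.
; Events also start, stop, skip time or reset on level streaming.
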(event Custom|UpdateEveryMinute
  ;[1 1 1 1 100] Timer
  (Clock|UpdateEveryMinuteFunction)
  (Clock|UpdateClock)
  (if (and (Utilities|IsValid (Variables|DayNightCycle|GetBP_SkySphere)) (Utilities|IsValid (Variables|DayNightCycle|GetDirectionalLightActor)))
    (switch int (Utilities|Select :Index (Variables|Time|GetArea) :NewEnumerator0 0 :NewEnumerator1 0 :NewEnumerator2 0 :NewEnumerator3 0 :NewEnumerator4 0 :NewEnumerator5 0 :NewEnumerator6 0 :NewEnumerator7 1 :NewEnumerator8 2 :NewEnumerator9 0 :NewEnumerator10 0 :NewEnumerator11 0 :NewEnumerator12 0 :NewEnumerator13 0 :NewEnumerator14 0 :NewEnumerator15 0 :NewEnumerator16 0 :NewEnumerator17 0 :NewEnumerator18 0 :NewEnumerator19 0 :NewEnumerator21 0 :NewEnumerator22 0 :NewEnumerator23 0 :NewEnumerator25 0 :NewEnumerator26 0 :NewEnumerator27 0 :NewEnumerator28 0 :NewEnumerator29 0 :NewEnumerator31 0 :NewEnumerator32 0 :NewEnumerator33 0 :NewEnumerator40 0 :NewEnumerator41 0 :NewEnumerator42 0 :NewEnumerator43 0)
      (:0
        (bind _time_seconds (Timeline|TimeSpeed_NormalTimeline PlayFromStart)
          (:Update
            (Variables|Time|SetTimeSeconds _time_seconds))))
      (:1
        (bind _time_seconds_2 (Timeline|TimeSpeed_SlowTimeline PlayFromStart)
          (:Update
            (Variables|Time|SetTimeSeconds _time_seconds_2))))
      (:2
        (bind _time_seconds_3 (Timeline|TimeSpeed_SpeedyTimeline PlayFromStart)
          (:Update
            (Variables|Time|SetTimeSeconds _time_seconds_3)))))
    (Lighting|UpdateSunandSky)))

(event EventTimeStart
  ;[1 0.2376 0.2077 1 100] START / STOP
  (if (Class|KismetSystemLibrary|TimerExistsHandle (Variables|Timer|GetTimerHandle_Weather))
    (Utilities|Time|UnpauseTimerbyHandle (Variables|Timer|GetTimerHandle_Weather))
    (else
      ;[1 1 1 1 100] Timer
      (Lighting|GetActors)
      (bind _returnvalue (Utilities|Time|SetTimerbyEvent (delegate Custom|UpdateEveryMinute) (Utilities|Select :Index (Variables|Time|GetArea) :NewEnumerator0 1.0 :NewEnumerator1 1.0 :NewEnumerator2 1.0 :NewEnumerator3 1.0 :NewEnumerator4 1.0 :NewEnumerator5 1.0 :NewEnumerator6 1.0 :NewEnumerator7 2.0 :NewEnumerator8 0.5 :NewEnumerator9 1.0 :NewEnumerator10 1.0 :NewEnumerator11 1.0 :NewEnumerator12 1.0 :NewEnumerator13 1.0 :NewEnumerator14 1.0 :NewEnumerator15 1.0 :NewEnumerator16 1.0 :NewEnumerator17 1.0 :NewEnumerator18 1.0 :NewEnumerator19 1.0 :NewEnumerator21 1.0 :NewEnumerator22 1.0 :NewEnumerator23 1.0 :NewEnumerator25 1.0 :NewEnumerator26 1.0 :NewEnumerator27 1.0 :NewEnumerator28 1.0 :NewEnumerator29 1.0 :NewEnumerator31 1.0 :NewEnumerator32 1.0 :NewEnumerator33 1.0 :NewEnumerator40 1.0 :NewEnumerator41 1.0 :NewEnumerator42 1.0 :NewEnumerator43 1.0) true))
      (Variables|Timer|SetTimerHandle_Weather _returnvalue))))

(event EventTimeStop
  ;[1 0.2376 0.2077 1 100] START / STOP
  (Utilities|Time|PauseTimerbyHandle (Variables|Timer|GetTimerHandle_Weather))
  (Utilities|FlowControl|Sequence
    (:then_0
      ;[1 1 1 1 100] Timer
      (bind _time_seconds (Timeline|TimeSpeed_NormalTimeline Stop)
        (:Update
          (Variables|Time|SetTimeSeconds _time_seconds))))
    (:then_1
      (bind _time_seconds_2 (Timeline|TimeSpeed_SlowTimeline Stop)
        (:Update
          (Variables|Time|SetTimeSeconds _time_seconds_2))))
    (:then_2
      (bind _time_seconds_3 (Timeline|TimeSpeed_SpeedyTimeline Stop)
        (:Update
          (Variables|Time|SetTimeSeconds _time_seconds_3)))))
  (Lighting|UpdateSunandSky))

(event EventTimeForwardExactHour
  (params (Exact%20Hour :type Integer))
  ;[0.6344 0.5744 1 1 100] FORWARD TIME
  (Clock|ForwardTimeExact Exact%20Hour))

(event EventTimeLevelStreaming
  (params (Area :type Enum_OST_Names%20Enum :default "NewEnumerator0"))
  ;[0.8604 0.3575 1 1 100] LOAD GAME / LEVEL STREAMING
  (Variables|Time|SetArea Area)
  (Utilities|FlowControl|Sequence
    (:then_0
      (Utilities|Time|ClearandInvalidateTimerbyHandle (Variables|Timer|GetTimerHandle_Weather))
      (Variables|Timer|SetTimerHandle_Weather ""))
    (:then_1
      ;[1 1 1 1 100] Timer
      (bind _time_seconds (Timeline|TimeSpeed_NormalTimeline Stop)
        (:Update
          (Variables|Time|SetTimeSeconds _time_seconds)
          (Lighting|UpdateSunandSky :!label _label))))
    (:then_2
      (bind _time_seconds_2 (Timeline|TimeSpeed_SlowTimeline Stop)
        (:Update
          (Variables|Time|SetTimeSeconds _time_seconds_2)
          (goto _label))))
    (:then_3
      (bind _time_seconds_3 (Timeline|TimeSpeed_SpeedyTimeline Stop)
        (:Update
          (Variables|Time|SetTimeSeconds _time_seconds_3)
          (goto _label))))
    (:then_4
      (Lighting|UpdateLights))
    (:then_5
      (Lighting|GetActors)
      (if (and (Utilities|IsValid (Variables|DayNightCycle|GetBP_SkySphere)) (Utilities|IsValid (Variables|DayNightCycle|GetDirectionalLightActor)))
        (Lighting|SetSunLighting)
        (Lighting|UpdateSunandSky)))))

(event EventTimeForwardHours
  (params (Add%20Hours :type Integer))
  ;[0.6344 0.5744 1 1 100] FORWARD TIME
  (Clock|ForwardTimeAddHours Add%20Hours))

(fn ConstructionScript)

(fn GetActors
  (Utilities|FlowControl|Sequence
    (:then_0
      (bind _outactors (Actor|GetAllActorsOfClass "/Script/Engine.DirectionalLight"))
      (if (> (Utilities|Array|Length _outactors) 0)
        (Variables|DayNightCycle|SetDirectionalLightActor (Utilities|Array|Get(acopy) _outactors))))
    (:then_1
      (bind _outactors_2 (Actor|GetAllActorsOfClass "/Game/BluePrints/Time/BP_Sky_Sphere_Custom.BP_Sky_Sphere_Custom_C"))
      (if (> (Utilities|Array|Length _outactors_2) 0)
        (Variables|DayNightCycle|SetBP_SkySphere (Utilities|Array|Get(acopy) _outactors_2))))))

(fn SetSunLighting
  (bind _directionallightactor (Variables|DayNightCycle|GetDirectionalLightActor))
  (Utilities|IsValid _directionallightactor
    (:Is%20Valid
      (bind _asdw1_game_instance (Utilities|Casting|CastToDW1_GameInstance (Game|GetGameInstance)))
      (bind _output_get (LocalVariables|SetGameInstance _asdw1_game_instance))
      (Rendering|Components|Light|SetCastShadows (Variables|/Script/Engine.Light|GetLightComponent _directionallightactor) (Utilities|Select :Index (Math|Integer|Clamp(Integer) (Utilities|Struct|BreakStruct_Time (Variables|/Game/Game/DW1_GameInstance.DW1_GameInstance_C|GetGame%20Time _output_get)) 0 23) :Option%200 false :Option%201 false :Option%202 false :Option%203 false :Option%204 false :Option%205 true :Option%206 true :Option%207 true :Option%208 true :Option%209 true :Option%2010 true :Option%2011 true :Option%2012 true :Option%2013 true :Option%2014 true :Option%2015 true :Option%2016 true :Option%2017 true :Option%2018 true :Option%2019 true :Option%2020 true :Option%2021 false :Option%2022 false :Option%2023 false)))))

(fn UpdateSunandSky
  (bind _directionallightactor (Variables|DayNightCycle|GetDirectionalLightActor))
  (bind _lightcomponent (Variables|/Script/Engine.Light|GetLightComponent _directionallightactor))
  (bind _asdw1_game_instance (Utilities|Casting|CastToDW1_GameInstance (Game|GetGameInstance)))
  (bind _output_get (LocalVariables|SetGameInstance _asdw1_game_instance))
  (bind _output_get_2 (LocalVariables|SetTimeLocal1 (Math|Integer|Clamp(Integer) (+ (* (.Hours (Utilities|Struct|BreakStruct_Time (Variables|/Game/Game/DW1_GameInstance.DW1_GameInstance_C|GetGame%20Time _output_get))) 60) (.Minutes (Utilities|Struct|BreakStruct_Time (Variables|/Game/Game/DW1_GameInstance.DW1_GameInstance_C|GetGame%20Time _output_get)))) 0 1439)))
  (LocalVariables|SetTimeLocal2 (Math|Integer|Clamp(Integer) (- _output_get_2 1) 0 1439))
  (Transformation|SetRelativeRotation _lightcomponent (Math|Rotator|MakeRotator 0.0 (Math|Curves|GetFloatValue (Variables|DayNightCycle|GetDayCurve) (Math|Float|Lerp (Math|Conversions|ToFloat(Integer) (LocalVariables|GetTimeLocal2)) (Math|Conversions|ToFloat(Integer) (LocalVariables|GetTimeLocal1)) (Math|Float|Clamp(Float) (Variables|Time|GetTimeSeconds)))) 0.0) false false)
  (Rendering|Components|Light|SetIntensity _lightcomponent (Math|Curves|GetFloatValue (Variables|DayNightCycle|GetSunIntensity_Curve) (Math|Float|Lerp (Math|Conversions|ToFloat(Integer) (LocalVariables|GetTimeLocal2)) (Math|Conversions|ToFloat(Integer) (LocalVariables|GetTimeLocal1)) (Math|Float|Clamp(Float) (Variables|Time|GetTimeSeconds)))))
  (Default|UpdateSunDirection (Variables|DayNightCycle|GetBP_SkySphere)))

(fn NewDayFunction
  (bind _asdw1_game_instance (Utilities|Casting|CastToDW1_GameInstance (Game|GetGameInstance)))
  (bind _output_get (LocalVariables|SetGameInstance _asdw1_game_instance))
  (if (> (Utilities|Struct|BreakStruct_Time (Variables|/Game/Game/DW1_GameInstance.DW1_GameInstance_C|GetGame%20Time _output_get)) 29)
    (Utilities|Struct|SetmembersinStruct_Time (Variables|/Game/Game/DW1_GameInstance.DW1_GameInstance_C|GetGame%20Time (LocalVariables|GetGameInstance)) (Math|Integer|Clamp(Integer) (+ (Utilities|Struct|BreakStruct_Time (Variables|/Game/Game/DW1_GameInstance.DW1_GameInstance_C|GetGame%20Time (LocalVariables|GetGameInstance))) 1) 0 999))
    (else
      (Utilities|Struct|SetmembersinStruct_Time (Variables|/Game/Game/DW1_GameInstance.DW1_GameInstance_C|GetGame%20Time (LocalVariables|GetGameInstance)) (Math|Integer|Clamp(Integer) (+ (Utilities|Struct|BreakStruct_Time (Variables|/Game/Game/DW1_GameInstance.DW1_GameInstance_C|GetGame%20Time (LocalVariables|GetGameInstance))) 1) 0 29))))
  ;[1 1 1] Triggers
  (Utilities|FlowControl|Sequence
    (:then_0
      (Math|Integer|IncrementInt (Utilities|Struct|BreakStruct_Digimon_Partner_Info (Variables|/Game/Game/DW1_GameInstance.DW1_GameInstance_C|GetPartner%20Info (LocalVariables|GetGameInstance)))))
    (:then_1
      (CallFunction|SetGameTrigger 87 false) ; Take Meat?
      (CallFunction|SetGameTrigger 196 false) ; Rain Plant Harvested?
    )
    (:then_2
      (if (Utilities|Struct|BreakStruct_Game_Triggers (Variables|/Game/Game/DW1_GameInstance.DW1_GameInstance_C|GetGame%20Triggers (LocalVariables|GetGameInstance)))
        (CallFunction|SetGameTrigger 179 true) ; Andromon dump repaired
      ))))

(fn UpdateAudio
  ;[1 1 1 1 100] UpdateAudio
  (bind _outactors (Actor|GetAllActorswithInterface "/Game/BluePrints/BPI/BPI_Audio.BPI_Audio_C"))
  (for _array_element _outactors
    (Class|BPIAudio|AudioSetBGM(Message) _array_element)))

(fn UpdateEveryMinuteFunction
  ;[1 1 1 1 100] Update
  (bind _asdw1_game_instance (Utilities|Casting|CastToDW1_GameInstance (Game|GetGameInstance)))
  (bind _output_get (LocalVariables|SetGameInstance _asdw1_game_instance))
  (if (>= (Utilities|Struct|BreakStruct_Time (Variables|/Game/Game/DW1_GameInstance.DW1_GameInstance_C|GetGame%20Time _output_get)) 59)
    ;[1 1 1 1 100] Update Every HOUR
    (Utilities|FlowControl|Sequence
      (:then_0
        (if (> (+ (Utilities|Struct|BreakStruct_Time (Variables|/Game/Game/DW1_GameInstance.DW1_GameInstance_C|GetGame%20Time (LocalVariables|GetGameInstance))) 1) 23)
          ;;[1 1 1] NEW DAY
          (Utilities|Struct|SetmembersinStruct_Time (Variables|/Game/Game/DW1_GameInstance.DW1_GameInstance_C|GetGame%20Time (LocalVariables|GetGameInstance)))
          (Clock|NewDayFunction)
          (else
            (Utilities|Struct|SetmembersinStruct_Time (Variables|/Game/Game/DW1_GameInstance.DW1_GameInstance_C|GetGame%20Time (LocalVariables|GetGameInstance)) (Math|Integer|Clamp(Integer) (+ (Utilities|Struct|BreakStruct_Time (Variables|/Game/Game/DW1_GameInstance.DW1_GameInstance_C|GetGame%20Time (LocalVariables|GetGameInstance))) 1) 0 23)))))
      (:then_1
        (Lighting|SetSunLighting)
        (Lighting|UpdateAudioLighting))
      (:then_2
        (bind _outactors (Actor|GetAllActorswithInterface "/Game/BluePrints/BPI/BPI_DigimonPartnerSystem.BPI_DigimonPartnerSystem_C"))
        (for _array_element _outactors
          (Class|BPIDigimonPartnerSystem|DigimonPartnerSystemUpdateStatus(Message) _array_element))))
    (else
      ;[1 1 1 1 100] Update Every Minute
      (Utilities|Struct|SetmembersinStruct_Time (Variables|/Game/Game/DW1_GameInstance.DW1_GameInstance_C|GetGame%20Time (LocalVariables|GetGameInstance)) (+ (Utilities|Struct|BreakStruct_Time (Variables|/Game/Game/DW1_GameInstance.DW1_GameInstance_C|GetGame%20Time _output_get)) 1)))))

(fn ForwardTimeAddHours
  (params (Add%20Hours :type Integer))
  (LocalVariables|SetAddTime (Math|Integer|Clamp(Integer) Add%20Hours 1 8))
  (bind _asdw1_game_instance (Utilities|Casting|CastToDW1_GameInstance (Game|GetGameInstance)))
  (bind _output_get (LocalVariables|SetGameInstance _asdw1_game_instance))
  (LocalVariables|SetTotalTime (+ (LocalVariables|GetAddTime) (Utilities|Struct|BreakStruct_Time (Variables|/Game/Game/DW1_GameInstance.DW1_GameInstance_C|GetGame%20Time _output_get))))
  (LocalVariables|SetIsDay?%20PreCalculate (.IsDay?%20Event (CallFunction|DetermineDayNight)))
  (Utilities|FlowControl|Sequence
    (:then_0
      ;[1 1 1 1 100] Set New Hour
      (if (> (LocalVariables|GetTotalTime) 23)
        (Utilities|Struct|SetmembersinStruct_Time (Variables|/Game/Game/DW1_GameInstance.DW1_GameInstance_C|GetGame%20Time (LocalVariables|GetGameInstance)) (Math|Integer|Clamp(Integer) (- (LocalVariables|GetTotalTime) (Class|KismetSystemLibrary|MakeLiteralInteger 24)) 0 23))
        (Clock|NewDayFunction)
        (else
          (Utilities|Struct|SetmembersinStruct_Time (Variables|/Game/Game/DW1_GameInstance.DW1_GameInstance_C|GetGame%20Time (LocalVariables|GetGameInstance)) (Math|Integer|Clamp(Integer) (LocalVariables|GetTotalTime) 0 23)))))
    (:then_1
      (Lighting|UpdateLights))
    (:then_2
      (Lighting|SetSunLighting))
    (:then_3
      (Lighting|UpdateSunandSky))
    (:then_4
      ;[1 1 1 1 100] Update Audio?
      (bind _returnvalue (Class|DataTableFunctionLibrary|DoesDataTableRowExist "/Game/Game/DataTables/Levels/DataTable_Level_Info.DataTable_Level_Info" (.CurrentLevelName (Utilities|Struct|BreakStruct_Game_Locations (Variables|/Game/Game/DW1_GameInstance.DW1_GameInstance_C|GetGame%20Location%20and%20Rotation (LocalVariables|GetGameInstance))))))
      (if _returnvalue
        (bind _returnvalue_2 (Utilities|GetDataTableRow "/Game/Game/DataTables/Levels/DataTable_Level_Info.DataTable_Level_Info" (.CurrentLevelName (Utilities|Struct|BreakStruct_Game_Locations (Variables|/Game/Game/DW1_GameInstance.DW1_GameInstance_C|GetGame%20Location%20and%20Rotation (LocalVariables|GetGameInstance)))))
          (:then
            (bind _output_get_2 (LocalVariables|SetLevelInfo _returnvalue_2))
            (LocalVariables|SetIsDay?%20AddLocal (.IsDay?%20Event (CallFunction|DetermineDayNight)))
            (if (and (Utilities|Select :Index (.Audio (Utilities|Struct|BreakStruct_Level_Info _output_get_2)) :NewEnumerator0 true :NewEnumerator1 true :NewEnumerator2 true :NewEnumerator3 true :NewEnumerator4 true :NewEnumerator5 true :NewEnumerator6 true :NewEnumerator7 true :NewEnumerator8 true :NewEnumerator9 true :NewEnumerator10 true :NewEnumerator11 true :NewEnumerator12 true :NewEnumerator13 true :NewEnumerator14 true :NewEnumerator15 false :NewEnumerator16 false :NewEnumerator17 false :NewEnumerator18 false :NewEnumerator19 false :NewEnumerator21 false :NewEnumerator22 false :NewEnumerator23 false :NewEnumerator25 false :NewEnumerator26 false :NewEnumerator27 false :NewEnumerator28 false :NewEnumerator29 false :NewEnumerator31 false :NewEnumerator32 false :NewEnumerator33 false :NewEnumerator40 false :NewEnumerator41 false :NewEnumerator42 false :NewEnumerator43 false) (Math|Boolean|NotEqual(Boolean) (LocalVariables|GetIsDay?%20PreCalculate) (LocalVariables|GetIsDay?%20AddLocal)))
              (Audio|UpdateAudio))))))))

(fn UpdateLights
  (bind _outactors (Actor|GetAllActorswithInterface "/Game/BluePrints/BPI/BPI_Lighting.BPI_Lighting_C"))
  (for _array_element _outactors
    (Class|BPILighting|LightingonOff(Message) _array_element (.IsDay?%20Event (CallFunction|DetermineDayNight)))))

(fn ForwardTimeExact
  (params (Exact%20Hour :type Integer))
  (LocalVariables|SetExactHour (Math|Integer|Clamp(Integer) Exact%20Hour 0 23))
  (bind _asdw1_game_instance (Utilities|Casting|CastToDW1_GameInstance (Game|GetGameInstance)))
  (bind _output_get (LocalVariables|SetGameInstance _asdw1_game_instance))
  (LocalVariables|SetCurrentHour (Math|Integer|Clamp(Integer) (Utilities|Struct|BreakStruct_Time (Variables|/Game/Game/DW1_GameInstance.DW1_GameInstance_C|GetGame%20Time _output_get)) 0 23))
  (Utilities|FlowControl|Sequence
    (:then_0
      ;[1 1 1 1 100] SET NEW HOUR
      (LocalVariables|SetIsDay?%20PreCalculate (.IsDay?%20Event (CallFunction|DetermineDayNight)))
      (Utilities|Struct|SetmembersinStruct_Time (Variables|/Game/Game/DW1_GameInstance.DW1_GameInstance_C|GetGame%20Time (LocalVariables|GetGameInstance)) (Math|Integer|Clamp(Integer) (LocalVariables|GetExactHour) 0 23))
      (LocalVariables|SetIsDay?%20AddLocal (.IsDay?%20Event (CallFunction|DetermineDayNight)))
      (if (> (LocalVariables|GetCurrentHour) (LocalVariables|GetExactHour))
        (Clock|NewDayFunction)))
    (:then_1
      (Lighting|UpdateLights))
    (:then_2
      (Lighting|SetSunLighting))
    (:then_3
      (Lighting|UpdateSunandSky))
    (:then_4
      ;[1 1 1 1 100] UPDATE AUDIO
      (bind _returnvalue (Class|DataTableFunctionLibrary|DoesDataTableRowExist "/Game/Game/DataTables/Levels/DataTable_Level_Info.DataTable_Level_Info" (.CurrentLevelName (Utilities|Struct|BreakStruct_Game_Locations (Variables|/Game/Game/DW1_GameInstance.DW1_GameInstance_C|GetGame%20Location%20and%20Rotation (LocalVariables|GetGameInstance))))))
      (if _returnvalue
        (bind _returnvalue_2 (Utilities|GetDataTableRow "/Game/Game/DataTables/Levels/DataTable_Level_Info.DataTable_Level_Info" (.CurrentLevelName (Utilities|Struct|BreakStruct_Game_Locations (Variables|/Game/Game/DW1_GameInstance.DW1_GameInstance_C|GetGame%20Location%20and%20Rotation (LocalVariables|GetGameInstance)))))
          (:then
            (if (and (Utilities|Select :Index (.Audio (Utilities|Struct|BreakStruct_Level_Info _returnvalue_2)) :NewEnumerator0 true :NewEnumerator1 true :NewEnumerator2 true :NewEnumerator3 true :NewEnumerator4 true :NewEnumerator5 true :NewEnumerator6 true :NewEnumerator7 true :NewEnumerator8 true :NewEnumerator9 true :NewEnumerator10 true :NewEnumerator11 true :NewEnumerator12 true :NewEnumerator13 true :NewEnumerator14 true :NewEnumerator15 false :NewEnumerator16 false :NewEnumerator17 false :NewEnumerator18 false :NewEnumerator19 false :NewEnumerator21 false :NewEnumerator22 false :NewEnumerator23 false :NewEnumerator25 false :NewEnumerator26 false :NewEnumerator27 false :NewEnumerator28 false :NewEnumerator29 false :NewEnumerator31 false :NewEnumerator32 false :NewEnumerator33 false :NewEnumerator40 false :NewEnumerator41 false :NewEnumerator42 false :NewEnumerator43 false) (Math|Boolean|NotEqual(Boolean) (LocalVariables|GetIsDay?%20PreCalculate) (LocalVariables|GetIsDay?%20AddLocal)))
              (Audio|UpdateAudio))))))))

(fn UpdateAudioLighting
  (bind _asdw1_game_instance (Utilities|Casting|CastToDW1_GameInstance (Game|GetGameInstance)))
  (bind _output_get (LocalVariables|SetGameInstance _asdw1_game_instance))
  (bind _returnvalue (Class|DataTableFunctionLibrary|DoesDataTableRowExist "/Game/Game/DataTables/Levels/DataTable_Level_Info.DataTable_Level_Info" (Utilities|Struct|BreakStruct_Game_Locations (Variables|/Game/Game/DW1_GameInstance.DW1_GameInstance_C|GetGame%20Location%20and%20Rotation _output_get))))
  (if _returnvalue
    (bind _returnvalue_2 (Utilities|GetDataTableRow "/Game/Game/DataTables/Levels/DataTable_Level_Info.DataTable_Level_Info" (Utilities|Struct|BreakStruct_Game_Locations (Variables|/Game/Game/DW1_GameInstance.DW1_GameInstance_C|GetGame%20Location%20and%20Rotation _output_get)))
      (:then
        (LocalVariables|SetLevelInfo _returnvalue_2)
        (if (and (Utilities|Select :Index (Utilities|Struct|BreakStruct_Level_Info (LocalVariables|GetLevelInfo)) :NewEnumerator0 true :NewEnumerator1 true :NewEnumerator2 true :NewEnumerator3 true :NewEnumerator4 true :NewEnumerator5 true :NewEnumerator6 true :NewEnumerator7 true :NewEnumerator8 true :NewEnumerator9 true :NewEnumerator10 true :NewEnumerator11 true :NewEnumerator12 true :NewEnumerator13 true :NewEnumerator14 true :NewEnumerator15 false :NewEnumerator16 false :NewEnumerator17 false :NewEnumerator18 false :NewEnumerator19 false :NewEnumerator21 false :NewEnumerator22 false :NewEnumerator23 false :NewEnumerator25 false :NewEnumerator26 false :NewEnumerator27 false :NewEnumerator28 false :NewEnumerator29 false :NewEnumerator31 false :NewEnumerator32 false :NewEnumerator33 false :NewEnumerator40 false :NewEnumerator41 false :NewEnumerator42 false :NewEnumerator43 false) (Utilities|Select :Index (Math|Integer|Clamp(Integer) (Utilities|Struct|BreakStruct_Time (Variables|/Game/Game/DW1_GameInstance.DW1_GameInstance_C|GetGame%20Time (LocalVariables|GetGameInstance))) 0 23) :Option%200 false :Option%201 false :Option%202 false :Option%203 false :Option%204 false :Option%205 false :Option%206 false :Option%207 false :Option%208 false :Option%209 true :Option%2010 false :Option%2011 false :Option%2012 false :Option%2013 false :Option%2014 false :Option%2015 false :Option%2016 false :Option%2017 false :Option%2018 false :Option%2019 false :Option%2020 false :Option%2021 true :Option%2022 false :Option%2023 false))
          (Audio|UpdateAudio)
          ;[1 1 1 1 100] FADE LIGHTING
          (bind _outactors (Actor|GetAllActorswithInterface "/Game/BluePrints/BPI/BPI_Lighting.BPI_Lighting_C"))
          (for _array_element _outactors
            (Class|BPILighting|LightingFade(Message) _array_element (.IsDay?%20Event (CallFunction|DetermineDayNight)))))))))

(fn UpdateClock
  (Utilities|IsValid (Variables|Widget|GetGameHUD)
    (:Is%20Valid
      (Class|BPIHUDGame|GameHUDClockUpdate(Message) (Variables|Widget|GetGameHUD) :!label _label))
    (:Is%20Not%20Valid
      (bind _foundwidgets (Widget|GetAllWidgetsOfClass "/Game/UI/GameHUD.GameHUD_C" true))
      (for _array_element _foundwidgets
        (Utilities|IsValid _array_element
          (:Is%20Valid
            (Variables|Widget|SetGameHUD _array_element)
            (goto _label)))))))