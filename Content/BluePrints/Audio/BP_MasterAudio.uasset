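; Master music actor that plays and crossfades sequentially between background tracks for levels and battles through one audio component.
; Events fade out, swap the sound returned by lookup functions over the OST data table, then fade back in.
; Level music matches the current level's data-table row, then filters by day/night or game triggers for story variants like Ogremon's theme and Toy Town.
; Battle tracks match type and clamped index.
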(event EventAudioSetBGM
  (bind _returnvalue (Math|Float|MakeLiteralFloat 2.0))
  (bind _audiocomponent (Variables|Components|GetAudioComponent))
  ;[1 1 1 1 200] Set BGM
  ;;[0 1 0.6549 1 100] START
  ;;[0 1 0.6549 1 100] Fade Out
  (Audio|Components|Audio|FadeOut _audiocomponent _returnvalue 0.0 "Linear" :!class /Script/Engine.AudioComponent)
  (Utilities|FlowControl|Delay _returnvalue)
  ;;[0 1 0.6549 1 100] Set Sound
  (Audio|Components|Audio|SetSound _audiocomponent (CallFunction|AudioSetBGMNormal))
  ;;[0 1 0.6549 1 100] Fade In
  (Audio|Components|Audio|FadeIn _audiocomponent _returnvalue 1.0 0.0 "Linear" :!class /Script/Engine.AudioComponent))

(event EventAudioFadeOut
  (params (FadeDuration :type Float%20%28single-precision%29))
  ;[0 1 0.2051 1 100] Fade Out
  (Audio|Components|Audio|FadeOut (Variables|Components|GetAudioComponent) (Math|Float|Clamp(Float) FadeDuration 0.0 2.0) 0.0 "Linear" :!class /Script/Engine.AudioComponent))

(event EventAudioStop
  ;[0 1 0.2051 1 100] STOP
  (Audio|Components|Audio|Stop (Variables|Components|GetAudioComponent)))

(event EventAudioSelectTrack
  (params (Index :type Integer) (Type :type Enum_OST_Names%20Enum :default "NewEnumerator0"))
  (bind _returnvalue (Math|Float|MakeLiteralFloat 0.2))
  (bind _audiocomponent (Variables|Components|GetAudioComponent))
  ;[1 1 1 1 200] Search Track
  ;;[0 1 0.6549 1 100] START
  ;;[0 1 0.6549 1 100] Fade Out
  (Audio|Components|Audio|FadeOut _audiocomponent _returnvalue 0.0 "Linear" :!class /Script/Engine.AudioComponent)
  (Utilities|FlowControl|Delay _returnvalue)
  ;;[0 1 0.6549 1 100] Set Sound
  (Audio|Components|Audio|SetSound _audiocomponent (CallFunction|AudioSetBGMBattle Index Type))
  ;;[0 1 0.6549 1 100] Fade In
  (Audio|Components|Audio|FadeIn _audiocomponent _returnvalue 1.0 0.0 "Linear" :!class /Script/Engine.AudioComponent))

(fn ConstructionScript)

(fn AudioSetBGMNormal
  (bind _asdw1_game_instance (Utilities|Casting|CastToDW1_GameInstance (Game|GetGameInstance))
    (:then
      (LocalVariables|SetGameInstance _asdw1_game_instance)
      ;[1 1 1 1 100] GET LEVEL INFO
      (bind _output_get (LocalVariables|SetCurrentLevel (Utilities|Struct|BreakStruct_Game_Locations (Variables|/Game/Game/DW1_GameInstance.DW1_GameInstance_C|GetGame%20Location%20and%20Rotation (LocalVariables|GetGameInstance)))))
      (bind _returnvalue (Class|DataTableFunctionLibrary|DoesDataTableRowExist "/Game/Game/DataTables/Levels/DataTable_Level_Info.DataTable_Level_Info" _output_get))
      (if _returnvalue
        (bind _returnvalue_2 (Utilities|GetDataTableRow "/Game/Game/DataTables/Levels/DataTable_Level_Info.DataTable_Level_Info" (Utilities|Struct|BreakStruct_Game_Locations (Variables|/Game/Game/DW1_GameInstance.DW1_GameInstance_C|GetGame%20Location%20and%20Rotation (LocalVariables|GetGameInstance))))
          (:then
            (LocalVariables|SetLevel%20Info _returnvalue_2)
            (bind _outrownames (DataTable|GetDataTableRowNames "/Game/Game/DataTables/Audio/DataTable_OST.DataTable_OST"))
            (bind _output_get_2 (LocalVariables|SetNameArray _outrownames))
            (bind _array_element (Utilities|Array|ForEachLoopwithBreak _output_get_2 :!label _label)
              (:LoopBody
                (bind _output_get_3 (LocalVariables|SetNameElement _array_element))
                (bind _returnvalue_3 (Utilities|GetDataTableRow "/Game/Game/DataTables/Audio/DataTable_OST.DataTable_OST" _output_get_3)
                  (:then
                    (bind _output_get_4 (LocalVariables|SetTrackLocal _returnvalue_3))
                    (if (== (Utilities|Struct|BreakStruct_OST _output_get_4) (Utilities|Struct|BreakStruct_Level_Info (LocalVariables|GetLevel%20Info)))
                      (switch Utilities|FlowControl|Switch|SwitchonEnum_OST_Names (Utilities|Struct|BreakStruct_OST (LocalVariables|GetTrackLocal))
                        (:NewEnumerator0
                          ;[0 0.5091 1 1 100] DAY / NIGHT
                          (if (Math|Boolean|Equal(Boolean) (Utilities|Struct|BreakStruct_OST (LocalVariables|GetTrackLocal)) (.IsDay?%20Audio (CallFunction|DetermineDayNight))) :!label _label_2
                            (LocalVariables|SetSuccess? true :!label _label_3)
                            (goto _label Break)))
                        (:NewEnumerator1
                          (goto _label_2))
                        (:NewEnumerator2
                          (goto _label_2))
                        (:NewEnumerator3
                          (goto _label_2))
                        (:NewEnumerator4
                          (goto _label_2))
                        (:NewEnumerator5
                          (goto _label_2))
                        (:NewEnumerator6
                          (goto _label_3))
                        (:NewEnumerator7
                          (goto _label_2))
                        (:NewEnumerator8
                          (goto _label_2))
                        (:NewEnumerator9
                          ;[1 1 1] Great Canyon - Ogremon
                          (if (Utilities|Struct|BreakStruct_Level_Info (LocalVariables|GetLevel%20Info))
                            (if (Math|Boolean|ANDBoolean (.Trigger83-YuramontoldyouabouttheInvisibleBridge (Utilities|Struct|BreakStruct_Game_Triggers (Variables|/Game/Game/DW1_GameInstance.DW1_GameInstance_C|GetGame%20Triggers (LocalVariables|GetGameInstance)))) (not (.Trigger193-BeatenOgremoninGreatCanyon (Utilities|Struct|BreakStruct_Game_Triggers (Variables|/Game/Game/DW1_GameInstance.DW1_GameInstance_C|GetGame%20Triggers (LocalVariables|GetGameInstance))))) (.Trigger215-YuramontoldaboutOgremonandhisbandits (Utilities|Struct|BreakStruct_Game_Triggers (Variables|/Game/Game/DW1_GameInstance.DW1_GameInstance_C|GetGame%20Triggers (LocalVariables|GetGameInstance)))))
                              ;[0.07902 0.2882 1 1 100] Ogremon Theme
                              (bind _array_element_2 (Utilities|Array|ForEachLoopwithBreak (LocalVariables|GetNameArray) :!label _label_4)
                                (:LoopBody
                                  (bind _returnvalue_4 (Utilities|GetDataTableRow "/Game/Game/DataTables/Audio/DataTable_OST.DataTable_OST" _array_element_2)
                                    (:then
                                      (bind _output_get_5 (LocalVariables|SetTrackLocal _returnvalue_4))
                                      (if (Utilities|Enum|Equal(Enum) (Utilities|Struct|BreakStruct_OST _output_get_5) "NewEnumerator42")
                                        (LocalVariables|SetSuccess? true)
                                        (goto _label_4 Break)))))
                                (:Completed
                                  (goto _label Break)))
                              (else
                                (goto _label_2)))
                            (else
                              (goto _label_2))))
                        (:NewEnumerator10
                          (goto _label_2))
                        (:NewEnumerator11
                          (goto _label_2))
                        (:NewEnumerator12
                          (goto _label_2))
                        (:NewEnumerator13
                          (goto _label_2))
                        (:NewEnumerator14
                          (goto _label_2))
                        (:NewEnumerator15
                          ;[1 1 1] Drill Tunnel
                          (if (Utilities|Struct|BreakStruct_Level_Info (LocalVariables|GetLevel%20Info))
                            (if (and (.Trigger15-RecruitedWhamon (Utilities|Struct|BreakStruct_Game_Triggers (Variables|/Game/Game/DW1_GameInstance.DW1_GameInstance_C|GetGame%20Triggers (LocalVariables|GetGameInstance)))) (not (.Trigger195-BeatenOgremoninDrillTunnel (Utilities|Struct|BreakStruct_Game_Triggers (Variables|/Game/Game/DW1_GameInstance.DW1_GameInstance_C|GetGame%20Triggers (LocalVariables|GetGameInstance))))))
                              (goto _label_4)
                              (else
                                (goto _label_3)))
                            (else
                              (goto _label_3))))
                        (:NewEnumerator16
                          ;[1 1 1] Lava Cave
                          (if (.Trigger18-RecruitedMeramon (Utilities|Struct|BreakStruct_Game_Triggers (Variables|/Game/Game/DW1_GameInstance.DW1_GameInstance_C|GetGame%20Triggers (LocalVariables|GetGameInstance))))
                            (LocalVariables|SetTrackLocal "")
                            (goto _label_3)
                            (else
                              (goto _label_3))))
                        (:NewEnumerator17
                          (goto _label_3))
                        (:NewEnumerator18
                          (goto _label_3))
                        (:NewEnumerator19
                          (goto _label_3))
                        (:NewEnumerator21
                          (goto _label_3))
                        (:NewEnumerator22
                          (goto _label_3))
                        (:NewEnumerator23
                          ;[1 1 1] Toy Town
                          (if (== (Utilities|Struct|BreakStruct_OST (LocalVariables|GetTrackLocal)) (select (.Trigger107-ToyTownEventdone (Utilities|Struct|BreakStruct_Game_Triggers (Variables|/Game/Game/DW1_GameInstance.DW1_GameInstance_C|GetGame%20Triggers (LocalVariables|GetGameInstance)))) 1 0))
                            (goto _label_3)))
                        (:NewEnumerator25
                          (goto _label_3))
                        (:NewEnumerator26
                          (goto _label_3))
                        (:NewEnumerator27
                          (goto _label_3))
                        (:NewEnumerator28
                          ;[1 1 1] Secret Beach Cave
                          (if (.Trigger15-RecruitedWhamon (Utilities|Struct|BreakStruct_Game_Triggers (Variables|/Game/Game/DW1_GameInstance.DW1_GameInstance_C|GetGame%20Triggers (LocalVariables|GetGameInstance))))
                            (goto _label_3)
                            (else
                              (goto _label_4))))
                        (:NewEnumerator29
                          ;[1 1 1] Ogre Fortress
                          (if (Utilities|Struct|BreakStruct_Level_Info (LocalVariables|GetLevel%20Info))
                            (if (not (.Trigger194-BeatenOgremoninOgreFortress (Utilities|Struct|BreakStruct_Game_Triggers (Variables|/Game/Game/DW1_GameInstance.DW1_GameInstance_C|GetGame%20Triggers (LocalVariables|GetGameInstance)))))
                              (goto _label_4)
                              (else
                                (goto _label_3)))
                            (else
                              (goto _label_3))))
                        (:NewEnumerator31
                          (goto _label_3))
                        (:NewEnumerator32
                          (goto _label_3))
                        (:NewEnumerator33
                          (goto _label_3))
                        (:NewEnumerator40
                          (goto _label_3))
                        (:NewEnumerator41
                          (goto _label_3))
                        (:NewEnumerator42
                          (goto _label_4))
                        (:NewEnumerator43
                          ;[0.07902 0.2882 1 1 100] Leomon Theme
                          (bind _array_element_3 (Utilities|Array|ForEachLoopwithBreak (LocalVariables|GetNameArray) :!label _label_5)
                            (:LoopBody
                              (bind _returnvalue_5 (Utilities|GetDataTableRow "/Game/Game/DataTables/Audio/DataTable_OST.DataTable_OST" _array_element_3)
                                (:then
                                  (bind _output_get_6 (LocalVariables|SetTrackLocal _returnvalue_5))
                                  (if (Utilities|Enum|Equal(Enum) (Utilities|Struct|BreakStruct_OST _output_get_6) "NewEnumerator43")
                                    (LocalVariables|SetSuccess? true)
                                    (goto _label_5 Break)))))
                            (:Completed
                              (goto _label Break)))))))))
              (:Completed
                (if (and (LocalVariables|GetSuccess?) (Utilities|IsValid (Utilities|Struct|BreakStruct_OST (LocalVariables|GetTrackLocal))))
                  (return (Utilities|Struct|BreakStruct_OST (LocalVariables|GetTrackLocal)))
                  (else
                    (return 0))))))
          (:RowNotFound
            (Development|PrintString (Utilities|String|Append "Level Name NOT FOUND -----> " (Utilities|String|ToString(Name) (Utilities|Struct|BreakStruct_Game_Locations (Variables|/Game/Game/DW1_GameInstance.DW1_GameInstance_C|GetGame%20Location%20and%20Rotation (LocalVariables|GetGameInstance))))) true true "(R=1.000000,G=0.000000,B=0.000000,A=1.000000)" :!label _label_6)
            (return 0)))
        (else
          (goto _label_6))))
    (:CastFailed
      (Development|PrintString "GameInstance FAILED" true true "(R=1.000000,G=0.000000,B=0.000000,A=1.000000)")
      (return 0))))

(fn AudioSetBGMBattle
  (params (BattleIndex :type Integer) (Type :type Enum_OST_Names%20Enum :default "NewEnumerator0"))
  (LocalVariables|SetIndexLocal (Math|Conversions|ToByte(Integer) (Math|Integer|Clamp(Integer) BattleIndex 0 3)))
  (LocalVariables|SetOST_Type Type)
  (bind _outrownames (DataTable|GetDataTableRowNames "/Game/Game/DataTables/Audio/DataTable_OST.DataTable_OST"))
  (bind _output_get (LocalVariables|SetNameArray _outrownames))
  (bind _array_element (Utilities|Array|ForEachLoopwithBreak _output_get :!label _label)
    (:LoopBody
      (bind _output_get_2 (LocalVariables|SetNameElement _array_element))
      (bind _returnvalue (Utilities|GetDataTableRow "/Game/Game/DataTables/Audio/DataTable_OST.DataTable_OST" _output_get_2)
        (:then
          (bind _output_get_3 (LocalVariables|SetTrackLocal _returnvalue))
          (if (and (Utilities|Enum|Equal(Enum) (LocalVariables|GetOST_Type) (.OSTName (Utilities|Struct|BreakStruct_OST _output_get_3))) (== (.Index (Utilities|Struct|BreakStruct_OST _output_get_3)) (LocalVariables|GetIndexLocal)))
            (LocalVariables|SetSuccess? true)
            (goto _label Break)))))
    (:Completed
      (if (and (LocalVariables|GetSuccess?) (Utilities|IsValid (Utilities|Struct|BreakStruct_OST (LocalVariables|GetTrackLocal))))
        (return (Utilities|Struct|BreakStruct_OST (LocalVariables|GetTrackLocal)))
        (else
          (return 0))))))

(fn AudioSelectTrack
  (params (Index :type Integer))
  (LocalVariables|SetIndexLocal Index)
  (bind _outrownames (DataTable|GetDataTableRowNames "/Game/Game/DataTables/Audio/DataTable_OST.DataTable_OST"))
  (LocalVariables|SetNameArray _outrownames)
  (if (Utilities|Array|IsValidIndex (LocalVariables|GetNameArray) (LocalVariables|GetIndexLocal))
    (bind _returnvalue (Utilities|GetDataTableRow "/Game/Game/DataTables/Audio/DataTable_OST.DataTable_OST" (Utilities|Array|Get(acopy) (LocalVariables|GetNameArray) (LocalVariables|GetIndexLocal)))
      (:then
        (LocalVariables|SetTrackLocal _returnvalue)
        (Utilities|IsValid (Utilities|Struct|BreakStruct_OST (LocalVariables|GetTrackLocal))
          (:Is%20Valid
            (return (Utilities|Struct|BreakStruct_OST (LocalVariables|GetTrackLocal))))
          (:Is%20Not%20Valid
            (return 0))))
      (:RowNotFound
        _)))
  (Development|PrintString "Index Not Valid")
  (return 0))