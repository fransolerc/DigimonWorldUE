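; Battle-rules function library for Digimon combat: validates incoming attacks, resolves hits, damage and status effects.
; IsReceveingAttack extracts technique data and ends the attack actor; GetChanceToHit compares a speed-adjusted accuracy to a threshold, with automatic-hit cases.
; CalculateDamage feeds partner or NPC stats into TechniqueCalculateDamage, subtracting HP only for the partner.
; Damage uses data-table specialty factors, offense versus defense or finisher charge, and usually random variance.
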(fn TechniqueCalculateDamage
  (params (TechniqueInfo :type Struct%20Technique%20Info%20Structure) (AttackerOffense :type Integer) (ReceiverDefense :type Integer) (FinisherCharge :type Integer) (ReceiverDigimonName :type Name))
  ;[1 1 1 1 100] VALUES
  (LocalVariables|SetTechniqueInfoLocal TechniqueInfo)
  (LocalVariables|SetAttackerOffenseLocal (Math|Integer|Clamp(Integer) AttackerOffense 1 9999))
  (LocalVariables|SetReceiverDefenseLocal (Math|Integer|Clamp(Integer) ReceiverDefense 1 9999))
  (LocalVariables|SetFinisherChargeLocal (Math|Integer|Clamp(Integer) FinisherCharge 0 80))
  (LocalVariables|SetReceiverDigimonNameLocal ReceiverDigimonName)
  ;[1 1 1 1 100] RECEIVER DIGIMON INFO
  (bind _returnvalue (Class|DataTableFunctionLibrary|DoesDataTableRowExist "/Game/Game/DataTables/DigimonInfo/DataTable_Digimon_Info.DataTable_Digimon_Info" (LocalVariables|GetReceiverDigimonNameLocal)))
  (if _returnvalue
    (bind _returnvalue_2 (Utilities|GetDataTableRow "/Game/Game/DataTables/DigimonInfo/DataTable_Digimon_Info.DataTable_Digimon_Info" (LocalVariables|GetReceiverDigimonNameLocal))
      (:then
        (LocalVariables|SetDigimonInfoLocal _returnvalue_2)
        ;[1 1 1 1 100] SPECIALTY FACTOR
        (bind _output_get (LocalVariables|SetSpecialtyArray (Utilities|Array|MakeArray (.Speciality1 (Utilities|Struct|BreakStruct_Digimon_Info (LocalVariables|GetDigimonInfoLocal))) (.Speciality2 (Utilities|Struct|BreakStruct_Digimon_Info (LocalVariables|GetDigimonInfoLocal))) (.Speciality3 (Utilities|Struct|BreakStruct_Digimon_Info (LocalVariables|GetDigimonInfoLocal))))))
        (for _array_element _output_get
          (LocalVariables|SetEnumIndex _array_element)
          (switch Utilities|FlowControl|Switch|SwitchonEnum_Technique_Element (Utilities|Struct|BreakStruct_Technique_Info (LocalVariables|GetTechniqueInfoLocal))
            (:NewEnumerator1
              (bind _returnvalue_3 (Utilities|GetDataTableRow "/Game/Game/DataTables/DataTable_SpecialtyFactors.DataTable_SpecialtyFactors" "Fire")
                (:then
                  (LocalVariables|SetSpecialtyLocal _returnvalue_3)
                  (LocalVariables|SetSpecialtyFactorCounter (+ (Utilities|Select :Index (LocalVariables|GetEnumIndex) :NewEnumerator1 (.Fire (Utilities|Struct|BreakStruct_SpecialtyFactors (LocalVariables|GetSpecialtyLocal))) :NewEnumerator11 (.Battle (Utilities|Struct|BreakStruct_SpecialtyFactors (LocalVariables|GetSpecialtyLocal))) :NewEnumerator5 (.Air (Utilities|Struct|BreakStruct_SpecialtyFactors (LocalVariables|GetSpecialtyLocal))) :NewEnumerator2 (.Earth (Utilities|Struct|BreakStruct_SpecialtyFactors (LocalVariables|GetSpecialtyLocal))) :NewEnumerator3 (.Ice (Utilities|Struct|BreakStruct_SpecialtyFactors (LocalVariables|GetSpecialtyLocal))) :NewEnumerator9 (.Mech (Utilities|Struct|BreakStruct_SpecialtyFactors (LocalVariables|GetSpecialtyLocal))) :NewEnumerator10 (.Filth (Utilities|Struct|BreakStruct_SpecialtyFactors (LocalVariables|GetSpecialtyLocal))) :NewEnumerator12 (.None (Utilities|Struct|BreakStruct_SpecialtyFactors (LocalVariables|GetSpecialtyLocal)))) (LocalVariables|GetSpecialtyFactorCounter)) :!label _label))))
            (:NewEnumerator11
              (bind _returnvalue_4 (Utilities|GetDataTableRow "/Game/Game/DataTables/DataTable_SpecialtyFactors.DataTable_SpecialtyFactors" "Battle")
                (:then
                  (LocalVariables|SetSpecialtyLocal _returnvalue_4)
                  (goto _label))))
            (:NewEnumerator5
              (bind _returnvalue_5 (Utilities|GetDataTableRow "/Game/Game/DataTables/DataTable_SpecialtyFactors.DataTable_SpecialtyFactors" "Air")
                (:then
                  (LocalVariables|SetSpecialtyLocal _returnvalue_5)
                  (goto _label))))
            (:NewEnumerator2
              (bind _returnvalue_6 (Utilities|GetDataTableRow "/Game/Game/DataTables/DataTable_SpecialtyFactors.DataTable_SpecialtyFactors" "Earth")
                (:then
                  (LocalVariables|SetSpecialtyLocal _returnvalue_6)
                  (goto _label))))
            (:NewEnumerator3
              (bind _returnvalue_7 (Utilities|GetDataTableRow "/Game/Game/DataTables/DataTable_SpecialtyFactors.DataTable_SpecialtyFactors" "Ice")
                (:then
                  (LocalVariables|SetSpecialtyLocal _returnvalue_7)
                  (goto _label))))
            (:NewEnumerator9
              (bind _returnvalue_8 (Utilities|GetDataTableRow "/Game/Game/DataTables/DataTable_SpecialtyFactors.DataTable_SpecialtyFactors" "Mech")
                (:then
                  (LocalVariables|SetSpecialtyLocal _returnvalue_8)
                  (goto _label))))
            (:NewEnumerator10
              (bind _returnvalue_9 (Utilities|GetDataTableRow "/Game/Game/DataTables/DataTable_SpecialtyFactors.DataTable_SpecialtyFactors" "Filth")
                (:then
                  (LocalVariables|SetSpecialtyLocal _returnvalue_9)
                  (goto _label))))
            (:NewEnumerator12
              (LocalVariables|SetSpecialtyFactorCounter (+ (LocalVariables|GetSpecialtyFactorCounter) 10)))))
        (if (Utilities|Struct|BreakStruct_Technique_Info (LocalVariables|GetTechniqueInfoLocal))
          ;[1 1 1 1 100] Finisher Result
          (return (Math|Integer|Clamp(Integer) (Math|Float|Floor (* (Math|Conversions|ToFloat(Integer) (+ (LocalVariables|GetAttackerOffenseLocal) (Utilities|Struct|BreakStruct_Technique_Info (LocalVariables|GetTechniqueInfoLocal)))) (/ (Math|Conversions|ToFloat(Byte) (LocalVariables|GetSpecialtyFactorCounter)) 3e+01) (Math|Float|Clamp(Float) (+ (/ (Math|Conversions|ToFloat(Integer) (- (LocalVariables|GetFinisherChargeLocal) 40)) 4e+01) 1.0) 1.0 2.0) (Math|Random|RandomFloatinRange 0.9 1.1))) 1 9999))
          (else
            ;[1 1 1 1 100] Normal Result
            (if (> (- (LocalVariables|GetAttackerOffenseLocal) (LocalVariables|GetReceiverDefenseLocal)) 500)
              (return (Math|Integer|Clamp(Integer) (Math|Float|Floor (* (Math|Conversions|ToFloat(Integer) (Utilities|Struct|BreakStruct_Technique_Info (LocalVariables|GetTechniqueInfoLocal))) (Math|Float|Clamp(Float) (+ (Math|Float|MakeLiteralFloat 1.0) (/ (- (Math|Conversions|ToFloat(Integer) (LocalVariables|GetAttackerOffenseLocal)) (Math|Conversions|ToFloat(Integer) (LocalVariables|GetReceiverDefenseLocal))) 5e+02)) 0.0 2.0) (/ (Math|Conversions|ToFloat(Byte) (LocalVariables|GetSpecialtyFactorCounter)) 3e+01))) 1 9999))
              (else
                (return (Math|Integer|Clamp(Integer) (Math|Float|Floor (* (Math|Conversions|ToFloat(Integer) (Utilities|Struct|BreakStruct_Technique_Info (LocalVariables|GetTechniqueInfoLocal))) (Math|Float|Clamp(Float) (+ 1.0 (/ (- (Math|Conversions|ToFloat(Integer) (LocalVariables|GetAttackerOffenseLocal)) (Math|Conversions|ToFloat(Integer) (LocalVariables|GetReceiverDefenseLocal))) 5e+02)) 0.0 2.0) (/ (Math|Conversions|ToFloat(Byte) (LocalVariables|GetSpecialtyFactorCounter)) 3e+01) (Math|Random|RandomFloatinRange 0.9 1.1))) 1 9999)))))))
      (:RowNotFound
        _)))
  (Development|PrintString 0 "DigimonName NOT FOUND" true true "(R=1.000000,G=0.000000,B=0.000000,A=1.000000)")
  (return 1))

(fn IsReceveingAttack?
  (params (TechniqueActor :type BP%20Master%20Technique%20Object%20Reference) (Actor :type Actor%20Object%20Reference))
  (LocalVariables|SetBP_AttackMovementLocal TechniqueActor)
  (LocalVariables|SetActorLocal Actor)
  (if (Math|Boolean|ANDBoolean (!= (Components|GetOwner (LocalVariables|GetBP_AttackMovementLocal)) (LocalVariables|GetActorLocal)) (Utilities|IsValid (LocalVariables|GetBP_AttackMovementLocal)) (Variables|/Game/BluePrints/Techniques/BP_MasterTechnique.BP_MasterTechnique_C|GetValid? (LocalVariables|GetBP_AttackMovementLocal)))
    (bind _asdw1_game_instance (Utilities|Casting|CastToDW1_GameInstance (Game|GetGameInstance))
      (:then
        (if (Variables|/Game/Game/DW1_GameInstance.DW1_GameInstance_C|GetIsBattleEvent? _asdw1_game_instance)
          ;[1 1 1 1 100] Get Variables
          (LocalVariables|SetTechniqueLocal (Variables|/Game/BluePrints/Techniques/BP_MasterTechnique.BP_MasterTechnique_C|GetTechniqueInfo (LocalVariables|GetBP_AttackMovementLocal)))
          (LocalVariables|SetOwnerOffenseLocal (Variables|/Game/BluePrints/Techniques/BP_MasterTechnique.BP_MasterTechnique_C|GetOwnerOffense (LocalVariables|GetBP_AttackMovementLocal)))
          (LocalVariables|SetOwnerSpeedLocal (Variables|/Game/BluePrints/Techniques/BP_MasterTechnique.BP_MasterTechnique_C|GetOwnerSpeed (LocalVariables|GetBP_AttackMovementLocal)))
          (LocalVariables|SetFinisherChargeLocal (Variables|/Game/BluePrints/Techniques/BP_MasterTechnique.BP_MasterTechnique_C|GetFinisherCharge (LocalVariables|GetBP_AttackMovementLocal)))
          (LocalVariables|SetLocationLocal (Transformation|GetActorLocation (LocalVariables|GetBP_AttackMovementLocal)))
          (Class|BPITechniques|TechniqueEnd(Message) (LocalVariables|GetBP_AttackMovementLocal))
          (return (Utilities|Select :Index (Utilities|Struct|BreakStruct_Technique_Info (LocalVariables|GetTechniqueLocal)) :NewEnumerator0 true :NewEnumerator1 true :NewEnumerator4 true :NewEnumerator5 true :NewEnumerator6 true :NewEnumerator12 false) (LocalVariables|GetTechniqueLocal) (LocalVariables|GetOwnerOffenseLocal) (LocalVariables|GetOwnerSpeedLocal) (LocalVariables|GetFinisherChargeLocal) (LocalVariables|GetLocationLocal))
          (else
            _)))
      (:CastFailed
        _)))
  (return false "" 0 0 0 "0, 0, 0"))

(fn GetChancetoHit
  (params (TechniqueInfo :type Struct%20Technique%20Info%20Structure) (DigimonName :type Name) (SpeedBuffer :type Integer) (AttackerSpeed :type Integer) (VictimSpeed :type Integer) (IsAttacking? :type Boolean))
  ;[1 1 1 1 100] Values
  (LocalVariables|SetTechniqueInfoLocal TechniqueInfo)
  (LocalVariables|SetDigimonNameLocal DigimonName)
  (LocalVariables|SetSpeedBufferLocal SpeedBuffer)
  (LocalVariables|SetAttackerSpeedLocal (Math|Integer|Clamp(Integer) AttackerSpeed 1 999))
  (LocalVariables|SetVictimSpeedLocal (Math|Integer|Clamp(Integer) VictimSpeed 1 999))
  (LocalVariables|SetIsAttacking?%20Local IsAttacking?)
  ;[1 1 1 1 100] Digimon Info
  (bind _returnvalue (Class|DataTableFunctionLibrary|DoesDataTableRowExist "/Game/Game/DataTables/DigimonInfo/DataTable_Digimon_Info.DataTable_Digimon_Info" (LocalVariables|GetDigimonNameLocal)))
  (if _returnvalue
    (bind _returnvalue_2 (Utilities|GetDataTableRow "/Game/Game/DataTables/DigimonInfo/DataTable_Digimon_Info.DataTable_Digimon_Info" (LocalVariables|GetDigimonNameLocal))
      (:then
        (LocalVariables|SetDigimonInfoLocal _returnvalue_2)
        ;[1 1 1 1 100] ChanceToHit
        (return (Math|Boolean|ORBoolean (Utilities|Select :Index (Utilities|Struct|BreakStruct_Digimon_Info (LocalVariables|GetDigimonInfoLocal)) :NewEnumerator0 true :NewEnumerator1 true :NewEnumerator2 false :NewEnumerator3 false :NewEnumerator4 false :NewEnumerator5 false) (<= (LocalVariables|GetSpeedBufferLocal) 0) (LocalVariables|GetIsAttacking?%20Local) (.IsFinisher? (Utilities|Struct|BreakStruct_Technique_Info (LocalVariables|GetTechniqueInfoLocal))) (> (- (Math|Conversions|ToFloat(Byte) (.Accuracy (Utilities|Struct|BreakStruct_Technique_Info (LocalVariables|GetTechniqueInfoLocal)))) (* (/ (Math|Conversions|ToFloat(Byte) (.Accuracy (Utilities|Struct|BreakStruct_Technique_Info (LocalVariables|GetTechniqueInfoLocal)))) 2.0) (/ (- (Math|Conversions|ToFloat(Integer) (LocalVariables|GetVictimSpeedLocal)) (* (Math|Conversions|ToFloat(Integer) (LocalVariables|GetAttackerSpeedLocal)) 0.1)) 1e+03))) 1e+02))))
      (:RowNotFound
        _)))
  (Development|PrintString 0 "DigimonName NOT VALID")
  (return false))

(fn CalculateDamage
  (params (TechniqueInfo :type Struct%20Technique%20Info%20Structure) (Offense :type Integer) (FinisherCharge :type Integer) (Actor :type Actor%20Object%20Reference))
  ;[1 1 1 1 100] VALUES
  (LocalVariables|SetTechniqueLocal TechniqueInfo)
  (LocalVariables|SetOwnerOffenseLocal (Math|Integer|Clamp(Integer) Offense 1 999))
  (LocalVariables|SetFinisherChargeLocal (Math|Integer|Clamp(Integer) FinisherCharge 0 80))
  (bind _output_get (LocalVariables|SetActorLocal Actor))
  (Utilities|Casting|CastToAI_DigimonPartner _output_get
    (:then
      ;[1 1 1 1 100] RECEIVE DAMAGE PARTNER
      (bind _asdw1_game_instance (Utilities|Casting|CastToDW1_GameInstance (Game|GetGameInstance))
        (:then
          (bind _output_get_2 (LocalVariables|SetGameInstance _asdw1_game_instance))
          (LocalVariables|SetDamageValue (CallFunction|TechniqueCalculateDamage (LocalVariables|GetTechniqueLocal) (LocalVariables|GetOwnerOffenseLocal) (Math|Integer|Clamp(Integer) (+ (.Defense (Utilities|Struct|BreakStruct_Digimon_Partner_Info (Variables|/Game/Game/DW1_GameInstance.DW1_GameInstance_C|GetPartner%20Info _output_get_2))) (Math|Integer|Clamp(Integer) (Utilities|Struct|BreakStruct_Battle_Disks (Variables|/Game/Game/DW1_GameInstance.DW1_GameInstance_C|GetBattleDisks _output_get_2)) 0 (Math|Float|Truncate (* (Math|Conversions|ToFloat(Integer) (.Defense (Utilities|Struct|BreakStruct_Digimon_Partner_Info (Variables|/Game/Game/DW1_GameInstance.DW1_GameInstance_C|GetPartner%20Info _output_get_2)))) 0.3)))) 1 999) (LocalVariables|GetFinisherChargeLocal) (.DigimonName (Utilities|Struct|BreakStruct_Digimon_Partner_Info (Variables|/Game/Game/DW1_GameInstance.DW1_GameInstance_C|GetPartner%20Info _output_get_2)))))
          (Utilities|Struct|SetmembersinStruct_Digimon_Partner_Info (Variables|/Game/Game/DW1_GameInstance.DW1_GameInstance_C|GetPartner%20Info (LocalVariables|GetGameInstance)) (Math|Integer|Clamp(Integer) (- (Utilities|Struct|BreakStruct_Digimon_Partner_Info (Variables|/Game/Game/DW1_GameInstance.DW1_GameInstance_C|GetPartner%20Info (LocalVariables|GetGameInstance))) (LocalVariables|GetDamageValue)) 0 9999))
          (return (LocalVariables|GetDamageValue)))
        (:CastFailed
          _)))
    (:CastFailed
      ;[1 1 1 1 100] RECEIVE DAMAGE NPC
      (bind _asai_npc (Utilities|Casting|CastToAI_NPC _output_get)
        (:then
          (LocalVariables|SetDamageValue (CallFunction|TechniqueCalculateDamage (LocalVariables|GetTechniqueLocal) (LocalVariables|GetOwnerOffenseLocal) (.Defense (Utilities|Struct|BreakStruct_Digimon_NPC_Info (Variables|/Game/AI/Pawn_NPC/AI_NPC.AI_NPC_C|GetNPC_Info _asai_npc))) (LocalVariables|GetFinisherChargeLocal) (.DigimonName (Utilities|Struct|BreakStruct_Digimon_NPC_Info (Variables|/Game/AI/Pawn_NPC/AI_NPC.AI_NPC_C|GetNPC_Info _asai_npc)))))
          (return (LocalVariables|GetDamageValue)))
        (:CastFailed
          _))))
  (return 1))

(fn CalculateEffect
  (params (TechniqueInfo :type Struct%20Technique%20Info%20Structure))
  (bind _output_get (LocalVariables|SetTechniqueInfoLocal TechniqueInfo))
  (if (.IsFinisher? (Utilities|Struct|BreakStruct_Technique_Info _output_get))
    _
    (else
      (switch Utilities|FlowControl|Switch|SwitchonEnum_Technique_Effect (.SpecialEffect (Utilities|Struct|BreakStruct_Technique_Info _output_get))
        (:NewEnumerator0
          _)
        (:NewEnumerator1
          (if (< (Math|Random|RandomIntegerinRange 0 99) (Math|Conversions|ToInteger(Byte) (.EffectChance (Utilities|Struct|BreakStruct_Technique_Info _output_get)))) :!label _label
            (return (Utilities|Struct|BreakStruct_Technique_Info (LocalVariables|GetTechniqueInfoLocal)))
            (else
              _)))
        (:NewEnumerator4
          (goto _label))
        (:NewEnumerator5
          (goto _label))
        (:NewEnumerator6
          (goto _label))
        (:NewEnumerator12
          _))))
  (return "NewEnumerator0"))