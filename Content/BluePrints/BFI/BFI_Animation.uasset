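; Blueprint function library of shared animation helpers for Digimon partner and NPC actors.
; SetAnimation maps a clamped index to a DigimonAnimation flag struct, sends it to the actor or a fallback AnimInstance, and returns the matching sequence length from the Digimon info DataTable, defaulting to one second.
; SetAnimationLocation returns a bone's socket location, spawns attack movement there when attacking, and draws a debug point.
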(fn SetAnimation
  (params (Actor :type Pawn%20Object%20Reference) (Anim%20Instance :type Anim%20Instance%20Object%20Reference) (Index :type Integer))
  ;[1 0.5955 0.5256 1 100] VALUES
  (LocalVariables|SetActorLocal Actor)
  (LocalVariables|SetAnimInstanceLocal Anim%20Instance)
  (LocalVariables|SetIndexLocal (Math|Integer|Clamp(Integer) Index 0 10))
  ;[0.4972 0.8896 1 1 100] SET ANIMATION
  (bind _asai_digimon_partner (Utilities|Casting|CastToAI_DigimonPartner (LocalVariables|GetActorLocal))
    (:then
      (bind _output_get (LocalVariables|SetAI_Partner _asai_digimon_partner))
      (Class|BPIAnimation|SetAnimation(Message) _output_get _output_get (Utilities|Select :Index (LocalVariables|GetIndexLocal) :Option%200 (Utilities|Struct|MakeStruct_Digimon_Animation 0.0 false "0.000000,0.000000,0.000000" 1.0 true) :Option%201 (Utilities|Struct|MakeStruct_Digimon_Animation 0.0 false "0.000000,0.000000,0.000000" 1.0 false true) :Option%202 (Utilities|Struct|MakeStruct_Digimon_Animation 0.0 false "0.000000,0.000000,0.000000" 1.0 false false true) :Option%203 (Utilities|Struct|MakeStruct_Digimon_Animation 0.0 false "0.000000,0.000000,0.000000" 1.0 false false false true) :Option%204 (Utilities|Struct|MakeStruct_Digimon_Animation 0.0 false "0.000000,0.000000,0.000000" 1.0 false false false false true) :Option%205 (Utilities|Struct|MakeStruct_Digimon_Animation 0.0 false "0.000000,0.000000,0.000000" 1.0 false false false false false true) :Option%206 (Utilities|Struct|MakeStruct_Digimon_Animation 0.0 false "0.000000,0.000000,0.000000" 1.0 false false false false false false true) :Option%207 (Utilities|Struct|MakeStruct_Digimon_Animation 0.0 false "0.000000,0.000000,0.000000" 1.0 false false false false false false false true) :Option%208 (Utilities|Struct|MakeStruct_Digimon_Animation 0.0 false "0.000000,0.000000,0.000000" 1.0 false false false false false false false false true) :Option%209 (Utilities|Struct|MakeStruct_Digimon_Animation 0.0 false "0.000000,0.000000,0.000000" 1.0 false false false false false false false false false true) :Option%2010 (Utilities|Struct|MakeStruct_Digimon_Animation 0.0 false)))
      ;[0.9479 0.7134 1 1 100] GET DURATION
      (bind _asdw1_game_instance (Utilities|Casting|CastToDW1_GameInstance (Game|GetGameInstance))
        (:then
          (LocalVariables|SetDigimonNameLocal (Utilities|Struct|BreakStruct_Digimon_Partner_Info (Variables|/Game/Game/DW1_GameInstance.DW1_GameInstance_C|GetPartner%20Info _asdw1_game_instance))))
        (:CastFailed
          (Development|PrintString 0 "Game Instance FAILED")
          (return 1.0))))
    (:CastFailed
      (bind _asai_npc (Utilities|Casting|CastToAI_NPC (LocalVariables|GetActorLocal))
        (:then
          (bind _output_get_2 (LocalVariables|SetAI_NPC _asai_npc))
          (Class|BPIAnimation|SetAnimation(Message) _output_get_2 _output_get_2 (Utilities|Select :Index (LocalVariables|GetIndexLocal) :Option%200 (Utilities|Struct|MakeStruct_Digimon_Animation 0.0 false "0.000000,0.000000,0.000000" 1.0 true) :Option%201 (Utilities|Struct|MakeStruct_Digimon_Animation 0.0 false "0.000000,0.000000,0.000000" 1.0 false true) :Option%202 (Utilities|Struct|MakeStruct_Digimon_Animation 0.0 false "0.000000,0.000000,0.000000" 1.0 false false true) :Option%203 (Utilities|Struct|MakeStruct_Digimon_Animation 0.0 false "0.000000,0.000000,0.000000" 1.0 false false false true) :Option%204 (Utilities|Struct|MakeStruct_Digimon_Animation 0.0 false "0.000000,0.000000,0.000000" 1.0 false false false false true) :Option%205 (Utilities|Struct|MakeStruct_Digimon_Animation 0.0 false "0.000000,0.000000,0.000000" 1.0 false false false false false true) :Option%206 (Utilities|Struct|MakeStruct_Digimon_Animation 0.0 false "0.000000,0.000000,0.000000" 1.0 false false false false false false true) :Option%207 (Utilities|Struct|MakeStruct_Digimon_Animation 0.0 false "0.000000,0.000000,0.000000" 1.0 false false false false false false false true) :Option%208 (Utilities|Struct|MakeStruct_Digimon_Animation 0.0 false "0.000000,0.000000,0.000000" 1.0 false false false false false false false false true) :Option%209 (Utilities|Struct|MakeStruct_Digimon_Animation 0.0 false "0.000000,0.000000,0.000000" 1.0 false false false false false false false false false true) :Option%2010 (Utilities|Struct|MakeStruct_Digimon_Animation 0.0 false)))
          (LocalVariables|SetDigimonNameLocal (Utilities|Struct|BreakStruct_Digimon_NPC_Info (Variables|/Game/AI/Pawn_NPC/AI_NPC.AI_NPC_C|GetNPC_Info (LocalVariables|GetAI_NPC)))))
        (:CastFailed
          (Class|BPIAnimation|SetAnimation(Message) (LocalVariables|GetAnimInstanceLocal) 0 (Utilities|Select :Index (LocalVariables|GetIndexLocal) :Option%200 (Utilities|Struct|MakeStruct_Digimon_Animation 0.0 false "0.000000,0.000000,0.000000" 1.0 true) :Option%201 (Utilities|Struct|MakeStruct_Digimon_Animation 0.0 false "0.000000,0.000000,0.000000" 1.0 false true) :Option%202 (Utilities|Struct|MakeStruct_Digimon_Animation 0.0 false "0.000000,0.000000,0.000000" 1.0 false false true) :Option%203 (Utilities|Struct|MakeStruct_Digimon_Animation 0.0 false "0.000000,0.000000,0.000000" 1.0 false false false true) :Option%204 (Utilities|Struct|MakeStruct_Digimon_Animation 0.0 false "0.000000,0.000000,0.000000" 1.0 false false false false true) :Option%205 (Utilities|Struct|MakeStruct_Digimon_Animation 0.0 false "0.000000,0.000000,0.000000" 1.0 false false false false false true) :Option%206 (Utilities|Struct|MakeStruct_Digimon_Animation 0.0 false "0.000000,0.000000,0.000000" 1.0 false false false false false false true) :Option%207 (Utilities|Struct|MakeStruct_Digimon_Animation 0.0 false "0.000000,0.000000,0.000000" 1.0 false false false false false false false true) :Option%208 (Utilities|Struct|MakeStruct_Digimon_Animation 0.0 false "0.000000,0.000000,0.000000" 1.0 false false false false false false false false true) :Option%209 (Utilities|Struct|MakeStruct_Digimon_Animation 0.0 false "0.000000,0.000000,0.000000" 1.0 false false false false false false false false false true) :Option%2010 (Utilities|Struct|MakeStruct_Digimon_Animation 0.0 false)))
          (return 1.0)))))
  (bind _returnvalue (Class|DataTableFunctionLibrary|DoesDataTableRowExist "/Game/Game/DataTables/DigimonInfo/DataTable_Digimon_Info.DataTable_Digimon_Info" (LocalVariables|GetDigimonNameLocal)))
  (if _returnvalue
    (bind _returnvalue_2 (Utilities|GetDataTableRow "/Game/Game/DataTables/DigimonInfo/DataTable_Digimon_Info.DataTable_Digimon_Info" (LocalVariables|GetDigimonNameLocal))
      (:then
        (bind _output_get_3 (LocalVariables|SetAnimationArray (Utilities|Array|MakeArray (.AnimationAttackShort (Utilities|Struct|BreakStruct_Digimon_Info _returnvalue_2)) (.AnimationAttackLong (Utilities|Struct|BreakStruct_Digimon_Info _returnvalue_2)) (.AnimationAttackSpecial01 (Utilities|Struct|BreakStruct_Digimon_Info _returnvalue_2)) (.AnimationAttackSpecial02 (Utilities|Struct|BreakStruct_Digimon_Info _returnvalue_2)) (.AnimationDamaged (Utilities|Struct|BreakStruct_Digimon_Info _returnvalue_2)) (.AnimationGuard (Utilities|Struct|BreakStruct_Digimon_Info _returnvalue_2)) (.AnimationGetUp (Utilities|Struct|BreakStruct_Digimon_Info _returnvalue_2)) (.AnimationDown (Utilities|Struct|BreakStruct_Digimon_Info _returnvalue_2)) (.AnimationWinGlad (Utilities|Struct|BreakStruct_Digimon_Info _returnvalue_2)) (.AnimationEat (Utilities|Struct|BreakStruct_Digimon_Info _returnvalue_2)))))
        (bind _output_get_4 (LocalVariables|SetSequenceLocal (Utilities|Array|Get(acopy) _output_get_3 (LocalVariables|GetIndexLocal))))
        (Utilities|IsValid _output_get_4
          (:Is%20Valid
            (return (Variables|/Script/Engine.AnimSequenceBase|GetSequenceLength (LocalVariables|GetSequenceLocal))))
          (:Is%20Not%20Valid
            _)))
      (:RowNotFound
        (Development|PrintString 0 (Utilities|String|Append "BFI Animation - " (Utilities|String|ToString(Name) (LocalVariables|GetDigimonNameLocal)) " NOT VALID") :!label _label)))
    (else
      (goto _label)))
  (return 1.0))

(fn SetAnimationLocation
  (params (Actor :type Pawn%20Object%20Reference) (BoneName :type Name) (IsAttacking? :type Boolean) (IsFinisher? :type Boolean))
  (LocalVariables|SetActorLocal Actor)
  (LocalVariables|SetBoneNameLocal BoneName)
  (LocalVariables|SetIsAttacking?Local IsAttacking?)
  (LocalVariables|SetIsFinisher?Local IsFinisher?)
  (bind _asai_digimon_partner (Utilities|Casting|CastToAI_DigimonPartner (LocalVariables|GetActorLocal))
    (:then
      (LocalVariables|SetLocationLocal (Transformation|GetSocketLocation (Variables|/Script/Engine.Character|GetMesh _asai_digimon_partner) (LocalVariables|GetBoneNameLocal)))
      (if (LocalVariables|GetIsAttacking?Local)
        (Default|AttackMovementSpawn _asai_digimon_partner (LocalVariables|GetLocationLocal) (LocalVariables|GetIsFinisher?Local))))
    (:CastFailed
      (bind _asai_npc (Utilities|Casting|CastToAI_NPC (LocalVariables|GetActorLocal))
        (:then
          (LocalVariables|SetLocationLocal (Transformation|GetSocketLocation (Variables|/Script/Engine.Character|GetMesh _asai_npc) (LocalVariables|GetBoneNameLocal)))
          (if (LocalVariables|GetIsAttacking?Local)
            (Default|AttackMovementSpawn _asai_npc (LocalVariables|GetLocationLocal) (LocalVariables|GetIsFinisher?Local))))
        (:CastFailed
          (Development|PrintString 0 "Get Bone Location - ACTOR NOT VALID")
          (return "0, 0, 0")))))
  (Rendering|Debug|DrawDebugPoint 0 (LocalVariables|GetLocationLocal) 8.0 "(R=1.000000,G=0.000000,B=0.000000,A=1.000000)" 8.0)
  (return (LocalVariables|GetLocationLocal)))