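; BP_Battle_Camera is a placeable battle setup actor that positions the player and camera when a battle starts.
; Its construction script applies configurable camera transform, box extent and player marker location to the Camera, Box and Billboard components.
; On BattleSystemStart, it walks the player controller's pawn to the Billboard and, if CameraView is set, blends the view to this actor's camera over one second.
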(event EventBattleSystemStart
  (params (IsRunEnabled? :type Boolean))
  (bind _returnvalue (Game|GetPlayerController 0))
  ;[0.1667 1 1 1 100] Battle Start
  (Utilities|FlowControl|Sequence
    (:then_0
      (AI|Navigation|SimpleMovetoLocation _returnvalue (Transformation|GetWorldLocation (Variables|Default|GetBillboard))))
    (:then_1
      (if (Variables|Default|GetCameraView?)
        (Game|Player|SetViewTargetwithBlend _returnvalue (Components|GetOwner (Variables|Default|GetCamera)) 1.0 "VTBlend_Linear" 0.0 false)))))

(fn ConstructionScript
  (Transformation|SetRelativeLocationAndRotation (Variables|Default|GetCamera) (Variables|Camera|GetCameraLocation) (Variables|Camera|GetCameraRotation) false false)
  (Components|Box|SetBoxExtent (Variables|Default|GetBox) (Variables|Box|GetBoxScale) true)
  (Transformation|SetRelativeLocation (Variables|Default|GetBillboard) (Variables|Player|GetPlayerLocation) false false))