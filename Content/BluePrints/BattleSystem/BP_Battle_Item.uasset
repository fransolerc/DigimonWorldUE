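; BP_Battle_Item is the thrown item visual in battle, flying from the player to the Digimon partner.
; On spawn it looks up the item's data table row for the billboard sprite, then finds the first valid AI_DigimonPartner.
; A timeline lerps XY toward the partner with a separate Z offset.
; It then triggers the partner's item bubble animation, sends the enable-input message to BPI_Battle actors and destroys itself.
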(event EventBattleSystemSpawnItem
  (params (ItemName :type Name :default "None"))
  (bind _returnvalue (Game|GetPlayerCharacter 0))
  (bind _returnvalue_2 (Transformation|GetActorLocation _returnvalue))
  (bind (_x _y _z) (Math|Vector|BreakVector _returnvalue_2))
  ;[1 1 1 1 100] Item Info
  (Utilities|FlowControl|DoOnce false
    (:Completed
      (bind _output_get (Variables|Default|SetItemName ItemName))
      (bind _returnvalue_3 (Class|DataTableFunctionLibrary|DoesDataTableRowExist "/Game/Game/DataTables/Item/DataTable_Item_Info.DataTable_Item_Info" _output_get))
      (if _returnvalue_3
        (bind _returnvalue_4 (Utilities|GetDataTableRow "/Game/Game/DataTables/Item/DataTable_Item_Info.DataTable_Item_Info" (Variables|Default|GetItemName))
          (:then
            (Rendering|Components|Sprite|SetSprite (Variables|Default|GetBillboard) (Utilities|Struct|BreakStruct_Item_Info _returnvalue_4))
            ;[1 1 1 1 100] Search Partner
            (bind _outactors (Actor|GetAllActorsOfClass "/Game/AI/Pawn_Partner/AI_DigimonPartner.AI_DigimonPartner_C"))
            (bind _array_element (Utilities|Array|ForEachLoopwithBreak _outactors :!label _label)
              (:LoopBody
                (bind _output_get_2 (Variables|Default|SetPartner _array_element))
                (Utilities|IsValid _output_get_2
                  (:Is%20Valid
                    (goto _label Break))))
              (:Completed
                (Utilities|IsValid (Variables|Default|GetPartner)
                  (:Is%20Valid
                    ;[1 1 1 1 100] MOVE ITEM SPAWN
                    (bind (_direction _xy _z_2) (Timeline|Línea%20de%20tiempo_0 PlayFromStart)
                      (:Update
                        (Transformation|SetActorLocation self (Math|Vector|MakeVector (Math|Float|Lerp _x (.X (Math|Vector|BreakVector (Transformation|GetActorLocation (Variables|Default|GetPartner)))) _xy) (Math|Float|Lerp _y (.Y (Math|Vector|BreakVector (Transformation|GetActorLocation (Variables|Default|GetPartner)))) _xy) (+ _z _z_2)) false false))
                      (:Finished
                        (Utilities|FlowControl|Sequence :!label _label_2
                          (:then_0
                            ;[1 1 1 1 100] Item Battle Animation
                            (bind _asbattle_partner_item_bubble (Utilities|Casting|CastToBattle_Partner_ItemBubble (UserInterface|GetUserWidgetObject (Variables|/Game/AI/Pawn_Partner/AI_DigimonPartner.AI_DigimonPartner_C|GetWidget_ItemBattle (Variables|Default|GetPartner))))
                              (:then
                                (Default|BattleAnimationFunction _asbattle_partner_item_bubble (Variables|Default|GetItemName)))
                              (:CastFailed
                                (Development|PrintString "Battle Partner Item Bubble NOT FOUND" true true "(R=1.000000,G=0.000000,B=0.000000,A=1.000000)"))))
                          (:then_1
                            (bind _outactors_2 (Actor|GetAllActorswithInterface "/Game/BluePrints/BPI/BPI_Battle.BPI_Battle_C"))
                            (for _array_element_2 _outactors_2
                              (Class|BPIBattle|BattleSystemEnableInput(Message) _array_element_2)))
                          (:then_2
                            ;[1 1 1 1 100] DESTROY
                            (Actor|DestroyActor self :!label _label_3))))))
                  (:Is%20Not%20Valid
                    (goto _label_2))))))
          (:RowNotFound
            (Development|PrintString (Utilities|String|Append "NOT FOUND -----> " (Utilities|String|ToString(Name) (Variables|Default|GetItemName))) true true "(R=1.000000,G=0.000000,B=0.000000,A=1.000000)" :!label _label_4)
            (goto _label_3)))
        (else
          (goto _label_4))))))

(fn ConstructionScript)