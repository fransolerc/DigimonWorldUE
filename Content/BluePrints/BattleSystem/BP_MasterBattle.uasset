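; BP_MasterBattle is the battle manager actor that handles battle flow and player input during Digimon fights.
; Input actions are relayed through interfaces to battle HUD or pause menu widgets, and menu-chosen items spawn as battle item actors.
; BattleSystem events run macros for start, victory, escape and partner death, updating the game instance and messaging AI, audio, dialogue and level streaming.
; While active, Tick turns the player to face the partner.
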(event EventTick
  (params (DeltaSeconds :type Float%20%28single-precision%29))
  (bind _returnvalue (Game|GetPlayerCharacter 0))
  ;[1 1 1 1 100] ROTATE PLAYER
  (Transformation|SetActorRotation _returnvalue (Math|Rotator|MakeRotator 0.0 0.0 (.Yaw (Math|Rotator|BreakRotator (Math|Rotator|FindLookatRotation (Transformation|GetActorLocation _returnvalue) (Transformation|GetActorLocation (Variables|Partner|GetPartner))))))))

(event EventBattleSystemStart
  (params (IsRunEnabled? :type Boolean))
  ;[0.1667 1 1 1 100] Battle Events
  (Utilities|BattleMacroStart IsRunEnabled?))

(event EventBattleSystemSpawnItem
  (params (ItemName :type Name :default "None"))
  ;[1 0.4271 0.9344 1 100] Spawn Item from Menu
  (CallFunction|SpawnItem ItemName)
  (CallFunction|LockInput false))

(event EventBattleSystemDeath2
  ;[0.1667 1 1 1 100] Battle Events
  (Utilities|BattleMacroDeath))

(event EventBattleSystemDeath1
  ;[0.1667 1 1 1 100] Battle Events
  (CallFunction|LockInput true)
  (Actor|Tick|SetActorTickEnabled false)
  (Variables|Battle|SetCanOpenInventory? false))

(event EventBattleSystemEnableInput
  ;[0 1 0.06661 1 200] INPUT
  ;;[0.3801 1 0 1 100] ENABLE INPUT
  (CallFunction|LockInput false)
  (Variables|Battle|SetCanOpenInventory? true))

(event EventBattleSystemCheckEnemies
  ;[0.1667 1 1 1 100] Battle Events
  (if (CallFunction|CheckEnemiesinBattle)
    (Utilities|BattleMacroEnd)))

(event EventBattleSystemRun
  ;[0.1667 1 1 1 100] Battle Events
  (if (CallFunction|CheckifCanRun)
    (Utilities|BattleMacroRun)))

(event Input|ActionEvents|InputActionCancel[Circle]
  (params (Key :type Key%20Structure))
  ;[0 1 0.06661 1 200] INPUT
  ;;[1 1 1 1 100] CANCEL
  (:Pressed
    (if (Game|IsGamePaused)
      (bind _foundwidgets (Class|WidgetBlueprintLibrary|GetAllWidgetswithInterface "/Game/BluePrints/BPI/BPI_HUD_Game.BPI_HUD_Game_C" true))
      (for _array_element _foundwidgets
        (Class|BPIHUDGame|PauseMenuCancel(Message) _array_element))
      (else
        (Development|PrintString "Hello")))))

(event Input|ActionEvents|InputActionKeyUp
  (params (Key :type Key%20Structure))
  ;[0 1 0.06661 1 200] INPUT
  ;;[1 1 1 1 100] UP/DOWN/RIGHT/LEFT
  (:Pressed
    (if (Game|IsGamePaused)
      (bind _foundwidgets (Class|WidgetBlueprintLibrary|GetAllWidgetswithInterface "/Game/BluePrints/BPI/BPI_HUD_Game.BPI_HUD_Game_C" true))
      (for _array_element _foundwidgets
        (Class|BPIHUDGame|PauseMenuUp(Message) _array_element)))))

(event Input|ActionEvents|InputActionKeyDown
  (params (Key :type Key%20Structure))
  ;[0 1 0.06661 1 200] INPUT
  ;;[1 1 1 1 100] UP/DOWN/RIGHT/LEFT
  (:Pressed
    (if (Game|IsGamePaused)
      (bind _foundwidgets (Class|WidgetBlueprintLibrary|GetAllWidgetswithInterface "/Game/BluePrints/BPI/BPI_HUD_Game.BPI_HUD_Game_C" true))
      (for _array_element _foundwidgets
        (Class|BPIHUDGame|PauseMenuDown(Message) _array_element)))))

(event Input|ActionEvents|InputActionKeyLeft
  (params (Key :type Key%20Structure))
  ;[0 1 0.06661 1 200] INPUT
  ;;[1 1 1 1 100] UP/DOWN/RIGHT/LEFT
  (:Pressed
    (if (Game|IsGamePaused)
      (bind _foundwidgets (Class|WidgetBlueprintLibrary|GetAllWidgetswithInterface "/Game/BluePrints/BPI/BPI_HUD_Game.BPI_HUD_Game_C" true))
      (for _array_element _foundwidgets
        (Class|BPIHUDGame|PauseMenuLeft(Message) _array_element))
      (else
        (bind _foundwidgets_2 (Class|WidgetBlueprintLibrary|GetAllWidgetswithInterface "/Game/BluePrints/BPI/BPI_HUD_Battle.BPI_HUD_Battle_C" true))
        (for _array_element_2 _foundwidgets_2
          (Class|BPIHUDBattle|BattleHUDBattleCommandsLeft(Message) _array_element_2))))))

(event Input|ActionEvents|InputActionKeyRight
  (params (Key :type Key%20Structure))
  ;[0 1 0.06661 1 200] INPUT
  ;;[1 1 1 1 100] UP/DOWN/RIGHT/LEFT
  (:Pressed
    (if (Game|IsGamePaused)
      (bind _foundwidgets (Class|WidgetBlueprintLibrary|GetAllWidgetswithInterface "/Game/BluePrints/BPI/BPI_HUD_Game.BPI_HUD_Game_C" true))
      (for _array_element _foundwidgets
        (Class|BPIHUDGame|PauseMenuRight(Message) _array_element))
      (else
        (bind _foundwidgets_2 (Class|WidgetBlueprintLibrary|GetAllWidgetswithInterface "/Game/BluePrints/BPI/BPI_HUD_Battle.BPI_HUD_Battle_C" true))
        (for _array_element_2 _foundwidgets_2
          (Class|BPIHUDBattle|BattleHUDBattleCommandsRight(Message) _array_element_2))))))

(event Input|ActionEvents|InputActionInteraction[Cross]
  (params (Key :type Key%20Structure))
  ;[0 1 0.06661 1 200] INPUT
  ;;[1 1 1 1 100] INTERACTION
  (:Pressed
    (if (Game|IsGamePaused)
      (bind _foundwidgets (Class|WidgetBlueprintLibrary|GetAllWidgetswithInterface "/Game/BluePrints/BPI/BPI_HUD_Game.BPI_HUD_Game_C" true))
      (for _array_element _foundwidgets
        (Class|BPIHUDGame|PauseMenuInteraction(Message) _array_element))
      (else
        (bind _foundwidgets_2 (Class|WidgetBlueprintLibrary|GetAllWidgetswithInterface "/Game/BluePrints/BPI/BPI_HUD_Battle.BPI_HUD_Battle_C" true))
        (for _array_element_2 _foundwidgets_2
          (Class|BPIHUDBattle|BattleHUDBattleCommandsInteraction(Message) _array_element_2))))))

(event Input|ActionEvents|InputActionPauseMenu[Start]
  (params (Key :type Key%20Structure))
  ;[0 1 0.06661 1 200] INPUT
  ;;[1 1 1 1 100] PAUSE MENU
  (:Pressed
    (if (Game|IsGamePaused)
      (bind _foundwidgets (Class|WidgetBlueprintLibrary|GetAllWidgetswithInterface "/Game/BluePrints/BPI/BPI_HUD_Game.BPI_HUD_Game_C" true))
      (for _array_element _foundwidgets
        (Class|BPIHUDGame|PauseMenuResume(Message) _array_element))
      (else
        (bind _returnvalue (UserInterface|CreateWidget "/Game/UI/GameHUD_Pause.GameHUD_Pause_C"))
        (UserInterface|Viewport|AddtoViewport _returnvalue 99)))))

(event Input|ActionEvents|InputActionOpenMenu[Triangle]
  (params (Key :type Key%20Structure))
  ;[0 1 0.06661 1 200] INPUT
  ;;[0.3291 0.7119 1 1 100] INVENTORY MENU
  (:Pressed
    (if (Variables|Battle|GetCanOpenInventory?)
      (CallFunction|LockInput true)
      (bind _foundwidgets (Class|WidgetBlueprintLibrary|GetAllWidgetswithInterface "/Game/BluePrints/BPI/BPI_HUD_Battle.BPI_HUD_Battle_C" true))
      (for _array_element _foundwidgets
        (Class|BPIHUDBattle|BattleHUDInventory(Message) _array_element)))))

(event Input|ActionEvents|InputActionRightTrigger
  (params (Key :type Key%20Structure))
  ;[0 1 0.06661 1 200] INPUT
  ;;[0.4133 1 0.9402 1 100] FINISHER
  (:Pressed
    (if (CallFunction|IsAlive?)
      (bind _foundwidgets (Class|WidgetBlueprintLibrary|GetAllWidgetswithInterface "/Game/BluePrints/BPI/BPI_HUD_Battle.BPI_HUD_Battle_C" true))
      (for _array_element _foundwidgets
        (Class|BPIHUDBattle|BattleHUDFinisherRightTrigger(Message) _array_element)))))

(event Input|ActionEvents|InputActionLeftTrigger
  (params (Key :type Key%20Structure))
  ;[0 1 0.06661 1 200] INPUT
  ;;[0.4133 1 0.9402 1 100] FINISHER
  (:Pressed
    (if (CallFunction|IsAlive?)
      (bind _foundwidgets (Class|WidgetBlueprintLibrary|GetAllWidgetswithInterface "/Game/BluePrints/BPI/BPI_HUD_Battle.BPI_HUD_Battle_C" true))
      (for _array_element _foundwidgets
        (Class|BPIHUDBattle|BattleHUDFinisherLeftTrigger(Message) _array_element)))))

(event Input|ActionEvents|InputActionFinisherMovement[Square]
  (params (Key :type Key%20Structure))
  ;[0 1 0.06661 1 200] INPUT
  ;;[0.4133 1 0.9402 1 100] FINISHER
  (:Pressed
    (if (CallFunction|IsAlive?)
      (bind _foundwidgets (Class|WidgetBlueprintLibrary|GetAllWidgetswithInterface "/Game/BluePrints/BPI/BPI_HUD_Battle.BPI_HUD_Battle_C" true))
      (for _array_element _foundwidgets
        (Class|BPIHUDBattle|BattleHUDFinisherInteraction(Message) _array_element)))))

(fn ConstructionScript)

(fn IsAlive?
  (bind _asdw1_game_instance (Utilities|Casting|CastToDW1_GameInstance (Game|GetGameInstance))
    (:then
      (return (> (Utilities|Struct|BreakStruct_Digimon_Partner_Info (Variables|/Game/Game/DW1_GameInstance.DW1_GameInstance_C|GetPartner%20Info _asdw1_game_instance)) 0)))
    (:CastFailed
      (return false))))

(fn CheckifCanRun
  (bind _asdw1_game_instance (Utilities|Casting|CastToDW1_GameInstance (Game|GetGameInstance))
    (:then
      (LocalVariables|SetGameInstance _asdw1_game_instance)
      (bind _output_get (LocalVariables|SetBooleanLocal (and (Variables|Battle|GetIsRunEnabled?) (> (Utilities|Struct|BreakStruct_Digimon_Partner_Info (Variables|/Game/Game/DW1_GameInstance.DW1_GameInstance_C|GetPartner%20Info (LocalVariables|GetGameInstance))) 0))))
      (return _output_get))
    (:CastFailed
      (return false))))

(fn CheckEnemiesinBattle
  ;[1 1 1 1 100] Comment
  (bind _outactors (Actor|GetAllActorsOfClass "/Game/AI/Pawn_NPC/AI_NPC.AI_NPC_C"))
  (for _array_element _outactors
    (bind _output_get (LocalVariables|SetNPC_Local _array_element))
    (Utilities|IsValid _output_get
      (:Is%20Valid
        (if (> (Variables|/Game/AI/Pawn_NPC/AI_NPC.AI_NPC_C|GetCurrent%20HP (LocalVariables|GetNPC_Local)) 0)
          (Math|Integer|IncrementInt (LocalVariables|GetCounter))))))
  (return (<= (LocalVariables|GetCounter) 0)))

(fn LockInput
  (params (Lock? :type Boolean))
  (bind _returnvalue (Game|GetPlayerController 0))
  (bind _self self)
  (if Lock?
    (Input|DisableInput _self _returnvalue)
    (else
      (Input|EnableInput _self _returnvalue))))

(fn SpawnItem
  (params (ItemName :type Name))
  (bind _output_get (LocalVariables|SetItemNameLocal ItemName))
  (bind _returnvalue (Class|DataTableFunctionLibrary|DoesDataTableRowExist "/Game/Game/DataTables/Item/DataTable_Item_Info.DataTable_Item_Info" _output_get))
  (if _returnvalue
    (Utilities|FlowControl|Sequence
      (:then_0
        (Variables|Battle|SetCanOpenInventory? false))
      (:then_1
        (bind _foundwidgets (Class|WidgetBlueprintLibrary|GetAllWidgetswithInterface "/Game/BluePrints/BPI/BPI_HUD_Battle.BPI_HUD_Battle_C" true))
        (for _array_element _foundwidgets
          (Class|BPIHUDBattle|BattleHUDDeathCountdownPause(Message) _array_element)))
      (:then_2
        (bind _returnvalue_2 (Game|SpawnActorfromClass "/Game/BluePrints/BattleSystem/BP_Battle_Item.BP_Battle_Item_C" (Math|Transform|MakeTransform (Transformation|GetActorLocation (Game|GetPlayerCharacter 0))) "AlwaysSpawn" self 0))
        (Class|BPIBattle|BattleSystemSpawnItem(Message) _returnvalue_2 (LocalVariables|GetItemNameLocal))))
    (else
      (Development|PrintString "ITEM INFO NOT FOUND")
      (Variables|Battle|SetCanOpenInventory? true))))