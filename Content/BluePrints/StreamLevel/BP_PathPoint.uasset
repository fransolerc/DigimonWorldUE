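; BP_PathPoint is a typed point marker actor, with Location, Monitor, Item and NPC as its types.
; Its construction script draws a short-lived debug sphere at the actor's location, colored by type.
; A custom event handles only the Item type, checking for ItemName in the item info DataTable and fetching that row, with nothing done with the result.
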(event Custom|CustomEvent_0
  (bind _itemname (Variables|Item|GetItemName))
  (switch Utilities|FlowControl|Switch|SwitchonEnum_PathPoint (Variables|Enum|GetType)
    (:NewEnumerator2
      (bind _returnvalue (Class|DataTableFunctionLibrary|DoesDataTableRowExist "/Game/Game/DataTables/Item/DataTable_Item_Info.DataTable_Item_Info" _itemname))
      (if _returnvalue
        (Utilities|GetDataTableRow "/Game/Game/DataTables/Item/DataTable_Item_Info.DataTable_Item_Info" _itemname)))))

(fn ConstructionScript
  (Rendering|Debug|DrawDebugSphere (Transformation|GetActorLocation self) 2e+02 12 (Utilities|Select :Index (Variables|Enum|GetType) :NewEnumerator0 "(R=1.000000,G=0.669426,B=0.000000,A=1.000000)" :NewEnumerator1 "(R=0.647162,G=0.000000,B=1.000000,A=1.000000)" :NewEnumerator2 "(R=0.094678,G=1.000000,B=0.000000,A=1.000000)" :NewEnumerator3 "(R=1.000000,G=0.000000,B=0.008376,A=1.000000)") 2.0 2.0))