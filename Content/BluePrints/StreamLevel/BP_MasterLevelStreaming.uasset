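; Master level streamer that swaps map levels from a data table row and index, teleporting player and Digimon partner to that entry.
; Normal requests pass a DoOnce and battle/streaming checks, which the run-from-battle event bypasses.
; LevelStreamingMacro locks input, dialogue and time behind a loading screen, clears actors and widgets, then respawns items, monitors and saved poop.
; It finally updates camera, audio and HUD, with a separate ending for trigger-100 events.
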(event EventLevelStreaming
  (params (LevelName :type Name :default "None") (Index :type Integer))
  ;[0.1357 1 0.4151 1 100] Level Streaming
  (Utilities|FlowControl|DoOnce false :!label _label
    (:Completed
      (Variables|Level|SetLoad%20Level%20Name LevelName)
      (Variables|Level|SetLevelIndex Index)
      (bind _asdw1_game_instance (Utilities|Casting|CastToDW1_GameInstance (Game|GetGameInstance))
        (:then
          (if (and (not (Variables|/Game/Game/DW1_GameInstance.DW1_GameInstance_C|GetIsBattleEvent? _asdw1_game_instance)) (not (Variables|/Game/Game/DW1_GameInstance.DW1_GameInstance_C|GetIsLevelStreaming? _asdw1_game_instance)))
            (bind _returnvalue (Class|DataTableFunctionLibrary|DoesDataTableRowExist "/Game/Game/DataTables/Levels/DataTable_Level_Info.DataTable_Level_Info" (Variables|Level|GetLoad%20Level%20Name)))
            (if _returnvalue
              (bind _returnvalue_2 (Utilities|GetDataTableRow "/Game/Game/DataTables/Levels/DataTable_Level_Info.DataTable_Level_Info" (Variables|Level|GetLoad%20Level%20Name))
                (:then
                  (bind _output_get (Variables|Level|SetLevelLoad%20Info _returnvalue_2))
                  (if (Math|Boolean|ANDBoolean (Utilities|IsValid (Class|GameplayStatics|GetStreamingLevel (Variables|Level|GetLoad%20Level%20Name))) (== (Utilities|Array|Length (.PlayerTransform (Utilities|Struct|BreakStruct_Level_Info _output_get))) (Utilities|Array|Length (.PartnerTransform (Utilities|Struct|BreakStruct_Level_Info _output_get)))) (Utilities|Array|IsValidIndex (.PlayerTransform (Utilities|Struct|BreakStruct_Level_Info _output_get)) (Variables|Level|GetLevelIndex)) (Utilities|Array|IsValidIndex (.PartnerTransform (Utilities|Struct|BreakStruct_Level_Info _output_get)) (Variables|Level|GetLevelIndex)))
                    (Utilities|LevelStreamingMacro
                      (:Reset
                        (Variables|Level|SetLevelIndex 0)
                        (goto _label Reset)))
                    (else
                      (Development|PrintString "LEVEL TO LOAD/UNLOAD NOT VALID")
                      (goto _label Reset))))
                (:RowNotFound
                  _)))
            (Development|PrintString "Level Streaming NOT FOUND" true true "(R=1.000000,G=0.000000,B=0.000000,A=1.000000)")
            (goto _label Reset)
            (else
              _)))
        (:CastFailed
          _))
      (Development|PrintString "LEVEL STREAMING DISABLED" true true "(R=1.000000,G=0.000000,B=0.000000,A=1.000000)" 4.0)
      (goto _label Reset))))

(event EventLevelStreamingRunfromBattle
  (params (LevelName :type Name :default "None") (Index :type Integer))
  ;[1 0.7773 0.3345 1 100] Run From Battle
  (Variables|Level|SetLoad%20Level%20Name LevelName)
  (Variables|Level|SetLevelIndex Index)
  ;[0.1357 1 0.4151 1 100] Level Streaming
  (bind _returnvalue (Class|DataTableFunctionLibrary|DoesDataTableRowExist "/Game/Game/DataTables/Levels/DataTable_Level_Info.DataTable_Level_Info" (Variables|Level|GetLoad%20Level%20Name)))
  (if _returnvalue
    (bind _returnvalue_2 (Utilities|GetDataTableRow "/Game/Game/DataTables/Levels/DataTable_Level_Info.DataTable_Level_Info" (Variables|Level|GetLoad%20Level%20Name))
      (:then
        (bind _output_get (Variables|Level|SetLevelLoad%20Info _returnvalue_2))
        (if (Math|Boolean|ANDBoolean (Utilities|IsValid (Class|GameplayStatics|GetStreamingLevel (Variables|Level|GetLoad%20Level%20Name))) (== (Utilities|Array|Length (.PlayerTransform (Utilities|Struct|BreakStruct_Level_Info _output_get))) (Utilities|Array|Length (.PartnerTransform (Utilities|Struct|BreakStruct_Level_Info _output_get)))) (Utilities|Array|IsValidIndex (.PlayerTransform (Utilities|Struct|BreakStruct_Level_Info _output_get)) (Variables|Level|GetLevelIndex)) (Utilities|Array|IsValidIndex (.PartnerTransform (Utilities|Struct|BreakStruct_Level_Info _output_get)) (Variables|Level|GetLevelIndex)))
          (Utilities|LevelStreamingMacro
            (:Reset
              (Variables|Level|SetLevelIndex 0)
              (Utilities|FlowControl|DoOnce false) ; enters at Reset
            ))
          (else
            (Development|PrintString "LEVEL TO LOAD/UNLOAD NOT VALID")
            (Utilities|FlowControl|DoOnce false) ; enters at Reset
          )))
      (:RowNotFound
        (Development|PrintString "Level Streaming NOT FOUND" true true "(R=1.000000,G=0.000000,B=0.000000,A=1.000000)" :!label _label)
        (Utilities|FlowControl|DoOnce false) ; enters at Reset
      ))
    (else
      (goto _label))))

(fn ConstructionScript)

(fn SpawnPoop
  (bind _asdw1_game_instance (Utilities|Casting|CastToDW1_GameInstance (Game|GetGameInstance)))
  (bind _output_get (LocalVariables|SetGameInstance _asdw1_game_instance))
  (bind _output_get_2 (LocalVariables|SetPoopArray (Utilities|Array|MakeArray (.PoopSlot0 (Utilities|Struct|BreakStruct_Poop_Slots (Variables|/Game/Game/DW1_GameInstance.DW1_GameInstance_C|GetPoop%20Array _output_get))) (.PoopSlot1 (Utilities|Struct|BreakStruct_Poop_Slots (Variables|/Game/Game/DW1_GameInstance.DW1_GameInstance_C|GetPoop%20Array _output_get))) (.PoopSlot2 (Utilities|Struct|BreakStruct_Poop_Slots (Variables|/Game/Game/DW1_GameInstance.DW1_GameInstance_C|GetPoop%20Array _output_get))) (.PoopSlot3 (Utilities|Struct|BreakStruct_Poop_Slots (Variables|/Game/Game/DW1_GameInstance.DW1_GameInstance_C|GetPoop%20Array _output_get))) (.PoopSlot4 (Utilities|Struct|BreakStruct_Poop_Slots (Variables|/Game/Game/DW1_GameInstance.DW1_GameInstance_C|GetPoop%20Array _output_get))) (.PoopSlot5 (Utilities|Struct|BreakStruct_Poop_Slots (Variables|/Game/Game/DW1_GameInstance.DW1_GameInstance_C|GetPoop%20Array _output_get))) (.PoopSlot6 (Utilities|Struct|BreakStruct_Poop_Slots (Variables|/Game/Game/DW1_GameInstance.DW1_GameInstance_C|GetPoop%20Array _output_get))) (.PoopSlot7 (Utilities|Struct|BreakStruct_Poop_Slots (Variables|/Game/Game/DW1_GameInstance.DW1_GameInstance_C|GetPoop%20Array _output_get))) (.PoopSlot8 (Utilities|Struct|BreakStruct_Poop_Slots (Variables|/Game/Game/DW1_GameInstance.DW1_GameInstance_C|GetPoop%20Array _output_get))) (.PoopSlot9 (Utilities|Struct|BreakStruct_Poop_Slots (Variables|/Game/Game/DW1_GameInstance.DW1_GameInstance_C|GetPoop%20Array _output_get))) (.PoopSlot10 (Utilities|Struct|BreakStruct_Poop_Slots (Variables|/Game/Game/DW1_GameInstance.DW1_GameInstance_C|GetPoop%20Array _output_get))) (.PoopSlot11 (Utilities|Struct|BreakStruct_Poop_Slots (Variables|/Game/Game/DW1_GameInstance.DW1_GameInstance_C|GetPoop%20Array _output_get))) (.PoopSlot12 (Utilities|Struct|BreakStruct_Poop_Slots (Variables|/Game/Game/DW1_GameInstance.DW1_GameInstance_C|GetPoop%20Array _output_get))) (.PoopSlot13 (Utilities|Struct|BreakStruct_Poop_Slots (Variables|/Game/Game/DW1_GameInstance.DW1_GameInstance_C|GetPoop%20Array _output_get))) (.PoopSlot14 (Utilities|Struct|BreakStruct_Poop_Slots (Variables|/Game/Game/DW1_GameInstance.DW1_GameInstance_C|GetPoop%20Array _output_get))) (.PoopSlot15 (Utilities|Struct|BreakStruct_Poop_Slots (Variables|/Game/Game/DW1_GameInstance.DW1_GameInstance_C|GetPoop%20Array _output_get))) (.PoopSlot16 (Utilities|Struct|BreakStruct_Poop_Slots (Variables|/Game/Game/DW1_GameInstance.DW1_GameInstance_C|GetPoop%20Array _output_get))) (.PoopSlot17 (Utilities|Struct|BreakStruct_Poop_Slots (Variables|/Game/Game/DW1_GameInstance.DW1_GameInstance_C|GetPoop%20Array _output_get))) (.PoopSlot18 (Utilities|Struct|BreakStruct_Poop_Slots (Variables|/Game/Game/DW1_GameInstance.DW1_GameInstance_C|GetPoop%20Array _output_get))) (.PoopSlot19 (Utilities|Struct|BreakStruct_Poop_Slots (Variables|/Game/Game/DW1_GameInstance.DW1_GameInstance_C|GetPoop%20Array _output_get))))))
  (for (_array_element _array_index) _output_get_2
    (if (Utilities|Name|Equal(Name) (.CurrentLevel (Utilities|Struct|BreakStruct_Poop_Info _array_element)) (Variables|Level|GetLoad%20Level%20Name))
      (Game|SpawnActorfromClass "/Game/BluePrints/Interactible/BP_Poop.BP_Poop_C" (Math|Transform|MakeTransform (.Location (Utilities|Struct|BreakStruct_Poop_Info _array_element))) "AlwaysSpawn" 0 _array_index (.Size (Utilities|Struct|BreakStruct_Poop_Info _array_element)) 0))))

(fn LevelIsValid?
  (params (Level%20Name :type Name))
  (bind _output_get (LocalVariables|SetLevelName_Local Level%20Name))
  (return (Utilities|IsValid (Class|GameplayStatics|GetStreamingLevel _output_get))))

(fn LevelFunction
  (bind _asdw1_game_instance (Utilities|Casting|CastToDW1_GameInstance (Game|GetGameInstance))
    (:then
      (bind _output_get (LocalVariables|SetGameInstanceLocal _asdw1_game_instance))
      (bind _output_get_2 (LocalVariables|SetPreviousLevelName (.CurrentLevelName (Utilities|Struct|BreakStruct_Game_Locations (Variables|/Game/Game/DW1_GameInstance.DW1_GameInstance_C|GetGame%20Location%20and%20Rotation _output_get)))))
      (LocalVariables|SetPreviousLevelIndex (.CurrentLevelIndex (Utilities|Struct|BreakStruct_Game_Locations (Variables|/Game/Game/DW1_GameInstance.DW1_GameInstance_C|GetGame%20Location%20and%20Rotation _output_get))))
      (bind _returnvalue (Class|DataTableFunctionLibrary|DoesDataTableRowExist "/Game/Game/DataTables/Levels/DataTable_Level_Info.DataTable_Level_Info" _output_get_2))
      (if _returnvalue
        (bind _returnvalue_2 (Utilities|GetDataTableRow "/Game/Game/DataTables/Levels/DataTable_Level_Info.DataTable_Level_Info" (LocalVariables|GetPreviousLevelName))
          (:then
            (Variables|Level|SetLevelPreviousInfo _returnvalue_2)
            (if (Utilities|IsValid (Class|GameplayStatics|GetStreamingLevel (Variables|Level|GetLoad%20Level%20Name)))
              (Utilities|Struct|SetmembersinStruct_Game_Locations (Variables|/Game/Game/DW1_GameInstance.DW1_GameInstance_C|GetGame%20Location%20and%20Rotation (LocalVariables|GetGameInstanceLocal)) (Variables|Level|GetLoad%20Level%20Name) (Variables|Level|GetLevelIndex) (LocalVariables|GetPreviousLevelName) (LocalVariables|GetPreviousLevelIndex))
              (return true (LocalVariables|GetPreviousLevelName))
              (else
                _)))
          (:RowNotFound
            _)))
      (Development|PrintString "CURRENT LEVEL NAME NOT VALID")
      (return false "None"))
    (:CastFailed
      (Development|PrintString "GAMEINSTANCE FAILED")
      (return false "None"))))

(fn ItemSpawnFunction
  (bind _output_get (LocalVariables|SetItemArray (CallFunction|ItemCalculateSpawn)))
  (for _array_element _output_get
    (bind _output_get_2 (LocalVariables|SetItemElement _array_element))
    (Game|SpawnActorfromClass "/Game/BluePrints/Interactible/BP_Item.BP_Item_C" (Math|Transform|MakeTransform (.Location (Utilities|Struct|BreakStruct_Item_Spawn _output_get_2))) "AlwaysSpawn" self (.ItemName (Utilities|Struct|BreakStruct_Item_Spawn _output_get_2)) 0)))

(fn MonitorSpawnFunction
  (bind (_monitor_array _index_array) (CallFunction|ItemCalculateMonitor))
  (bind _returnvalue (Math|Float|MakeLiteralFloat 1.5))
  (LocalVariables|SetMonitorArray _monitor_array)
  (LocalVariables|SetIndexArray _index_array)
  (for (_array_element _array_index) (LocalVariables|GetMonitorArray)
    (bind _output_get (LocalVariables|SetMonitorElement _array_element))
    (LocalVariables|SetIndexElement _array_index)
    (if (Utilities|Array|IsValidIndex (LocalVariables|GetIndexArray) (LocalVariables|GetIndexElement))
      (Game|SpawnActorfromClass "/Game/BluePrints/Interactible/BP_Monitor.BP_Monitor_C" (Math|Transform|MakeTransform (.Location (Math|Transform|BreakTransform (Utilities|Struct|BreakStruct_Item_Monitor _output_get))) (Math|Rotator|MakeRotator 0.0 0.0 (.Yaw (Math|Rotator|BreakRotator (.Rotation (Math|Transform|BreakTransform (Utilities|Struct|BreakStruct_Item_Monitor _output_get)))))) (Math|Vector|MakeVector _returnvalue _returnvalue _returnvalue)) "AlwaysSpawn" 0 (Utilities|Array|Get(acopy) (LocalVariables|GetIndexArray) (LocalVariables|GetIndexElement)) (Utilities|Struct|BreakStruct_Item_Monitor (LocalVariables|GetMonitorElement)) 0))))