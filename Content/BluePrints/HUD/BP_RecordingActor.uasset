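; Stage actor that films the Digimon partner's death and digivolution cinematics through its own camera.
; Meshes, animations and materials load from the Digimon data table.
; Death streams in Jijimon's house, moves player and partner there, then timelines shrink or move components and start the death dialogue.
; Digivolution spins the current form with glow and wireframe, swaps meshes under a white fade, notifies the partner system and destroys itself.
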(event EventRecordingActorDestroy
  ;[1 1 1 1 200] DIGIVOLUTION
  ;;[1 1 1 1 100] DESTROY
  (Actor|DestroyActor self))

(event EventRecordingActorDeath
  (bind _skeletalmesh_digimon (Variables|Default|GetSkeletalMesh_Digimon))
  ;[1 1 1 1 200] DEATH CINEMATIC 1
  (Utilities|FlowControl|DoOnce false
    (:Completed
      (Utilities|DeathCinematicMacro
        (:Output
          (bind (_direction _scale _sphere_location) (Timeline|Death_01 PlayFromStart)
            (:Update
              (Transformation|SetRelativeScale3D _skeletalmesh_digimon (* _scale (Utilities|Struct|BreakStruct_Digimon_Info (Variables|Digivolution|GetDigimonInfo))))
              (Transformation|SetRelativeLocation (Variables|Default|GetSphere_Life) _sphere_location false false))
            (:Finished
              (Utilities|FlowControl|Sequence
                (:then_0
                  (Components|DestroyComponent (Variables|Default|GetSphere_Life)))
                (:then_1
                  (for _index (range 0 (- (Rendering|Material|GetNumMaterials _skeletalmesh_digimon) 1))
                    (Rendering|Material|SetMaterial _skeletalmesh_digimon _index "/Game/Material/Material_Life_Sphere.Material_Life_Sphere")))
                (:then_2
                  (bind _blackfade_jijimon (Timeline|Death_02 PlayFromStart)
                    (:Update
                      (Transformation|SetRelativeLocation (Variables|Default|GetPlane_Jijimon) (Math|Vector|MakeVector _blackfade_jijimon 0.0 0.0) false false))
                    (:Finished
                      (bind _outactors (Actor|GetAllActorswithInterface "/Game/BluePrints/BPI/BPI_Dialogue.BPI_Dialogue_C"))
                      (for _array_element _outactors
                        (Class|BPIDialogue|DialogueSystemLock(Message) _array_element false)
                        (Class|BPIDialogue|DialogueSystemValuesSet(Message) _array_element 0 "/Game/Game/DataTables/Dialogue/Events/DataTable_Dialogue_DeathSequence.DataTable_Dialogue_DeathSequence" true)))))))))))))

(event EventRecordingActorDigivolution
  (params (Digimon%20Name :type Name :default "None"))
  (bind _returnvalue (Math|Float|MakeLiteralFloat 1.0))
  (bind _returnvalue_2 (Game|GetPlayerCameraManager 0))
  (bind _digimoninfo (Variables|Digivolution|GetDigimonInfo))
  (bind _skeletalmesh_digimon (Variables|Default|GetSkeletalMesh_Digimon))
  (bind _skeletalmesh_digimon_2 (Variables|Default|GetSkeletalMesh_Digimon))
  (bind (_mesh _animation _material) (Utilities|Struct|BreakStruct_Digimon_Info _digimoninfo))
  ;[1 1 1 1 200] DIGIVOLUTION
  ;;[1 1 1 1 100] Add Mesh
  (bind _valid_ (CallFunction|AddMeshDigivolution Digimon%20Name))
  (if _valid_
    (Utilities|FlowControl|DoOnce false
      (:Completed
        ;;[1 1 1 1 100] Destroy Components
        (Components|DestroyComponent (Variables|Default|GetSphere_Life))
        ;;[1 1 1 1 100] CAMERA
        (Game|Player|SetViewTargetwithBlend (Game|GetPlayerController 0) (Components|GetOwner (Variables|Default|GetCamera)) 0.0 "VTBlend_Linear" 0.0 false)
        (Utilities|FlowControl|Delay 1.0)
        (CameraFades|StartCameraFade :self (Game|GetPlayerCameraManager 0) :FromAlpha 1.0 :Duration _returnvalue :bShouldFadeAudio true :bHoldWhenFinished true)
        (Utilities|FlowControl|Delay _returnvalue)
        (bind (_direction _rotation _glow) (Timeline|Digivolution_Sequence_Timeline PlayFromStart)
          (:Update
            (Rendering|Material|SetScalarParameterValueonMaterials _skeletalmesh_digimon_2 "Glow" _glow)
            (Transformation|SetWorldRotation _skeletalmesh_digimon_2 (Math|Rotator|MakeRotator 0.0 0.0 _rotation) false false))
          (:Sound%20and%20Materials
            (Utilities|FlowControl|Sequence
              (:then_0
                (Audio|PlaySound2D "/Game/Audio/SFX/Ambient/Digivolution_01.Digivolution_01" 1.0 1.0 0.0 0 0))
              (:then_1
                (Rendering|Material|SetMaterial (Variables|Default|GetPlane) 0 "/Game/Material/Neon/Material_Glow_Digievolution1.Material_Glow_Digievolution1")
                (for _index (range 0 (- (Rendering|Material|GetNumMaterials _skeletalmesh_digimon) 1))
                  (Rendering|Material|SetMaterial _skeletalmesh_digimon _index "/Game/Material/Neon/Material_Wireframe_Inst.Material_Wireframe_Inst")))
              (:then_2
                (CallFunction|SetAnimation 0 (Components|SkeletalMesh|GetAnimInstance (Variables|Default|GetSkeletalMesh_Digimon))))))
          (:White%20Fade
            (bind _isa (Utilities|FlowControl|FlipFlop)
              (:A
                _)
              (:B
                _))
            (if _isa
              (CameraFades|StartCameraFade _returnvalue_2 0.0 1.0 1.0 "(R=1.000000,G=1.000000,B=1.000000,A=1.000000)" false true)
              (Utilities|FlowControl|Delay 1.0)
              (Class|SkeletalMeshComponent|SetAnimClass (Variables|Default|GetSkeletalMesh_Digimon))
              (Class|SkinnedMeshComponent|SetSkeletalMesh (Variables|Default|GetSkeletalMesh_Digimon) _mesh true)
              (Class|SkeletalMeshComponent|SetAnimClass (Variables|Default|GetSkeletalMesh_Digimon) _animation)
              (for (_array_element _array_index) _material
                (Rendering|Material|SetMaterial (Variables|Default|GetSkeletalMesh_Digimon) _array_index _array_element))
              (else
                (CameraFades|StartCameraFade _returnvalue_2 1.0 0.0 1.0 "(R=1.000000,G=1.000000,B=1.000000,A=1.000000)" false true))))
          (:Finish%20and%20Fade
            (CameraFades|StartCameraFade :self (Game|GetPlayerCameraManager 0) :ToAlpha 1.0 :Duration 1.0 :bShouldFadeAudio true :bHoldWhenFinished true)
            (Utilities|FlowControl|Delay 1.2)
            (bind _outactors (Actor|GetAllActorswithInterface "/Game/BluePrints/BPI/BPI_DigimonPartnerSystem.BPI_DigimonPartnerSystem_C"))
            (for _array_element_2 _outactors
              (Class|BPIDigimonPartnerSystem|DigivolutionEnd(Message) _array_element_2))
            (Actor|DestroyActor self)))))
    (else
      (Development|PrintString "Digimon Name NOT FOUND" true true "(R=1.000000,G=0.000000,B=0.000000,A=1.000000)"))))

(event EventRecordingActorSetMesh
  (params (Digimon%20Name :type Name :default "None"))
  ;[1 0.4453 0.7623 1 200] Set Mesh
  (Components|DestroyComponent (Variables|Default|GetSphere_Life))
  (bind _valid_ (CallFunction|AddMesh Digimon%20Name))
  (if (not _valid_)
    (Development|PrintString "Digimon Name NOT FOUND" true true "(R=1.000000,G=0.000000,B=0.000000,A=1.000000)")))

(fn ConstructionScript)

(fn AddMeshDigivolution
  (params (DigivolutionName :type Name))
  (bind _camera (Variables|Default|GetCamera))
  (bind _skeletalmesh_digimon (Variables|Default|GetSkeletalMesh_Digimon))
  (bind _skeletalmesh_digimon_2 (Variables|Default|GetSkeletalMesh_Digimon))
  (bind _relativelocation (Variables|/Script/Engine.SceneComponent|GetRelativeLocation _camera))
  (bind (_x _y _z) (Math|Vector|BreakVector _relativelocation))
  (Variables|Digivolution|SetDigivolutionName DigivolutionName)
  ;[1 1 1] Clean Mesh
  (Class|SkeletalMeshComponent|SetAnimClass _skeletalmesh_digimon)
  (Class|SkinnedMeshComponent|SetSkeletalMesh _skeletalmesh_digimon 0 true)
  ;[1 1 1] Digivolution Info
  (bind _returnvalue (Class|DataTableFunctionLibrary|DoesDataTableRowExist "/Game/Game/DataTables/DigimonInfo/DataTable_Digimon_Info.DataTable_Digimon_Info" (Variables|Digivolution|GetDigivolutionName)))
  (if _returnvalue
    (bind _returnvalue_2 (Utilities|GetDataTableRow "/Game/Game/DataTables/DigimonInfo/DataTable_Digimon_Info.DataTable_Digimon_Info" (Variables|Digivolution|GetDigivolutionName))
      (:then
        (Variables|Digivolution|SetDigimonInfo _returnvalue_2)
        ;[1 1 1] Current Digimon Mesh
        (bind _asdw1_game_instance (Utilities|Casting|CastToDW1_GameInstance (Game|GetGameInstance))
          (:then
            (LocalVariables|SetCurrentDigimonName (Utilities|Struct|BreakStruct_Digimon_Partner_Info (Variables|/Game/Game/DW1_GameInstance.DW1_GameInstance_C|GetPartner%20Info _asdw1_game_instance)))
            (bind _returnvalue_3 (Class|DataTableFunctionLibrary|DoesDataTableRowExist "/Game/Game/DataTables/DigimonInfo/DataTable_Digimon_Info.DataTable_Digimon_Info" (LocalVariables|GetCurrentDigimonName)))
            (if _returnvalue_3
              (bind _returnvalue_4 (Utilities|GetDataTableRow "/Game/Game/DataTables/DigimonInfo/DataTable_Digimon_Info.DataTable_Digimon_Info" (LocalVariables|GetCurrentDigimonName))
                (:then
                  (LocalVariables|SetCurrentDigimonInfo _returnvalue_4)
                  (Class|SkinnedMeshComponent|SetSkeletalMesh _skeletalmesh_digimon_2 (.Mesh (Utilities|Struct|BreakStruct_Digimon_Info (LocalVariables|GetCurrentDigimonInfo))) true)
                  (Class|SkeletalMeshComponent|SetAnimClass _skeletalmesh_digimon_2 (.Animation (Utilities|Struct|BreakStruct_Digimon_Info (LocalVariables|GetCurrentDigimonInfo))))
                  (for (_array_element _array_index) (.Material (Utilities|Struct|BreakStruct_Digimon_Info (LocalVariables|GetCurrentDigimonInfo)))
                    (Rendering|Material|SetMaterial _skeletalmesh_digimon_2 _array_index _array_element))
                  (Transformation|SetRelativeLocation (Variables|Default|GetCamera) (Math|Vector|MakeVector (+ (Math|Conversions|ToFloat(Integer) (Math|Integer|Clamp(Integer) (Utilities|Struct|BreakStruct_Digimon_Info (LocalVariables|GetCurrentDigimonInfo)) 0 2000)) _x) _y (+ _z (Math|Conversions|ToFloat(Integer) (Math|Integer|Clamp(Integer) (Utilities|Struct|BreakStruct_Digimon_Info (LocalVariables|GetCurrentDigimonInfo)) 0 2000)))) false false)
                  (return true))
                (:RowNotFound
                  (return false)))
              (else
                (Development|PrintString "DigimonName ROW NOT FOUND" false)
                (return false))))
          (:CastFailed
            (return false))))
      (:RowNotFound
        _))
    (else
      (Development|PrintString "DigimonName ROW NOT FOUND")))
  (return false))

(fn AddMesh
  (params (DigivolutionName :type Name))
  (bind _camera (Variables|Default|GetCamera))
  (bind _skeletalmesh_digimon (Variables|Default|GetSkeletalMesh_Digimon))
  (bind _skeletalmesh_digimon_2 (Variables|Default|GetSkeletalMesh_Digimon))
  (bind _relativelocation (Variables|/Script/Engine.SceneComponent|GetRelativeLocation _camera))
  (bind (_x _y _z) (Math|Vector|BreakVector _relativelocation))
  (LocalVariables|SetCurrentDigimonName DigivolutionName)
  ;[1 1 1 1 200] Clean Mesh
  (Class|SkeletalMeshComponent|SetAnimClass _skeletalmesh_digimon)
  (Class|SkinnedMeshComponent|SetSkeletalMesh _skeletalmesh_digimon 0 true)
  ;[1 1 1 1 200] Digimon Info
  (bind _returnvalue (Class|DataTableFunctionLibrary|DoesDataTableRowExist "/Game/Game/DataTables/DigimonInfo/DataTable_Digimon_Info.DataTable_Digimon_Info" (LocalVariables|GetCurrentDigimonName)))
  (if _returnvalue
    (bind _returnvalue_2 (Utilities|GetDataTableRow "/Game/Game/DataTables/DigimonInfo/DataTable_Digimon_Info.DataTable_Digimon_Info" (LocalVariables|GetCurrentDigimonName))
      (:then
        (Variables|Digivolution|SetDigimonInfo _returnvalue_2)
        ;[1 1 1 1 200] Set Digimon Mesh
        (Class|SkinnedMeshComponent|SetSkeletalMesh _skeletalmesh_digimon_2 (.Mesh (Utilities|Struct|BreakStruct_Digimon_Info (Variables|Digivolution|GetDigimonInfo))) true)
        (Class|SkeletalMeshComponent|SetAnimClass _skeletalmesh_digimon_2 (.Animation (Utilities|Struct|BreakStruct_Digimon_Info (Variables|Digivolution|GetDigimonInfo))))
        (for (_array_element _array_index) (.Material (Utilities|Struct|BreakStruct_Digimon_Info (Variables|Digivolution|GetDigimonInfo)))
          (Rendering|Material|SetMaterial _skeletalmesh_digimon_2 _array_index _array_element))
        (Transformation|SetRelativeLocation (Variables|Default|GetCamera) (Math|Vector|MakeVector _x _y (+ _z (Math|Conversions|ToFloat(Integer) (Utilities|Struct|BreakStruct_Digimon_Info (Variables|Digivolution|GetDigimonInfo))))) false false)
        (return true))
      (:RowNotFound
        (return false)))
    (else
      (Development|PrintString "DigimonName ROW NOT FOUND")
      (return false))))