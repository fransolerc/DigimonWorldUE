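; BP_Elevator is an environment actor that animates an elevator's two doors when its GameEvent fires.
; GameEvent plays a 2D sound and runs a timeline that slides the left and right door components along their local Y axis.
; When the timeline finishes, it plays a second sound and sends DialogueSystemUpdateMessage to every actor implementing BPI_Dialogue, linking the door animation to dialogue progression.
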(event EventGameEvent
  (params (Index :type Integer))
  (Audio|PlaySound2D "/Game/Audio/SFX/Ambient/Elevator01.Elevator01" 1.0 1.0 0.0 0 0)
  (bind (_direction _left _right) (Timeline|Línea%20de%20tiempo_0 PlayFromStart)
    (:Update
      (Transformation|SetRelativeLocation (Variables|Default|GetGC03_ElevatorDoor_L) (Math|Vector|MakeVector 0.0 _left 0.0) false false)
      (Transformation|SetRelativeLocation (Variables|Default|GetGC03_ElevatorDoor_R) (Math|Vector|MakeVector 0.0 _right 0.0) false false))
    (:Finished
      (Audio|PlaySound2D "/Game/Audio/SFX/Ambient/elevator02.Elevator02" 1.0 1.0 0.0 0 0)
      (bind _outactors (Actor|GetAllActorswithInterface "/Game/BluePrints/BPI/BPI_Dialogue.BPI_Dialogue_C"))
      (for _array_element _outactors
        (Class|BPIDialogue|DialogueSystemUpdate(Message) _array_element true)))))

(fn ConstructionScript)