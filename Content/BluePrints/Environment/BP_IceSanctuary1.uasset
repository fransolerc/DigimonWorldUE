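; BP_IceSanctuary1 is an Ice Sanctuary environment actor that manages a movable block and an Angemon statue.
; GameEvent slides the block along Y with a one-shot timeline, then sends a dialogue update to every BPI_Dialogue actor.
; BeginPlay restores state from GameInstance triggers: Angemon recruitment or the second statue talk places the block aside and removes the statue, while stepping into the light only removes the statue.
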(event EventBeginPlay
  ;[1 1 1 1 100] BeginPlay
  (bind _asdw1_game_instance (Utilities|Casting|CastToDW1_GameInstance (Game|GetGameInstance)))
  (Variables|Default|SetGameInstance _asdw1_game_instance)
  (if (.Trigger27-RecruitedAngemon (Utilities|Struct|BreakStruct_Game_Triggers (Variables|/Game/Game/DW1_GameInstance.DW1_GameInstance_C|GetGame%20Triggers (Variables|Default|GetGameInstance))))
    (Transformation|SetRelativeLocation (Variables|Default|GetCube) "0,-680.000000,50.000000" false false :!label _label)
    (Components|DestroyComponent (Variables|Default|GetMesh_Digimon_AngemonStatue) :!label _label_2)
    (elif (.Trigger102-IceSanctuary-SecondTalkwithStatue (Utilities|Struct|BreakStruct_Game_Triggers (Variables|/Game/Game/DW1_GameInstance.DW1_GameInstance_C|GetGame%20Triggers (Variables|Default|GetGameInstance))))
      (goto _label)
      (elif (.Trigger103-IceSanctuary-SteppedintotheLight (Utilities|Struct|BreakStruct_Game_Triggers (Variables|/Game/Game/DW1_GameInstance.DW1_GameInstance_C|GetGame%20Triggers (Variables|Default|GetGameInstance))))
        (goto _label_2)))))

(event EventGameEvent
  (params (Boolean :type Boolean))
  ;[1 1 1 1 100] MOVE BLOCK
  (Utilities|FlowControl|DoOnce false
    (:Completed
      (bind _location (Timeline|Línea%20de%20tiempo_0 PlayFromStart)
        (:Update
          (Transformation|SetRelativeLocation (Variables|Default|GetCube) (Math|Vector|MakeVector 0.0 _location 5e+01) false false))
        (:Finished
          (bind _outactors (Actor|GetAllActorswithInterface "/Game/BluePrints/BPI/BPI_Dialogue.BPI_Dialogue_C"))
          (for _array_element _outactors
            (Class|BPIDialogue|DialogueSystemUpdate(Message) _array_element true)))))))

(fn ConstructionScript)