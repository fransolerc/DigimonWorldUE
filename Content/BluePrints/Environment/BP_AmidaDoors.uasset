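; BP_AmidaDoors is an Amida Forest door whose Correct flag sets a circle or cross decal in the construction script.
; Only correct doors react to player overlap, once, playing a sound, stopping time and fading the HUD through interface broadcasts, and disabling input.
; A timeline then sinks the door.
; When it finishes, Centarumon's dialogue autoplays and every TriggerBox and Amida door is destroyed.
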(event OnComponentBeginOverlap(BoxCollision)
  (params (OverlappedComponent :type Primitive%20Component%20Object%20Reference) (OtherActor :type Actor%20Object%20Reference) (OtherComp :type Primitive%20Component%20Object%20Reference) (OtherBodyIndex :type Integer) (bFromSweep :type Boolean) (SweepResult :type Hit%20Result%20Structure%20%28by%20ref%29))
  (bind _self self)
  (bind _returnvalue (Transformation|GetActorLocation _self))
  (bind (_x _y _z) (Math|Vector|BreakVector _returnvalue))
  ;[1 1 1 1 200] Box Collision
  (Utilities|Casting|CastToJugador OtherActor)
  (if (Variables|Default|GetCorrect?)
    (Utilities|FlowControl|DoOnce false
      (:Completed
        (Utilities|FlowControl|Sequence
          (:then_0
            (Audio|PlaySound2D "/Game/Audio/SFX/Ambient/AmidaForest03.AmidaForest03" 1.0 1.0 0.0 0 0))
          (:then_1
            (bind _outactors (Actor|GetAllActorswithInterface "/Game/BluePrints/BPI/BPI_Time.BPI_Time_C"))
            (for _array_element _outactors
              (Class|BPITime|TimeStop(Message) _array_element)))
          (:then_2
            (bind _foundwidgets (Class|WidgetBlueprintLibrary|GetAllWidgetswithInterface "/Game/BluePrints/BPI/BPI_HUD_Game.BPI_HUD_Game_C" true))
            (for _array_element_2 _foundwidgets
              (Class|BPIHUDGame|GameHUDFadeOut(Message) _array_element_2)))
          (:then_3
            (Input|DisableInput (Game|GetPlayerCharacter 0) (Game|GetPlayerController 0)))
          (:then_4
            (Components|DestroyComponent (Variables|Default|GetBoxCollision)))
          (:then_5
            (bind _location (Timeline|Línea%20de%20tiempo_0 PlayFromStart)
              (:Update
                (Transformation|SetActorLocation self (Math|Vector|MakeVector _x _y (- _z _location)) false false))
              (:Finished
                (Utilities|FlowControl|Sequence
                  (:then_0
                    (bind _outactors_2 (Actor|GetAllActorswithInterface "/Game/BluePrints/BPI/BPI_Dialogue.BPI_Dialogue_C"))
                    (for _array_element_3 _outactors_2
                      (Class|BPIDialogue|DialogueSystemLock(Message) _array_element_3 false)
                      (Class|BPIDialogue|DialogueSystemValuesSet(Message) _array_element_3 0 "/Game/Game/DataTables/Dialogue/AmidaForest/DataTable_Dialogue_AmidaForest_Centarumon.DataTable_Dialogue_AmidaForest_Centarumon" true)))
                  (:then_1
                    (bind _outactors_3 (Actor|GetAllActorsOfClass "/Script/Engine.TriggerBox"))
                    (for _array_element_4 _outactors_3
                      (Utilities|IsValid _array_element_4
                        (:Is%20Valid
                          (Actor|DestroyActor _array_element_4)))))
                  (:then_2
                    (bind _outactors_4 (Actor|GetAllActorsOfClass "BP_AmidaDoors_C"))
                    (for _array_element_5 _outactors_4
                      (Utilities|IsValid _array_element_5
                        (:Is%20Valid
                          (Actor|DestroyActor _array_element_5))))))))))))))

(fn ConstructionScript
  (Rendering|Components|Decal|SetDecalMaterial (Variables|Default|GetDecal) (select (Variables|Default|GetCorrect?) "/Game/Material/AmidaForest/Material_AmidaDoors_Circle.Material_AmidaDoors_Circle" "/Game/Material/AmidaForest/Material_AmidaDoors_Cross.Material_AmidaDoors_Cross")))