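; BP_SecretBeachCave is an environment actor for the secret beach cave that shows a submarine until Whamon is recruited.
; On BeginPlay it reads the Trigger15RecruitedWhamon flag from DW1_GameInstance and, if set, destroys the submarine body, upper door, door lock and side door components.
; Otherwise a timeline drives the submarine body's relative Z position, leaving X and Y unchanged.
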(event EventBeginPlay
  (bind _submarine_body (Variables|Default|Getsubmarine_body))
  (bind _relativelocation (Variables|/Script/Engine.SceneComponent|GetRelativeLocation _submarine_body))
  (bind (_x _y) (Math|Vector|BreakVector _relativelocation))
  (bind _asdw1_game_instance (Utilities|Casting|CastToDW1_GameInstance (Game|GetGameInstance)))
  (if (Utilities|Struct|BreakStruct_Game_Triggers (Variables|/Game/Game/DW1_GameInstance.DW1_GameInstance_C|GetGame%20Triggers _asdw1_game_instance))
    (Components|DestroyComponent (Variables|Default|Getsubmarine_body))
    (else
      (bind _location (Timeline|Línea%20de%20tiempo_1 PlayFromStart)
        (:Update
          (Transformation|SetRelativeLocation _submarine_body (Math|Vector|MakeVector _x _y _location) false false))))))

(fn ConstructionScript)