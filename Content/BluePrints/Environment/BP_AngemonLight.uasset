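; BP_AngemonLight is an Ice Sanctuary trigger actor that starts the stepped-into-the-light dialogue event.
; On BeginPlay it caches the game instance and destroys itself if that event's game trigger is already set.
; The first player overlap with its sphere sends unlock and auto-play dialogue messages, with the event's data table, to every BPI_Dialogue actor.
; It only reads the trigger flag and never sets it.
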(event OnComponentBeginOverlap(Sphere1)
  (params (OverlappedComponent :type Primitive%20Component%20Object%20Reference) (OtherActor :type Actor%20Object%20Reference) (OtherComp :type Primitive%20Component%20Object%20Reference) (OtherBodyIndex :type Integer) (bFromSweep :type Boolean) (SweepResult :type Hit%20Result%20Structure%20%28by%20ref%29))
  ;[1 1 1 1 100] OVERLAP
  (Utilities|Casting|CastToJugador OtherActor)
  (Utilities|FlowControl|DoOnce false
    (:Completed
      (if (not (.Trigger103-IceSanctuary-SteppedintotheLight (Utilities|Struct|BreakStruct_Game_Triggers (Variables|/Game/Game/DW1_GameInstance.DW1_GameInstance_C|GetGame%20Triggers (Variables|Default|GetAs%20DW1%20Game%20Instance)))))
        (bind _outactors (Actor|GetAllActorswithInterface "/Game/BluePrints/BPI/BPI_Dialogue.BPI_Dialogue_C"))
        (for _array_element _outactors
          (Class|BPIDialogue|DialogueSystemLock(Message) _array_element false)
          (Class|BPIDialogue|DialogueSystemValuesSet(Message) _array_element 0 "/Game/Game/DataTables/Dialogue/IceSanctuary/DataTable_Dialogue_IceSanctuary_Event1.DataTable_Dialogue_IceSanctuary_Event1" true))))))

(event EventBeginPlay
  ;[1 1 1 1 100] BeginPlay
  (bind _asdw1_game_instance (Utilities|Casting|CastToDW1_GameInstance (Game|GetGameInstance)))
  (Variables|Default|SetAs%20DW1%20Game%20Instance _asdw1_game_instance)
  (if (.Trigger103-IceSanctuary-SteppedintotheLight (Utilities|Struct|BreakStruct_Game_Triggers (Variables|/Game/Game/DW1_GameInstance.DW1_GameInstance_C|GetGame%20Triggers (Variables|Default|GetAs%20DW1%20Game%20Instance))))
    (Actor|DestroyActor self)))

(fn ConstructionScript)