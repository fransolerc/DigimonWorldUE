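; Lovely Attack technique: a projectile-style actor that homes in on its target, a partner Digimon or NPC.
; Timeline updates interpolate its location toward the target and set its yaw from a rotation track; the location track feeds VInterpTo's delta time.
; An invalid target prints an error and destroys the actor.
; TechniqueEnd destroys the mesh and capsule and stops the timeline.
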(event EventTechniqueEnd
  (bind _targetactor (Variables|Default|GetTargetActor))
  (Components|DestroyComponent (Variables|Default|GetStaticMesh))
  (bind (_direction _rotation _location) (Timeline|Línea%20de%20tiempo_0 Stop)
    (:Update
      (bind _asai_digimon_partner (Utilities|Casting|CastToAI_DigimonPartner _targetactor)
        (:then
          (Variables|Default|SetTarget (Transformation|GetActorLocation _asai_digimon_partner))
          (Transformation|SetActorLocationAndRotation self (Math|Interpolation|VInterpTo (Transformation|GetActorLocation self) (Variables|Default|GetTarget) _location 0.1) (Math|Rotator|MakeRotator 0.0 0.0 _rotation) :!label _label))
        (:CastFailed
          (bind _asai_npc (Utilities|Casting|CastToAI_NPC _targetactor)
            (:then
              (Variables|Default|SetTarget (Transformation|GetActorLocation _asai_npc))
              (goto _label))
            (:CastFailed
              (Development|PrintString "ACTOR NOT VALID")
              (Actor|DestroyActor self))))))))

(fn ConstructionScript
  (|CallParentFunction))