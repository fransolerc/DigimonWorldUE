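; Electric Cloud technique actor that moves from its owner to a target, each being a Digimon partner or NPC AI.
; A timeline, with no Play call in the graph, re-reads both locations each update, lerping XY and offsetting Z from the target's height.
; On finish it enables sphere overlaps for 0.2 seconds and swaps black-cloud trails for megaspark trails.
; An invalid owner or target destroys the actor.
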(fn ConstructionScript
  (|CallParentFunction))