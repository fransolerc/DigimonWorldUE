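; BP_Technique_PartyTime is a technique actor that travels from its owner to TargetActor, each either a Digimon partner or an NPC.
; On BeginPlay a timeline interpolates X/Y between both live positions and adds a height curve to the target's Z, destroying the actor if either cast fails.
; When the timeline finishes, the mesh is removed and the capsule generates overlap events for a brief window before being destroyed.
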(event EventBeginPlay
  (bind _self self)
  (bind _capsule (Variables|Default|GetCapsule))
  (bind _targetactor (Variables|Default|GetTargetActor))
  (bind _returnvalue (Components|GetOwner _self))
  (bind (_direction _xy _z) (Timeline|Línea%20de%20tiempo_0 PlayFromStart)
    (:Update
      (bind _asai_digimon_partner (Utilities|Casting|CastToAI_DigimonPartner _returnvalue)
        (:then
          (Variables|Default|SetSpawn (Transformation|GetActorLocation _asai_digimon_partner))
          (bind _asai_digimon_partner_2 (Utilities|Casting|CastToAI_DigimonPartner _targetactor :!label _label)
            (:then
              (Variables|Default|SetTarget (Transformation|GetActorLocation _asai_digimon_partner_2))
              (Transformation|SetActorLocation self (Math|Vector|MakeVector (Math|Float|Lerp (.X (Math|Vector|BreakVector (Variables|Default|GetSpawn))) (.X (Math|Vector|BreakVector (Variables|Default|GetTarget))) _xy) (Math|Float|Lerp (.Y (Math|Vector|BreakVector (Variables|Default|GetSpawn))) (.Y (Math|Vector|BreakVector (Variables|Default|GetTarget))) _xy) (+ _z (.Z (Math|Vector|BreakVector (Variables|Default|GetTarget))))) false false :!label _label_2))
            (:CastFailed
              (bind _asai_npc (Utilities|Casting|CastToAI_NPC _targetactor)
                (:then
                  (Variables|Default|SetTarget (Transformation|GetActorLocation _asai_npc))
                  (goto _label_2))
                (:CastFailed
                  (Development|PrintString "ACTOR NOT VALID" :!label _label_3)
                  (Actor|DestroyActor self))))))
        (:CastFailed
          (bind _asai_npc_2 (Utilities|Casting|CastToAI_NPC _returnvalue)
            (:then
              (Variables|Default|SetSpawn (Transformation|GetActorLocation _asai_npc_2))
              (goto _label))
            (:CastFailed
              (goto _label_3))))))
    (:Finished
      (Variables|/Script/Engine.PrimitiveComponent|SetbGenerateOverlapEvents _capsule true)
      (Components|DestroyComponent (Variables|Default|GetStaticMesh))
      (Utilities|FlowControl|Delay 0.2)
      (Components|DestroyComponent _capsule))))

(fn ConstructionScript
  (|CallParentFunction))